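; Base boss enemy Blueprint that feeds its AI Blackboard and provides shared hooks for attacks and temporary invincibility frames.
; BeginPlay writes ranged AoE and melee attack distances, and pawn sensing stores a seen BP_Player as the target.
; Attacks set an IsAttacking key and call PlayMontage, while a timer clears the i-frame flag.
; DeathSequence and SpecialAttack are empty, and DecideTarget is a placeholder that always reports a target.
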(event `self.ReceiveBeginPlay`
  (`self.SettingBBVariables`))

(event `Start_I_Frames`
  (params (Duration :type "Float (double-precision)"))
  ; IFrames
  (set `self.Iframe Active` true)
  (`KismetSystemLibrary.K2_SetTimerDelegate` (delegate `Stop_I_Frames`) Duration))

(event `IsAttacking?`
  (params (`IsAttacking?` :type Boolean))
  ; IsAttacking BB
  (`BlackboardComponent.SetValueAsBool` (`AIBlueprintHelperLibrary.GetBlackboard` null) "IsAttacking?" `IsAttacking?`))

(event `/Game/AI/BossAI/IF_EnemyBehaviourPass.AttackInterface`
  (`self.IsAttacking?` true)
  (`|PlayMontage` (`self.Mesh`)))

(event `Stop_I_Frames`
  ; IFrames
  (set `self.Iframe Active` false))

(event `DeathSequence`)

(event `SettingBBVariables`
  ; BlackBoard Variables
  (`BlackboardComponent.SetValueAsFloat` (`AIBlueprintHelperLibrary.GetBlackboard` null) "RangedAoeAttackDistance" (`self.RangedAoeAttackDistance`))
  (`BlackboardComponent.SetValueAsFloat` (`AIBlueprintHelperLibrary.GetBlackboard` null) "MeleeAttackDistance" (`self.MeleeAttackDistance`)))

(event `/Game/AI/BossAI/IF_EnemyBehaviourPass.SpecialAttack`)

(event `self.PawnSensing.OnSeePawn`
  (params (Pawn :type "Pawn Object Reference"))
  (bind (_asbp_player _bsuccess) (cast `/Game/Blueprints/BP_Player` Pawn :!pure true))
  (bind _returnvalue (`AIBlueprintHelperLibrary.GetBlackboard` (`AIBlueprintHelperLibrary.GetAIController` self)))
  (bind _output_get (set `self.ChaseTarget` _asbp_player))
  (if _bsuccess
    (`BlackboardComponent.SetValueAsObject` _returnvalue "Player" _output_get)
    (`BlackboardComponent.SetValueAsBool` _returnvalue "FoundPlayer" true)))

(fn `DecideTarget`
  (params (`TargetRanged?` :type Boolean))
  (returns (`Has Target?` :type Boolean) (Player :type "Actor Object Reference"))
  (if `TargetRanged?`
    ; Check if ranged character in game
    (if true
      ; Set BB player value to ranged Player
      (return true null)
      (else
        _))
    (else
      ; Check if Melee character in game
      (if true
        ; Set BB player value to Melee player
        (return true null)
        (else
          _))))
  ; Set BB player value to random player
  (return true null))

(fn `UserConstructionScript`)