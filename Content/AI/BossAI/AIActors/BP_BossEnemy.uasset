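; Boss enemy character that waits for players to spawn, then runs BT_BossEnemy.
; Sight and damage set the chase target, while blackboard keys carry attack distances, cooldowns and health from the health component.
; Exposes attack events: radial slam with camera shake and distance-scaled launch, randomized fireball fan, and portals spawned near every player.
; Helper functions pick targets by closest distance or randomly by ranged/melee weapon choice.
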(event `SettingBBVariables`
  ;[1 0.004025 0.7835] BlackBoard Variables
  (`BlackboardComponent.SetValueAsFloat` (`AIBlueprintHelperLibrary.GetBlackboard` null) "RangedAoeAttackDistance" (`self.RangedAoeAttackDistance`))
  (`BlackboardComponent.SetValueAsFloat` (`AIBlueprintHelperLibrary.GetBlackboard` null) "MeleeAttackDistance" (`self.MeleeAttackDistance`))
  (`BlackboardComponent.SetValueAsFloat` (`AIBlueprintHelperLibrary.GetBlackboard` null) "BackAwayDistance" (`self.BackAwayDistance`)))

(event `Toggle Attack Cooldown`
  (params (Cooldown :type "Float (double-precision)"))
  (bind _returnvalue (`AIBlueprintHelperLibrary.GetBlackboard` (`AIBlueprintHelperLibrary.GetAIController` self)))
  ;[1 0.004025 0.7835] Sets Attack Cooldown - Called from toggle cooldown task
  (`KismetSystemLibrary.Delay` Cooldown)
  (`/Engine/EditorBlueprintResources/StandardMacros.IsValid` _returnvalue
    (:`Is Valid`
      (`BlackboardComponent.SetValueAsBool` _returnvalue "AttackCooldown" false))))

(event `self.PawnSensing.OnSeePawn`
  (params (Pawn :type "Pawn Object Reference"))
  ;[1 0.004025 0.7835] Trigger Chase On Sight
  (`self.Set Chase Target` Pawn))

(event `self.ReceiveBeginPlay`
  (bind _ac_enemyhealthcomponent (`self.AC_EnemyHealthComponent`))
  (bind _maxhealth (`/Game/Blueprints/Components/AC_HealthComponent.MaxHealth` _ac_enemyhealthcomponent))
  (bind _returnvalue (`AIBlueprintHelperLibrary.GetBlackboard` (`AIBlueprintHelperLibrary.GetAIController` self)))
  ;[1 0.004025 0.7835] Initializes Health Values
  (`KismetSystemLibrary.Delay` 0.5)
  (bind _outactors (`GameplayStatics.GetAllActorsOfClass` "/Game/Blueprints/BP_Player.BP_Player_C" :!label _label))
  (if (`KismetArrayLibrary.Array_IsEmpty` _outactors)
    (`KismetSystemLibrary.Delay` 0.2)
    (goto _label)
    (else
      (for _array_element _outactors
        (`KismetArrayLibrary.Array_Add` (`self.AllKnownPlayers`) _array_element))
      (`AIController.RunBehaviorTree` (`AIBlueprintHelperLibrary.GetAIController` self) "/Game/AI/BossAI/BehaviourTree/BT_BossEnemy.BT_BossEnemy")
      (`self.SettingBBVariables`)
      (`/Game/Blueprints/Components/AC_HealthComponent.HealthCompInit` _ac_enemyhealthcomponent)
      (`BlackboardComponent.SetValueAsFloat` _returnvalue "MaxHealth" _maxhealth)
      (`BlackboardComponent.SetValueAsFloat` _returnvalue "CurrentHealth" _maxhealth)
      (set `PawnSensingComponent.bSeePawns` true (`self.PawnSensing`)))))

(event `self.ReceiveAnyDamage`
  (params (Damage :type "Float (single-precision)") (DamageType :type "DamageType Object Reference") (InstigatedBy :type "Controller Object Reference") (DamageCauser :type "Actor Object Reference"))
  (bind _ac_enemyhealthcomponent (`self.AC_EnemyHealthComponent`))
  (bind _currenthealth (`/Game/Blueprints/Components/AC_HealthComponent.CurrentHealth` _ac_enemyhealthcomponent))
  ;[1 0.004025 0.7835] Handles Damage
  (`/Game/Blueprints/Components/AC_HealthComponent.TakeDamage` (`self.AC_EnemyHealthComponent`) self Damage DamageType InstigatedBy DamageCauser)
  (`self.Set Chase Target` DamageCauser)
  (`KismetSystemLibrary.DelayUntilNextTick`)
  (`BlackboardComponent.SetValueAsFloat` (`AIBlueprintHelperLibrary.GetBlackboard` (`AIBlueprintHelperLibrary.GetAIController` self)) "CurrentHealth" _currenthealth)
  (if (>= (/ _currenthealth (`/Game/Blueprints/Components/AC_HealthComponent.MaxHealth` _ac_enemyhealthcomponent)) 0.33)
    (`BlackboardComponent.SetValueAsBool` (`AIBlueprintHelperLibrary.GetBlackboard` null) "CurrentHealth" true)
    (if (<= _currenthealth 0.0)
      (`self.K2_DestroyActor`))))

(event `/Game/Interfaces/IF_EnemyBehaviourPass.AbilityCooldown`
  (params (Cooldown :type "Float (double-precision)") (AbilityBBName :type Name))
  ;[1 0.004025 0.7835] AbilityCooldown
  (`KismetSystemLibrary.K2_SetTimerDelegate` (delegate `AbilitysCooldown`) Cooldown true))

(event `Set Chase Target`
  (params (Player :type "Actor Object Reference"))
  (bind (_asbp_player _bsuccess) (cast `/Game/Blueprints/BP_Player` Player :!pure true))
  (bind _returnvalue (`AIBlueprintHelperLibrary.GetBlackboard` (`AIBlueprintHelperLibrary.GetAIController` self)))
  ;[1 0.004025 0.7835] Sets chase target and values for the BT
  (bind _output_get (set `self.ChaseTarget` _asbp_player))
  (if _bsuccess
    (`BlackboardComponent.SetValueAsObject` _returnvalue "Player" _output_get)
    (`BlackboardComponent.SetValueAsBool` _returnvalue "HasBeenAlerted" true)
    (`BlackboardComponent.SetValueAsBool` _returnvalue "FarFromPlayer" false)))

(event `AbilitysCooldown`
  ;[1 0.004025 0.7835] AbilityCooldown
  (`BlackboardComponent.SetValueAsBool` (`AIBlueprintHelperLibrary.GetBlackboard` null) (stale `/Game/Interfaces/IF_EnemyBehaviourPass.AbilityCooldown` AbilityBBName) false))

(event `/Game/Interfaces/IF_EnemyBehaviourPass.UpdateSpeed`
  (params (Speed :type "Float (double-precision)"))
  ;[1 0.004025 0.7835] UpdateSPeed
  (set `CharacterMovementComponent.MaxWalkSpeed` Speed (`self.CharacterMovement`)))

(event `/Game/Interfaces/IF_EnemyBehaviourPass.SpecialAttack`
  (bind _returnvalue (`self.K2_GetActorLocation`))
  ; DashAttack
  (`GameplayStatics.ApplyRadialDamageWithFalloff` 30.0 10.0 (`self.K2_GetActorLocation`) 100.0 300.0 2.0 "/Game/Blueprints/WeaponDamageTypes/BP_DamageType_EnemyMelee.BP_DamageType_EnemyMelee_C" (`|MakeArray` self :!type "Actor Object Reference") self null "ECC_WorldStatic")
  (`LegacyCameraShake.StartLegacyCameraShake` (`GameplayStatics.GetPlayerCameraManager` 0) "/Game/AI/BossAI/BP_BossCameraShake.BP_BossCameraShake_C")
  (bind (_outhits _returnvalue_2) (`KismetSystemLibrary.SphereTraceMultiForObjects` :`Start` _returnvalue :`End` _returnvalue :`Radius` 300.0 :`ObjectTypes` (`|MakeArray` "ObjectTypeQuery3" :!type "EObjectTypeQuery Enum") :`DrawDebugType` "ForDuration"))
  (if _returnvalue_2
    (for _array_element _outhits
      (bind (_bblockinghit _binitialoverlap _time _distance _location _impactpoint _normal _impactnormal _physmat _hitactor _hitcomponent _hitbonename _bonename _hititem _elementindex _faceindex _tracestart) (`GameplayStatics.BreakHitResult` _array_element))
      (bind _ascharacter (cast `Character` _hitactor))
      (bind _returnvalue_3 (`KismetMathLibrary.Vector_Distance` _impactpoint _tracestart))
      (`self.LaunchCharacter` _ascharacter (`KismetMathLibrary.MakeVector` 0.0 0.0 (* (`KismetMathLibrary.SelectFloat` 0.5 (`KismetMathLibrary.SelectFloat` 0.8 1.0 (> _returnvalue_3 100.0)) (> _returnvalue_3 200.0)) 1000.0)) false true))))

(event `self.AC_EnemyHealthComponent.DeathEvent`
  ;[0.162 0.02956 0.3515] Death event - needs development and moving to parent. This is bound to the dispatcher in the health component
)

(event `/Game/Interfaces/IF_EnemyBehaviourPass.AimAt`
  (params (Rotation :type "Rotator Structure"))
  (bind (_returnvalue_roll _returnvalue_pitch) (`KismetMathLibrary.BreakRotator` (`SceneComponent.K2_GetComponentRotation` (`self.RootComponent`))))
  (bind (_returnvalue_roll_2 _returnvalue_pitch_2 _returnvalue_yaw) (`KismetMathLibrary.BreakRotator` (`KismetMathLibrary.RInterpTo` (`SceneComponent.K2_GetComponentRotation` (`self.RootComponent`)) Rotation (`GameplayStatics.GetWorldDeltaSeconds`) 15.0)))
  ; Aim At
  (`SceneComponent.K2_SetWorldRotation` (`self.RootComponent`) (`KismetMathLibrary.MakeRotator` _returnvalue_roll _returnvalue_pitch _returnvalue_yaw) false false))

(event `/Game/Interfaces/IF_EnemyBehaviourPass.AttackInterface`
  (bind _arrow1 (`self.Arrow1`))
  (bind (_returnvalue_roll _returnvalue_pitch _returnvalue_yaw) (`KismetMathLibrary.BreakRotator` (`SceneComponent.K2_GetComponentRotation` (`self.Arrow1`))))
  ; Summon Projectiles
  (for _index (range (`KismetMathLibrary.RandomIntegerInRange` -4 -2) (+ (`KismetMathLibrary.RandomIntegerInRange` 2 4) 1))
    (`|SpawnActorFromClass` "/Game/AI/EnemyProjectiles/BossProjectiles/BP_LichFireBall.BP_LichFireBall_C" (`KismetMathLibrary.MakeTransform` (+ (`SceneComponent.K2_GetComponentLocation` _arrow1) (* (`SceneComponent.GetRightVector` _arrow1) (* _index 50))) (`KismetMathLibrary.MakeRotator` _returnvalue_roll _returnvalue_pitch (+ _returnvalue_yaw (* _index 10)))) "Undefined" "MultiplyWithRoot" null null)))

(event `/Game/Interfaces/IF_EnemyBehaviourPass.SummonPortals`
  (bind _returnvalue (`KismetMathLibrary.RandomIntegerInRange` -1 1))
  (bind _returnvalue_2 (`KismetMathLibrary.RandomIntegerInRange` -1 1))
  ; PortalAttack
  (for _array_element (`self.AllKnownPlayers`)
    (bind _returnvalue_3 (`self.K2_GetActorLocation` _array_element))
    (bind _returnvalue_4 (+ _returnvalue_3 (`KismetMathLibrary.MakeVector` (* (select `bool` (== _returnvalue 0) :`false` _returnvalue :`true` 1) (`KismetMathLibrary.RandomFloatInRange` -200.0 200.0)) (* (select `bool` (== _returnvalue_2 0) :`false` _returnvalue_2 :`true` 1) (`KismetMathLibrary.RandomFloatInRange` -200.0 200.0)) 100.0)))
    (`|SpawnActorFromClass` "/Game/AI/EnemyProjectiles/BossProjectiles/BP_Portals.BP_Portals_C" (`KismetMathLibrary.MakeTransform` _returnvalue_4 (`KismetMathLibrary.FindLookAtRotation` _returnvalue_4 _returnvalue_3)) "Undefined" "MultiplyWithRoot" null _array_element null)))

(fn `DecideTarget`
  (params (`TargetRanged?` :type Boolean))
  (returns (`Has Target?` :type Boolean) (Player :type "Actor Object Reference"))
  (locals (RangedPlayers :type "Map of Actor Object Reference to /Game/Blueprints/Data/E_AvailableWeaponTypes Enum") (MeleePlayers :type "Map of Actor Object Reference to /Game/Blueprints/Data/E_AvailableWeaponTypes Enum"))
  (bind _returnvalue (select `bool` `TargetRanged?` :`false` (`local.MeleePlayers`) :`true` (`local.RangedPlayers`)))
  (for _array_element (`self.AllKnownPlayers`)
    (bind _chosenweapons (message `/Game/Interfaces/IF_PlayerInfoPass.ChosenWeaponPass` _array_element))
    (if (or (`|EnumEquality` _chosenweapons "NewEnumerator1") (`|EnumEquality` _chosenweapons "NewEnumerator2"))
      (`BlueprintMapLibrary.Map_Add` (`local.RangedPlayers`) _array_element _chosenweapons)
      (else
        (`BlueprintMapLibrary.Map_Add` (`local.MeleePlayers`) _array_element _chosenweapons))))
  (if (`BlueprintMapLibrary.Map_IsEmpty` _returnvalue)
    (return true (`KismetArrayLibrary.Array_Random` (`self.AllKnownPlayers`)))
    (else
      (bind _values (`BlueprintMapLibrary.Map_Values` _returnvalue))
      (return true (`BlueprintMapLibrary.Map_GetKeyValueByIndex` _returnvalue (`.OutIndex` (`KismetArrayLibrary.Array_Random` _values)))))))

(fn `GetClosestPlayer`
  (params (`TargetRanged?` :type Boolean))
  (returns (ClosestPlayer :type "Actor Object Reference"))
  (locals (PlayersDistance :type "Map of Float (double-precision) to Actor Object Reference") (MeleePlayers :type "Array of Actor Object Reference") (RangedPlayers :type "Array of Actor Object Reference"))
  (for _array_element (`self.AllKnownPlayers`)
    (`BlueprintMapLibrary.Map_Add` (`local.PlayersDistance`) (`KismetMathLibrary.Conv_IntToDouble` (`KismetMathLibrary.Round` (`KismetMathLibrary.Vector_Distance` (`self.K2_GetActorLocation` _array_element) (`self.K2_GetActorLocation`)))) _array_element))
  (bind _keys (`BlueprintMapLibrary.Map_Keys` (`local.PlayersDistance`)))
  (bind (_value _returnvalue) (`BlueprintMapLibrary.Map_Find` (`local.PlayersDistance`) (`.MinValue` (`KismetMathLibrary.MinOfFloatArray` _keys))))
  (if _returnvalue
    (return _value)
    (else
      (return (`KismetArrayLibrary.Array_Random` (`self.AllKnownPlayers`))))))

(fn `UserConstructionScript`)