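; Enraged lich boss fireball projectile that explodes when destroyed; this Blueprint adds only the destruction behavior to its parent.
; On Destroyed it spawns a small Niagara fire explosion tinted to the point light's color.
; It then applies radial enemy-melee-type damage, effectively flat because base and minimum match, ignoring the instigator.
; A final sphere trace over the blast radius runs, but its results are unused.
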(event `self.ReceiveDestroyed`
  (bind _returnvalue (`self.K2_GetActorLocation`))
  (bind _array (`|MakeArray` (`self.GetInstigator`) :!type "Actor Object Reference"))
  (bind _returnvalue_2 (`NiagaraFunctionLibrary.SpawnSystemAtLocation` "/Game/VFX/NiagaraSystem/Fire/NS_FireExplosionSmall.NS_FireExplosionSmall" (`self.K2_GetActorLocation`)))
  (`NiagaraComponent.SetVariableLinearColor` _returnvalue_2 "FireColor" (`LightComponentBase.GetLightColor` (`self.PointLight`)))
  (`GameplayStatics.ApplyRadialDamageWithFalloff` 5.0 5.0 _returnvalue 100.0 200.0 2.5 "/Game/Blueprints/WeaponDamageTypes/BP_DamageType_EnemyMelee.BP_DamageType_EnemyMelee_C" _array null null)
  (`KismetSystemLibrary.SphereTraceSingleForObjects` _returnvalue _returnvalue 200.0 (`|MakeArray` "ObjectTypeQuery9" :!type "EObjectTypeQuery Enum") false _array))

(fn `UserConstructionScript`
  (`parent.UserConstructionScript`))