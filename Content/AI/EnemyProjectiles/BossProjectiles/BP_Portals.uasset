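; BP_Portals is a boss projectile portal that aims at a target actor and launches a lich fireball.
; On BeginPlay, a Timeline stretched to LifeTime turns the portal toward the target's location on every update.
; When the Timeline finishes, it spawns BP_LichFireBall with the portal's location and rotation.
; The construction script sets the actor's lifespan to the same LifeTime, so expiry coincides with the shot.
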(event `self.ReceiveBeginPlay`
  (`TimelineComponent.SetTimelineLength` (`self.Timeline`) (`self.LifeTime`))
  (`Timeline|Timeline` :!via `PlayFromStart`
    (:`Update`
      (`self.K2_SetActorRotation` (`KismetMathLibrary.FindLookAtRotation` (`self.K2_GetActorLocation`) (`self.K2_GetActorLocation` (`self.Target`)))))
    (:`Finished`
      (`|SpawnActorFromClass` "/Game/AI/EnemyProjectiles/BossProjectiles/BP_LichFireBall.BP_LichFireBall_C" (`KismetMathLibrary.MakeTransform` (`self.K2_GetActorLocation`) (`self.K2_GetActorRotation`)) "Undefined" "MultiplyWithRoot" null null))))

(fn `UserConstructionScript`
  (`self.SetLifeSpan` (`self.LifeTime`)))