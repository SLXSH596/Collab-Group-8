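; Boss projectile actor for the goat attack that deals damage on contact and explodes when it leaves play.
; An overlap on its sphere applies direct damage to the other actor, then destroys the projectile.
; EndPlay spawns the goat explosion Niagara effect slightly above its location and applies radial falloff damage that ignores the instigator.
; Both hits use the enemy melee damage type.
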(event `self.Sphere1.OnComponentBeginOverlap`
  (params (OverlappedComponent :type "PrimitiveComponent Object Reference") (OtherActor :type "Actor Object Reference") (OtherComp :type "PrimitiveComponent Object Reference") (OtherBodyIndex :type Integer) (bFromSweep :type Boolean) (SweepResult :type "HitResult Structure (by ref)"))
  (`GameplayStatics.ApplyDamage` OtherActor 10.0 null null "/Game/Blueprints/WeaponDamageTypes/BP_DamageType_EnemyMelee.BP_DamageType_EnemyMelee_C")
  (`self.K2_DestroyActor`))

(event `self.ReceiveDestroyed`)

(event `self.ReceiveEndPlay`
  (params (EndPlayReason :type "EEndPlayReason Enum" :default "Destroyed"))
  (bind _returnvalue (+ (`self.K2_GetActorLocation`) (0.0 0.0 15.0)))
  (`NiagaraFunctionLibrary.SpawnSystemAtLocation` "/Game/AI/TestAssets/CHimeraTest/NS_GoatExplosion.NS_GoatExplosion" _returnvalue)
  (`GameplayStatics.ApplyRadialDamageWithFalloff` 15.0 5.0 _returnvalue 50.0 190.0 1.0 "/Game/Blueprints/WeaponDamageTypes/BP_DamageType_EnemyMelee.BP_DamageType_EnemyMelee_C" (`|MakeArray` (`self.GetInstigator`) :!type "Actor Object Reference") null null))

(fn `UserConstructionScript`
  (`parent.UserConstructionScript`))