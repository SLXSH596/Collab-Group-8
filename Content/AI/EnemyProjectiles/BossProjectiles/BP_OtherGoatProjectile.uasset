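; Boss goat projectile that hurts what it touches and explodes when destroyed.
; Each bounce spawns a scream Niagara effect, and Sphere1 overlaps apply damage without destroying the projectile here.
; On destruction it deals small radial damage that ignores the instigator and spawns an explosion effect.
; A debug-drawn sphere trace also runs at that point, but its result is unused.
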(event `self.ReceiveBeginPlay`
  (add `ProjectileMovementComponent.OnProjectileBounce` (`self.ProjectileMovement`) (delegate `OnProjectileBounce_Event`)))

(event `OnProjectileBounce_Event`
  (params (ImpactResult :type "HitResult Structure (by ref)") (ImpactVelocity :type "Vector Structure (by ref)"))
  (bind _sphere (`self.Sphere`))
  (`NiagaraFunctionLibrary.SpawnSystemAtLocation` "/Game/AI/TestAssets/CHimeraTest/NS_GoatScreamBounce.NS_GoatScreamBounce" (`SceneComponent.K2_GetComponentLocation` _sphere) (`SceneComponent.K2_GetComponentRotation` _sphere)))

(event `self.Sphere1.OnComponentBeginOverlap`
  (params (OverlappedComponent :type "PrimitiveComponent Object Reference") (OtherActor :type "Actor Object Reference") (OtherComp :type "PrimitiveComponent Object Reference") (OtherBodyIndex :type Integer) (bFromSweep :type Boolean) (SweepResult :type "HitResult Structure (by ref)"))
  (`GameplayStatics.ApplyDamage` OtherActor 10.0 null null "/Game/Blueprints/WeaponDamageTypes/BP_DamageType_EnemyMelee.BP_DamageType_EnemyMelee_C"))

(event `self.ReceiveDestroyed`
  (bind _returnvalue (`self.K2_GetActorLocation`))
  (bind _array (`|MakeArray` (`self.GetInstigator`) :!type "Actor Object Reference"))
  (`GameplayStatics.ApplyRadialDamageWithFalloff` 5.0 5.0 _returnvalue 50.0 100.0 2.5 "/Game/Blueprints/WeaponDamageTypes/BP_DamageType_EnemyMelee.BP_DamageType_EnemyMelee_C" _array null null)
  (`KismetSystemLibrary.SphereTraceSingleForObjects` _returnvalue _returnvalue 100.0 (`|MakeArray` "ObjectTypeQuery9" :!type "EObjectTypeQuery Enum") false _array "ForDuration" true (struct :`R` 1.0 :`A` 1.0) (struct :`G` 1.0 :`A` 1.0) 2.0)
  (`NiagaraFunctionLibrary.SpawnSystemAtLocation` "/Game/AI/TestAssets/CHimeraTest/NS_GoatExplosion.NS_GoatExplosion" _returnvalue))

(fn `UserConstructionScript`
  (`parent.UserConstructionScript`))