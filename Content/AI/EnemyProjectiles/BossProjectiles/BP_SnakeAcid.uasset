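; BP_SnakeAcid is a boss acid projectile that bursts on overlap and spawns a small poison bomb.
; When Sphere1 overlaps any actor, it deals damage tagged as enemy melee, spawns a small explosion and a BP_PoisonBombSmall just above its location, then destroys itself.
; The reused Niagara fire explosion takes its FireColor from the projectile's PointLight color.
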(event `self.Sphere1.OnComponentBeginOverlap`
  (params (OverlappedComponent :type "PrimitiveComponent Object Reference") (OtherActor :type "Actor Object Reference") (OtherComp :type "PrimitiveComponent Object Reference") (OtherBodyIndex :type Integer) (bFromSweep :type Boolean) (SweepResult :type "HitResult Structure (by ref)"))
  (`GameplayStatics.ApplyDamage` OtherActor 10.0 null null "/Game/Blueprints/WeaponDamageTypes/BP_DamageType_EnemyMelee.BP_DamageType_EnemyMelee_C")
  (bind _returnvalue (`NiagaraFunctionLibrary.SpawnSystemAtLocation` "/Game/VFX/NiagaraSystem/Fire/NS_FireExplosionSmall.NS_FireExplosionSmall" (`self.K2_GetActorLocation`)))
  (`NiagaraComponent.SetVariableLinearColor` _returnvalue "FireColor" (`LightComponentBase.GetLightColor` (`self.PointLight`)))
  (`|SpawnActorFromClass` "/Game/Blueprints/Hazards/BP_PoisonBombSmall.BP_PoisonBombSmall_C" (`KismetMathLibrary.MakeTransform` (+ (`self.K2_GetActorLocation`) (0.0 0.0 5.0))) "Undefined" "MultiplyWithRoot" null null)
  (`self.K2_DestroyActor`))

(fn `UserConstructionScript`
  (`parent.UserConstructionScript`))