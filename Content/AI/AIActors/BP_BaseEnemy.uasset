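; Base enemy actor that chases, attacks and flees from players, taking its stats from a data table scaled by modifier multipliers.
; It feeds stats, health, target and flee state to the AI controller's Blackboard.
; An aggro sphere and incoming damage track players and pick chase targets, favouring the closest unless a modifier forces one.
; Components handle health, damage indication and montage-notified weapon attacks, with sounds and death effects.
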(event `self.ReceiveBeginPlay`
  (bind _ac_enemyhealthcomponent (`self.AC_EnemyHealthComponent`))
  ;[1 0.004025 0.7835] Initialise Enemy
  (bind _returnvalue (`|GetDataTableRow` "/Game/AI/AIActors/EnemyData/DT_EnemyStats.DT_EnemyStats" (`self.DataTableRow`))
    (:`then`
      (bind _output_get (set `self.EnemyData` _returnvalue))
      (set `/Game/Components/Player/AC_HealthComponent.MaxHealth` (* (`.Health_2_0B0470FD4315E09987AEB8A4D11DB9F9` (break `/Game/AI/AIActors/EnemyData/ST_EnemyStats` _output_get)) (`self.ModifierHealthMultiplier`)) _ac_enemyhealthcomponent)
      (`/Game/Components/Player/AC_HealthComponent.HealthCompInit` _ac_enemyhealthcomponent null)
      (`PrimitiveComponent.SetCollisionEnabled` (`self.AggroRangeSphere`) "NoCollision")
      (set `self.Weapon` (`self.GetComponentByClass` "/Game/Components/Weapons/AC_WeaponBase.AC_WeaponBase_C"))
      (`KismetSystemLibrary.DelayUntilNextTick`)
      (`self.Initialise`)
      ;[0.06301 0.6939 0.1441] Damage Indicator
      (`/Game/Components/Pawns/AC_DamageIndicator.Initiate` (`self.AC_DamageIndicator`) (`self.Mesh`) (`self.Mat Thickness`)))))

(event `self.ReceiveDestroyed`)

(event `Initialise`
  (bind (_health _damage _speed _attackrange _attackcooldown _knockback _fleethreshold _canflee _crit _avoidancerange _enemysound) (break `/Game/AI/AIActors/EnemyData/ST_EnemyStats` (`self.EnemyData`)))
  (bind _maxhealth (`/Game/Components/Player/AC_HealthComponent.MaxHealth` (`self.AC_EnemyHealthComponent`)))
  (bind _returnvalue (`AIBlueprintHelperLibrary.GetBlackboard` (`AIBlueprintHelperLibrary.GetAIController` self)))
  (bind _returnvalue_2 (`AIBlueprintHelperLibrary.GetBlackboard` (`AIBlueprintHelperLibrary.GetAIController` self)))
  ;[1 0.004025 0.7835] Enemy Initialiser
  (`PrimitiveComponent.SetCollisionEnabled` (`self.AggroRangeSphere`) "QueryOnly")
  (`/Engine/EditorBlueprintResources/StandardMacros.IsValid` _returnvalue_2
    (:`Is Valid`
      (`BlackboardComponent.SetValueAsFloat` _returnvalue_2 "MaxHealth" _maxhealth)
      (`BlackboardComponent.SetValueAsFloat` _returnvalue_2 "CurrentHealth" _maxhealth)
      (`BlackboardComponent.SetValueAsFloat` _returnvalue "Damage" (* _damage (`self.ModifierDamageMultiplier`)))
      (`BlackboardComponent.SetValueAsFloat` _returnvalue "AttackRange" _attackrange)
      (`BlackboardComponent.SetValueAsFloat` _returnvalue "AttackCooldownDuration" _attackcooldown)
      (`BlackboardComponent.SetValueAsFloat` _returnvalue "FleeHealthThreshold" _fleethreshold)
      (`BlackboardComponent.SetValueAsBool` _returnvalue "CanFlee" _canflee)
      (set `self.CanFlee` _canflee)
      (set `CharacterMovementComponent.MaxWalkSpeed` (* _speed (`self.ModifierSpeedMultiplier`)) (`self.CharacterMovement`))
      (set `self.EnemySound` _enemysound))))

(event `self.AggroRangeSphere.OnComponentBeginOverlap`
  (params (OverlappedComponent :type "PrimitiveComponent Object Reference") (OtherActor :type "Actor Object Reference") (OtherComp :type "PrimitiveComponent Object Reference") (OtherBodyIndex :type Integer) (bFromSweep :type Boolean) (SweepResult :type "HitResult Structure (by ref)"))
  ;[1 0.004025 0.7835] Triggers Enemy Agro and handles player data
  (bind _valid_player (`self.CheckPlayer` OtherActor))
  (if _valid_player
    (`self.SetPlayersInRange` OtherActor true :!label _label)
    (`self.SetChaseTarget` OtherActor)
    (`self.TriggerFlee`)
    (else
      (bind _valid_player_2 (`self.AddPlayer` OtherActor))
      (if _valid_player_2
        (goto _label)))))

(event `self.AggroRangeSphere.OnComponentEndOverlap`
  (params (OverlappedComponent :type "PrimitiveComponent Object Reference") (OtherActor :type "Actor Object Reference") (OtherComp :type "PrimitiveComponent Object Reference") (OtherBodyIndex :type Integer))
  ;[1 0.004025 0.7835] Triggers End Chase Sequence
  (bind _valid_player (`self.CheckPlayer` OtherActor))
  (if _valid_player
    (`self.SetPlayersInRange` OtherActor)
    (`self.EndChase` OtherActor)))

(event `SetChaseTarget`
  (params (Player :type "Actor Object Reference"))
  (bind _returnvalue (`AIBlueprintHelperLibrary.GetBlackboard` (`AIBlueprintHelperLibrary.GetAIController` self)))
  (bind _returnvalue_2 (`AIBlueprintHelperLibrary.GetBlackboard` (`AIBlueprintHelperLibrary.GetAIController` self)))
  ;[1 0.004025 0.7835] Handles Chase Behaviour
  (`/Engine/EditorBlueprintResources/StandardMacros.IsValid` _returnvalue_2
    (:`Is Valid`
      (if (`self.ModifierTargetPlayer`)
        (bind _continue (`self.ModifierCheck`))
        (if _continue
          (set `self.ChaseTarget` (`self.ModifierPlayerTarget`))
          (`BlackboardComponent.SetValueAsObject` _returnvalue "Player" (`self.ChaseTarget`) :!label _label_2)
          (`BlackboardComponent.SetValueAsBool` _returnvalue "CanSeePlayer" true))
        (elif (`BlackboardComponent.GetValueAsBool` _returnvalue_2 "CanSeePlayer")
          (bind _chase_target (`self.HandleChasePriority`))
          (set `self.ChaseTarget` _chase_target)
          (`/Engine/EditorBlueprintResources/StandardMacros.IsValid` _returnvalue :!label _label_3
            (:`Is Valid`
              (goto _label_2)))
          (elif true
            (set `self.ChaseTarget` Player)
            (goto _label_3)))))))

(event `EndChase`
  (params (Player :type "Actor Object Reference"))
  (bind _returnvalue (`AIBlueprintHelperLibrary.GetBlackboard` (`AIBlueprintHelperLibrary.GetAIController` self)))
  ;[1 0.004025 0.7835] Handles Ending Chase Behaviour
  (if (== Player (`self.ChaseTarget`))
    (if (> (`KismetArrayLibrary.Array_Length` (`self.PlayersInRange`)) 0)
      (`self.SetChaseTarget` (`|GetArrayItem` (`self.PlayersInRange`)))
      (else
        (`/Engine/EditorBlueprintResources/StandardMacros.IsValid` _returnvalue
          (:`Is Valid`
            (`BlackboardComponent.SetValueAsBool` _returnvalue "CanSeePlayer" false)))))))

(event `self.ReceiveAnyDamage`
  (params (Damage :type "Float (single-precision)") (DamageType :type "DamageType Object Reference") (InstigatedBy :type "Controller Object Reference") (DamageCauser :type "Actor Object Reference"))
  (bind _returnvalue (`AIBlueprintHelperLibrary.GetBlackboard` (`AIBlueprintHelperLibrary.GetAIController` self)))
  ;[1 0.004025 0.7835] Handles damage, and triggers agro
  (`/Game/Components/Player/AC_HealthComponent.TakeDamage` (`self.AC_EnemyHealthComponent`) self Damage DamageType InstigatedBy DamageCauser)
  (`/Engine/EditorBlueprintResources/StandardMacros.IsValid` _returnvalue
    (:`Is Valid`
      (`self.PlayHitSound` DamageCauser)
      (`BlackboardComponent.SetValueAsFloat` _returnvalue "CurrentHealth" (`/Game/Components/Player/AC_HealthComponent.CurrentHealth` (`self.AC_EnemyHealthComponent`)))
      (if (`KismetArrayLibrary.Array_Contains` (`self.PlayersInRange`) DamageCauser)
        (`self.TriggerFlee` :!label _label_4)
        (else
          (bind _valid_player (`self.CheckPlayer` DamageCauser))
          (if _valid_player
            (`self.SetPlayersInRange` DamageCauser true :!label _label_5)
            (`self.SetChaseTarget` DamageCauser)
            (goto _label_4)
            (else
              (bind _valid_player_2 (`self.AddPlayer` DamageCauser))
              (if _valid_player_2
                (goto _label_5)))))))))

(event `self.AC_EnemyHealthComponent.OnDeath`
  ;[1 0.004025 0.7835] Death Trigger
  (`self.OnEnemyDeath` self)
  (bind _returnvalue (`GameplayStatics.SpawnSoundAtLocation` (`self.EnemySound`) (`self.K2_GetActorLocation`) (struct) 1.0 1.0 0.0 null null))
  (`AudioParameterControllerInterface.SetIntParameter` _returnvalue "None" 0)
  (`self.HandleDeath`)
  (`self.K2_DestroyActor`))

(event `/Game/Interfaces/BPI_BaseEnemyInterface.ToggleCooldown`
  (params (`Blackboard Name` :type Name) (Cooldown :type "Float (double-precision)"))
  (bind _returnvalue (`AIBlueprintHelperLibrary.GetBlackboard` (`AIBlueprintHelperLibrary.GetAIController` self)))
  ;[1 0.004025 0.7835] Toggle Enemy Cooldowns
  (`KismetSystemLibrary.Delay` Cooldown)
  (`/Engine/EditorBlueprintResources/StandardMacros.IsValid` _returnvalue
    (:`Is Valid`
      (`BlackboardComponent.SetValueAsBool` _returnvalue (`KismetSystemLibrary.MakeLiteralName` `Blackboard Name`) false))))

(event `/Game/Interfaces/BPI_BaseEnemyInterface.ChangeFocus`
  (params (`Set Focus` :type Boolean) (`Focus Target` :type "Actor Object Reference"))
  (bind _returnvalue (`AIBlueprintHelperLibrary.GetAIController` self))
  ;[1 0.004025 0.7835] Set Enemy Focus
  (if `Set Focus`
    (`AIController.K2_SetFocus` _returnvalue `Focus Target`)
    (else
      (`AIController.K2_ClearFocus` _returnvalue))))

(event `ChangeModiferPlayerTarget`
  (params (Player :type "Actor Object Reference"))
  ;[1 0.004025 0.7835] Modifier Event to swap player targets
  (set `self.ModifierPlayerTarget` Player)
  (`self.EndChase` (`self.ChaseTarget`)))

(event `EnemyAgroActive`
  (params (Target :type "Actor Object Reference"))
  (set `self.ModifierPlayerTarget` Target)
  (set `self.ModifierTargetPlayer` true))

(event `/Game/Interfaces/BPI_BaseEnemyInterface.TriggerAttack`
  (params (Damage :type "Float (double-precision)"))
  (bind _weapon (`self.Weapon`))
  (bind _attackmontage (`self.AttackMontage`))
  ;[1 0.004025 0.7835] Triggers Enemy Attack
  (`/Engine/EditorBlueprintResources/StandardMacros.IsValid` _weapon
    (:`Is Valid`
      (set `/Game/Components/Weapons/AC_WeaponBase.BaseDamage` Damage _weapon)
      ;;[0.162 0.02956 0.3515] Play Montage if valid before attack, else just do the attack - MONTAGE MUST HAVE NOTIFY
      (`/Engine/EditorBlueprintResources/StandardMacros.IsValid` _attackmontage
        (:`Is Valid`
          (`|PlayMontage` (`self.Mesh`) _attackmontage
            (:`OnNotifyBegin`
              _)))
        (:`Is Not Valid`
          _))
      (`/Game/Components/Weapons/AC_WeaponBase.LightAttack` _weapon)
      (bind _returnvalue (`GameplayStatics.SpawnSoundAtLocation` (`self.EnemySound`) (`self.K2_GetActorLocation`) (struct) 1.0 1.0 0.0 null null))
      (`AudioParameterControllerInterface.SetIntParameter` _returnvalue "None" 1))))

(event `/Game/Interfaces/BPI_BaseEnemyInterface.UpdateSpeed`
  (params (SpeedMultiplier :type "Float (double-precision)"))
  ;[1 0.004025 0.7835] Interface call to Modify Enemy Speed
  (set `CharacterMovementComponent.MaxWalkSpeed` (* SpeedMultiplier (* (`self.ModifierSpeedMultiplier`) (`.Speed_26_20A1A289426ADCF5F49BF29B32BDB475` (break `/Game/AI/AIActors/EnemyData/ST_EnemyStats` (`self.EnemyData`))))) (`self.CharacterMovement`)))

(event `/Game/Interfaces/BPI_BaseEnemyInterface.StopChase`
  (`self.EndChase` (`self.ChaseTarget`)))

(event `/Game/Interfaces/BPI_BaseEnemyInterface.PlayMovementAudio`)

(fn `AddPlayer`
  (params (Player :type "Actor Object Reference"))
  (returns (`Valid Player` :type Boolean))
  ;[1 0.004025 0.7835] Adds a player to the array if the enemy has not yet seen all players
  (if (== (`KismetArrayLibrary.Array_Length` (`self.Players`)) (`self.maxNumberOfPlayers`))
    (return false)
    (elif (`.bSuccess` (cast `/Game/Blueprints/Player/BP_Player` Player :!pure true))
      (`KismetArrayLibrary.Array_Add` (`self.Players`) Player)
      (return true)
      (else
        (return false)))))

(fn `CheckPlayer`
  (params (Player :type "Actor Object Reference"))
  (returns (`Valid Player` :type Boolean))
  ;[1 0.004025 0.7835] Checks if the enemy has seen the player
  (return (`KismetArrayLibrary.Array_Contains` (`self.Players`) Player)))

(fn `GetClosestPlayer`
  (returns (Actor :type "Actor Object Reference"))
  (bind _chase_target (`self.HandleChasePriority`))
  (return _chase_target))

(fn `GetFleeLocation`
  (params (Player :type "Actor Object Reference"))
  (returns (MultiplePlayersInRange :type Boolean) (FleeTarget :type "Vector Structure"))
  (locals (MidPointVector :type "Vector Structure"))
  (bind _players (`self.Players`))
  ;[1 0.004025 0.7835] Calculates Flee Location
  (if (not (> (`KismetArrayLibrary.Array_Length` (`self.Players`)) 1))
    (return false (`self.K2_GetActorLocation` Player))
    (else
      ;;[1 0.004025 0.7835] Calculates Central Point to flee from
      (for _array_element _players
        (set `local.MidPointVector` (+ (`local.MidPointVector`) (`self.K2_GetActorLocation` _array_element))))
      (return true (/ (`local.MidPointVector`) (`KismetArrayLibrary.Array_Length` _players))))))

(fn `HandleChasePriority`
  (returns (`Chase Target` :type "Actor Object Reference"))
  (locals (ClosestDistance :type "Float (double-precision)") (`Closest Player` :type "Actor Object Reference"))
  ;[1 0.004025 0.7835] Selects a Player to target
  (set `local.ClosestDistance` 5000.0)
  (for _array_element (`self.PlayersInRange`)
    (bind _returnvalue (`self.GetDistanceTo` _array_element self))
    (if (< _returnvalue (`local.ClosestDistance`))
      (set `local.Closest Player` _array_element)
      (set `local.ClosestDistance` _returnvalue)))
  (return (`local.Closest Player`)))

(fn `HandleDeath`
  (bind _returnvalue (`NiagaraFunctionLibrary.SpawnSystemAtLocation` "/Game/VFX/NiagaraSystem/Fire/NS_FireExplosionSmall.NS_FireExplosionSmall" (`SceneComponent.K2_GetComponentLocation` (`self.AggroRangeSphere`))))
  (`NiagaraComponent.SetVariableLinearColor` _returnvalue "FireColor" (`self.DeathColor`))
  (bind _returnvalue_2 (`GameplayStatics.SpawnSoundAtLocation` "/Game/Audio/MetaSounds/SFX/MS_Campfire.MS_Campfire" (`self.K2_GetActorLocation`) (struct) 1.0 1.0 0.0 null null))
  (`AudioParameterControllerInterface.SetIntParameter` _returnvalue_2 "Type" 2))

(fn `ModifierCheck`
  (returns (Continue :type Boolean))
  (for _array_element (`self.PlayersInRange`)
    (if (== _array_element (`self.ModifierPlayerTarget`))
      (return true)))
  (return false))

(fn `PlayHitSound`
  (params (Instigator :type "Actor Object Reference"))
  (bind _chosenweapons (message `/Game/Interfaces/BPI_PlayerInfoPass.ChosenWeaponPass` Instigator))
  (switch `/Game/Blueprints/Data/E_AvailableWeaponTypes` _chosenweapons
    (:`NewEnumerator0`
      (set `self.HitSfxIndex` 3))
    (:`NewEnumerator2`
      (set `self.HitSfxIndex` 2)))
  (bind _returnvalue (`GameplayStatics.SpawnSoundAtLocation` (`self.EnemySound`) (`self.K2_GetActorLocation`) (struct) 1.0 1.0 0.0 null null))
  (`AudioParameterControllerInterface.SetIntParameter` _returnvalue "None" (`self.HitSfxIndex`))
  (return))

(fn `SetPlayersInRange`
  (params (Player :type "Actor Object Reference") (EnterRange :type Boolean))
  (bind _playersinrange (`self.PlayersInRange`))
  ;[1 0.004025 0.7835] Adds and remove players in agro range
  (if EnterRange
    (`KismetArrayLibrary.Array_AddUnique` _playersinrange Player)
    (else
      (`KismetArrayLibrary.Array_RemoveItem` _playersinrange Player)))
  (return))

(fn `TriggerFlee`
  (returns (Running :type Boolean))
  (bind _ac_enemyhealthcomponent (`self.AC_EnemyHealthComponent`))
  ;[1 0.004025 0.7835] Checks conditions to see if enemy should run away
  (if (and (`self.CanFlee`) (<= (/ (`/Game/Components/Player/AC_HealthComponent.CurrentHealth` _ac_enemyhealthcomponent) (`/Game/Components/Player/AC_HealthComponent.MaxHealth` _ac_enemyhealthcomponent)) (`BlackboardComponent.GetValueAsFloat` (`AIBlueprintHelperLibrary.GetBlackboard` (`AIBlueprintHelperLibrary.GetAIController` self)) "FleeHealthThreshold")))
    (`BlackboardComponent.SetValueAsBool` (`AIBlueprintHelperLibrary.GetBlackboard` null) "Fleeing" true)
    (return true)
    (else
      (return false))))

(fn `UserConstructionScript`)