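; AI-controlled tail part of the Chimera enemy that runs the BT_ChimeraParts behavior tree when possessed.
; An overlap volume toggles the HasBeenAlerted blackboard key, and attack calls send a secondary attack message to the instigator.
; SecondaryProjSpawn deals enemy melee damage through a debug-drawn sphere trace around the Tail, rather than spawning a projectile.
; Targeting functions are stubs, and a timed grab-and-release sequence is left unconnected.
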(event `self.ReceivePossessed`
  (params (NewController :type "Controller Object Reference"))
  (`AIController.RunBehaviorTree` (`AIBlueprintHelperLibrary.GetAIController` self) "/Game/AI/BehaviourTree/BT_ChimeraParts.BT_ChimeraParts"))

(event `/Game/Interfaces/BPI_EnemyBehaviourPass.SecondaryProjSpawn`
  (bind _returnvalue (`SceneComponent.K2_GetComponentLocation` (`self.Tail`)))
  (bind _outhits (`KismetSystemLibrary.SphereTraceMultiForObjects` :`Start` _returnvalue :`End` _returnvalue :`Radius` 200.0 :`ObjectTypes` (`|MakeArray` "ObjectTypeQuery9" :!type "EObjectTypeQuery Enum") :`DrawDebugType` "ForDuration"))
  (for _array_element _outhits
    (`GameplayStatics.ApplyDamage` (`.HitActor` (`GameplayStatics.BreakHitResult` _array_element)) 5.0 null null "/Game/Blueprints/WeaponDamageTypes/BP_DamageType_EnemyMelee.BP_DamageType_EnemyMelee_C")))

(event `/Game/Interfaces/BPI_EnemyBehaviourPass.AttackInterface`
  (message `/Game/Interfaces/BPI_EnemyBehaviourPass.SecondaryAttack` (`self.GetInstigator`)))

(event `self.HasBeenAlerted?.OnComponentBeginOverlap`
  (params (OverlappedComponent :type "PrimitiveComponent Object Reference") (OtherActor :type "Actor Object Reference") (OtherComp :type "PrimitiveComponent Object Reference") (OtherBodyIndex :type Integer) (bFromSweep :type Boolean) (SweepResult :type "HitResult Structure (by ref)"))
  (`BlackboardComponent.SetValueAsBool` (`AIBlueprintHelperLibrary.GetBlackboard` null) "HasBeenAlerted" true)
  (`KismetSystemLibrary.PrintString` "WOW"))

(event `self.HasBeenAlerted?.OnComponentEndOverlap`
  (params (OverlappedComponent :type "PrimitiveComponent Object Reference") (OtherActor :type "Actor Object Reference") (OtherComp :type "PrimitiveComponent Object Reference") (OtherBodyIndex :type Integer))
  (`BlackboardComponent.SetValueAsBool` (`AIBlueprintHelperLibrary.GetBlackboard` null) "HasBeenAlerted" false))

(fn `DecideTarget`
  (params (`TargetRanged?` :type Boolean))
  (returns (`Has Target?` :type Boolean) (Player :type "Actor Object Reference"))
  (return false null))

(fn `GetClosestPlayer`
  (params (`TargetRanged?` :type Boolean))
  (returns (ClosestPlayer :type "Actor Object Reference"))
  (return null))

(fn `UserConstructionScript`)