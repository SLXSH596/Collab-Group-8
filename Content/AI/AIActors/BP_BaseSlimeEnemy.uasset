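; BP_BaseSlimeEnemy is the base Blueprint for slime enemies, extending a parent AI enemy with slime-specific death audio and flee behavior.
; On BeginPlay it binds to the enemy death event, spawning the slime MetaSound at its location and setting its State parameter.
; Initialise gives each slime a small random chance to flee, writing the CanFlee flag to the Blackboard for AI use.
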(event `self.ReceiveBeginPlay`
  (`parent.ReceiveBeginPlay`)
  (add `self.OnEnemyDeath` (delegate `Slime Death`)))

(event `Slime Death` :!signature `self.OnEnemyDeath`
  (params (`Enemy Character` :type "/Game/AI/AIActors/BP_BaseEnemy Object Reference"))
  (bind _returnvalue (`GameplayStatics.SpawnSoundAtLocation` "/Game/Audio/MetaSounds/Enemies/MS_Enemy_Slime.MS_Enemy_Slime" (`self.K2_GetActorLocation`) (struct) 1.0 1.0 0.0 null null))
  (`AudioParameterControllerInterface.SetIntParameter` _returnvalue "State" 0))

(event `self.Initialise`
  (`parent.Initialise`)
  (if (< (`KismetMathLibrary.RandomFloat`) 0.1)
    (bind _output_get (set `self.CanFlee` true))
    (`BlackboardComponent.SetValueAsBool` (`AIBlueprintHelperLibrary.GetBlackboard` null) "CanFlee" _output_get)))

(fn `UserConstructionScript`
  (`parent.UserConstructionScript`))