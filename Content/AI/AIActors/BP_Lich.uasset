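; Lich boss enemy whose max health scales with the number of joined players.
; Montage-driven attacks include a dash, a staff swing, a fireball fan and portals spawned at random offsets around each known player.
; The slam deals falloff radial damage at the staff socket, shakes the camera and launches nearby characters upward by distance.
; An Enraged state swaps the fireball class and adds extra portals.
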(event `self.ReceiveBeginPlay`
  (bind _ac_enemyhealthcomponent (`self.AC_EnemyHealthComponent`))
  (`parent.ReceiveBeginPlay`)
  (set `/Game/Components/Player/AC_HealthComponent.MaxHealth` (* (* (`/Game/Components/Player/AC_HealthComponent.MaxHealth` _ac_enemyhealthcomponent) (`/Game/Blueprints/GI_GameInstance.CurrentJoinCount` (cast `/Game/Blueprints/GI_GameInstance` (`GameplayStatics.GetGameInstance`) :!pure true))) 0.75) _ac_enemyhealthcomponent))

(event `/Game/Interfaces/BPI_EnemyBehaviourPass.DashAttack`
  ; DashAttack#
  (bind _returnvalue (`GameplayStatics.SpawnSoundAtLocation` "/Game/Audio/MetaSounds/Enemies/MS_Boss_Lich_Vocals.MS_Boss_Lich_Vocals" (`self.K2_GetActorLocation`) (struct) 1.0 1.0 0.0 null null))
  (`AudioParameterControllerInterface.SetIntParameter` _returnvalue "State" 0)
  (`|PlayMontage` (`self.Mesh`) "/Game/Animation/AnimMontages/AM_LichDashAttack.AM_LichDashAttack"
    (:`OnCompleted`
      _)
    (:`OnBlendOut`
      _))
  (message `/Game/Interfaces/BPI_EnemyBehaviourPass.UpdateAnimations` self false))

(event `/Game/Interfaces/BPI_EnemyBehaviourPass.SlamDamageSpawn`
  (bind _returnvalue (`SceneComponent.GetSocketLocation` (`self.Mesh`) "StaffSocket"))
  ; DashAttack#
  (`NiagaraFunctionLibrary.SpawnSystemAtLocation` "/Game/VFX/NiagaraSystem/NS_Shockwave1.NS_Shockwave1" (`SceneComponent.GetSocketLocation` (`self.Mesh`) "StaffSocket") (struct) (2.0 2.0 2.0))
  (bind _returnvalue_2 (`GameplayStatics.SpawnSoundAtLocation` "/Game/Audio/MetaSounds/SFX/MS_Magic_Impacts.MS_Magic_Impacts" (`SceneComponent.GetSocketLocation` (`self.Mesh`) "StaffSocket") (struct) 1.0 1.0 0.0 null null))
  (`AudioParameterControllerInterface.SetIntParameter` _returnvalue_2 "State" 1)
  (`GameplayStatics.ApplyRadialDamageWithFalloff` 40.0 15.0 (`SceneComponent.GetSocketLocation` (`self.Mesh`) "StaffSocket") 100.0 300.0 2.0 "/Game/Blueprints/WeaponDamageTypes/BP_DamageType_EnemyMelee.BP_DamageType_EnemyMelee_C" (`|MakeArray` self :!type "Actor Object Reference") self null "ECC_WorldStatic")
  (`LegacyCameraShake.StartLegacyCameraShake` (`GameplayStatics.GetPlayerCameraManager` 0) "/Game/AI/BP_BossCameraShake.BP_BossCameraShake_C")
  (bind (_outhits _returnvalue_3) (`KismetSystemLibrary.SphereTraceMultiForObjects` _returnvalue _returnvalue 350.0 (`|MakeArray` "ObjectTypeQuery3" :!type "EObjectTypeQuery Enum")))
  (if _returnvalue_3
    (for _array_element _outhits
      (bind (_bblockinghit _binitialoverlap _time _distance _location _impactpoint _normal _impactnormal _physmat _hitactor _hitcomponent _hitbonename _bonename _hititem _elementindex _faceindex _tracestart) (`GameplayStatics.BreakHitResult` _array_element))
      (bind _ascharacter (cast `Character` _hitactor))
      (bind _returnvalue_4 (`KismetMathLibrary.Vector_Distance` _impactpoint _tracestart))
      (`self.LaunchCharacter` _ascharacter (`KismetMathLibrary.MakeVector` 0.0 0.0 (* (`KismetMathLibrary.SelectFloat` 0.5 (`KismetMathLibrary.SelectFloat` 0.8 1.0 (> _returnvalue_4 100.0)) (> _returnvalue_4 200.0)) 1000.0)) false true))))

(event `/Game/Interfaces/BPI_EnemyBehaviourPass.AttackInterface`
  ; DashAttack#
  (`|PlayMontage` (`self.Mesh`) "/Game/Animation/AnimMontages/AM_LichSwingAttack.AM_LichSwingAttack"
    (:`then`
      (bind _returnvalue (`GameplayStatics.SpawnSoundAtLocation` "/Game/Audio/MetaSounds/Weapons/MS_Staff.MS_Staff" (`self.K2_GetActorLocation`) (struct) 1.0 1.0 0.0 null null))
      (`AudioParameterControllerInterface.SetIntParameter` _returnvalue "State" 2))))

(event `/Game/Interfaces/BPI_EnemyBehaviourPass.ProjectileSpawn`
  (bind _arrow1 (`self.Arrow1`))
  (bind (_returnvalue_roll _returnvalue_pitch _returnvalue_yaw) (`KismetMathLibrary.BreakRotator` (`SceneComponent.K2_GetComponentRotation` (`self.Arrow1`))))
  (bind _returnvalue (select `bool` (`self.Enraged?`) :`false` 3 :`true` 2))
  ; Summon Projectiles
  (for _index (range (* _returnvalue -1) (+ _returnvalue 1))
    (`|SpawnActorFromClass` (select `bool` (`self.Enraged?`) :`false` "/Game/AI/EnemyProjectiles/BossProjectiles/BP_LichFireBall.BP_LichFireBall_C" :`true` "/Game/AI/EnemyProjectiles/BossProjectiles/BP_LichFireBallEnraged.BP_LichFireBallEnraged_C" :!type "Actor Class Reference") (`KismetMathLibrary.MakeTransform` (+ (`SceneComponent.K2_GetComponentLocation` _arrow1) (* (`SceneComponent.GetRightVector` _arrow1) (* _index 50))) (`KismetMathLibrary.MakeRotator` _returnvalue_roll _returnvalue_pitch (+ _returnvalue_yaw (* _index 10)))) "Undefined" "MultiplyWithRoot" null null)))

(event `/Game/Interfaces/BPI_EnemyBehaviourPass.SecondaryProjSpawn`
  (bind _returnvalue (`KismetMathLibrary.RandomIntegerInRange` -1 1))
  (bind _returnvalue_2 (`KismetMathLibrary.RandomIntegerInRange` -1 1))
  ; PortalAttack
  (for _array_element (`self.AllKnownPlayers`)
    (bind _returnvalue_3 (`self.K2_GetActorLocation` _array_element))
    (bind _returnvalue_4 (+ _returnvalue_3 (`KismetMathLibrary.MakeVector` (* (select `bool` (== _returnvalue 0) :`false` _returnvalue :`true` 1) (`KismetMathLibrary.RandomFloatInRange` -300.0 300.0)) (* (select `bool` (== _returnvalue_2 0) :`false` _returnvalue_2 :`true` 1) (`KismetMathLibrary.RandomFloatInRange` -300.0 300.0)) 155.0)))
    (bind _returnvalue_5 (`GameplayStatics.SpawnSoundAtLocation` "/Game/Audio/MetaSounds/Enemies/MS_Boss_Lich.MS_Boss_Lich" _returnvalue_4 (struct) 1.0 1.0 0.0 null null))
    (`AudioParameterControllerInterface.SetIntParameter` _returnvalue_5 "State" 1)
    (bind _returnvalue_6 (`KismetMathLibrary.FindLookAtRotation` _returnvalue_4 _returnvalue_3))
    (`|SpawnActorFromClass` "/Game/AI/EnemyProjectiles/BossProjectiles/BP_Portals.BP_Portals_C" (`KismetMathLibrary.MakeTransform` _returnvalue_4 _returnvalue_6) "Undefined" "MultiplyWithRoot" null _array_element (`KismetMathLibrary.SelectFloat` 0.5 0.7 (`self.Enraged?`)) null)
    (if (`self.Enraged?`)
      (`|SpawnActorFromClass` "/Game/AI/EnemyProjectiles/BossProjectiles/BP_Portals.BP_Portals_C" (`KismetMathLibrary.MakeTransform` _returnvalue_4 _returnvalue_6) "Undefined" "MultiplyWithRoot" null _array_element 0.5 null)
      (bind _returnvalue_7 (`GameplayStatics.SpawnSoundAtLocation` "/Game/Audio/MetaSounds/Enemies/MS_Boss_Lich.MS_Boss_Lich" _returnvalue_4 (struct) 1.0 1.0 0.0 null null))
      (`AudioParameterControllerInterface.SetIntParameter` _returnvalue_7 "State" 1))))

(event `/Game/Interfaces/BPI_EnemyBehaviourPass.SecondaryAttack`
  ; PortalAttack
  (`|PlayMontage` (`self.Mesh`) "/Game/Animation/AnimMontages/AM_LichPortalAttack.AM_LichPortalAttack"))

(event `/Game/Interfaces/BPI_EnemyBehaviourPass.UpdateAnimations`
  (params (`Charging?` :type Boolean))
  (bind _returnvalue (`SkeletalMeshComponent.GetAnimInstance` (`self.Mesh`)))
  ; UpdateANimation
  (message `/Game/Interfaces/BPI_EnemyBehaviourPass.UpdateAnimations` _returnvalue `Charging?`)
  (`self.StopAnimMontage` (`AnimInstance.GetCurrentActiveMontage` _returnvalue)))

(fn `UserConstructionScript`
  (`parent.UserConstructionScript`))