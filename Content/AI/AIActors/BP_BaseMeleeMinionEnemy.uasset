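; Base melee minion enemy that attaches itself to a leader enemy through its AI Blackboard.
; Overlaps on LeaderDetectionRange query the other actor with LeaderCheckMessage, and a positive reply calls SetLeader.
; A DoOnce keeps the first leader found, writing LeaderEnemy and FoundLeader to the Blackboard.
; LeaderDead clears FoundLeader and resets the DoOnce when the dead leader matches, so a later overlap can assign another.
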(event `self.LeaderDetectionRange.OnComponentBeginOverlap`
  (params (OverlappedComponent :type "PrimitiveComponent Object Reference") (OtherActor :type "Actor Object Reference") (OtherComp :type "PrimitiveComponent Object Reference") (OtherBodyIndex :type Integer) (bFromSweep :type Boolean) (SweepResult :type "HitResult Structure (by ref)"))
  ;[1 0.004025 0.7835] Sets Leader if in range
  (bind _valid (message `/Game/Interfaces/IF_MeleeLeader.LeaderCheck` OtherActor))
  (if _valid
    (`self.SetLeader` OtherActor)))

(event `/Game/Interfaces/IF_MeleeMinion.SetLeader`
  (params (Leader :type "Actor Object Reference"))
  (bind _returnvalue (`AIBlueprintHelperLibrary.GetBlackboard` null))
  ;[1 0.004025 0.7835] Sets leader variables in BT
  (`/Engine/EditorBlueprintResources/StandardMacros.DoOnce` false :!label _label
    (:`Completed`
      (`BlackboardComponent.SetValueAsObject` _returnvalue "LeaderEnemy" Leader)
      (`BlackboardComponent.SetValueAsBool` _returnvalue "FoundLeader" true))))

(event `/Game/Interfaces/IF_MeleeMinion.LeaderDead`
  (params (Leader :type "Actor Object Reference"))
  (if (== Leader (`BlackboardComponent.GetValueAsObject` (`AIBlueprintHelperLibrary.GetBlackboard` null) "LeaderEnemy"))
    (`BlackboardComponent.SetValueAsBool` (`AIBlueprintHelperLibrary.GetBlackboard` null) "FoundLeader" false)
    (goto _label :!via `Reset`)))

(fn `UserConstructionScript`
  (`parent.UserConstructionScript`))