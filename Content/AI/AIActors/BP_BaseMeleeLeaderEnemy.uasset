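; Melee leader enemy that keeps track of its minions and notifies them when it dies.
; LeaderCheck adds the calling minion to the Minions array without duplicates and always returns true.
; HandleDeath runs the parent death logic, then sends LeaderDeadMessage with itself to every still-valid minion.
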(fn `HandleDeath`
  (`parent.HandleDeath`)
  (for _array_element (`self.Minions`)
    (`/Engine/EditorBlueprintResources/StandardMacros.IsValid` _array_element
      (:`Is Valid`
        (message `/Game/Interfaces/BPI_MeleeMinion.LeaderDead` _array_element self))))
  (return))

(fn `LeaderCheck`
  (params (Minion :type "Actor Object Reference"))
  (returns (Valid :type Boolean))
  (`KismetArrayLibrary.Array_AddUnique` (`self.Minions`) Minion)
  (return true))

(fn `UserConstructionScript`
  (`parent.UserConstructionScript`))