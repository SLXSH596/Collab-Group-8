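; Base goblin enemy character Blueprint that adds secondary physics and a death sound to its parent enemy class.
; On BeginPlay it enables physics simulation on the mesh bodies below the Tail and Head bones, excluding those bones themselves.
; It also binds to the enemy death event, which spawns the goblin MetaSound at the actor's location and sets its State parameter to select the sound.
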(event `self.ReceiveBeginPlay`
  (bind _mesh (`self.Mesh`))
  (`parent.ReceiveBeginPlay`)
  (`SkeletalMeshComponent.SetAllBodiesBelowSimulatePhysics` _mesh "Tail" true false)
  (`SkeletalMeshComponent.SetAllBodiesBelowSimulatePhysics` _mesh "Head" true false)
  (add `self.OnEnemyDeath` (delegate `Goblin Death`)))

(event `Goblin Death` :!signature `self.OnEnemyDeath`
  (params (`Enemy Character` :type "/Game/AI/AIActors/BP_BaseEnemy Object Reference"))
  (bind _returnvalue (`GameplayStatics.SpawnSoundAtLocation` "/Game/Audio/MetaSounds/Enemies/MS_Enemy_Goblin.MS_Enemy_Goblin" (`self.K2_GetActorLocation`) (struct) 1.0 1.0 0.0 null null))
  (`AudioParameterControllerInterface.SetIntParameter` _returnvalue "State" 1))

(fn `UserConstructionScript`
  (`parent.UserConstructionScript`))