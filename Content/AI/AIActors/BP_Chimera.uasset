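; BP_Chimera is an AI enemy actor that assembles a multi-part creature and provides a tail melee attack.
; On BeginPlay it runs parent logic, then spawns separate BP_ChimeraTail and BP_ChimeraBody actors, attached to its Tail and SnakeHead components respectively.
; SecondaryAttack sphere-traces a short distance forward from the Tail and applies enemy melee damage to every Pawn hit.
; DashAttack and AttackInterface events are empty.
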(event `self.ReceiveBeginPlay`
  (bind _tail (`self.Tail`))
  (bind _snakehead (`self.SnakeHead`))
  (`parent.ReceiveBeginPlay`)
  (bind _returnvalue (`|SpawnActorFromClass` "/Game/AI/AIActors/BP_ChimeraTail.BP_ChimeraTail_C" (`KismetMathLibrary.MakeTransform` (`SceneComponent.K2_GetComponentLocation` _tail) (`SceneComponent.K2_GetComponentRotation` _tail)) "Undefined" "MultiplyWithRoot" null null))
  (`self.K2_AttachToComponent` _returnvalue (`self.Tail`) "None" "SnapToTarget" "SnapToTarget" "KeepWorld" true)
  (bind _returnvalue_2 (`|SpawnActorFromClass` "/Game/AI/AIActors/BP_ChimeraBody.BP_ChimeraBody_C" (`KismetMathLibrary.MakeTransform` (`SceneComponent.K2_GetComponentLocation` _snakehead) (`SceneComponent.K2_GetComponentRotation` _snakehead)) "Undefined" "MultiplyWithRoot" null null))
  (`self.K2_AttachToComponent` _returnvalue_2 (`self.SnakeHead`) "None" "SnapToTarget" "SnapToTarget" "KeepWorld" true))

(event `/Game/Interfaces/IF_EnemyBehaviourPass.SecondaryAttack`
  (bind _tail (`self.Tail`))
  (bind _returnvalue (`SceneComponent.K2_GetComponentLocation` _tail))
  (bind _outhits (`KismetSystemLibrary.SphereTraceMultiForObjects` _returnvalue (+ _returnvalue (* (`SceneComponent.GetForwardVector` _tail) 100.0)) 50.0 (`|MakeArray` "ObjectTypeQuery3" :!type "EObjectTypeQuery Enum")))
  (for _array_element _outhits
    (`GameplayStatics.ApplyDamage` (`.HitActor` (`GameplayStatics.BreakHitResult` _array_element)) 5.0 null null "/Game/Blueprints/WeaponDamageTypes/BP_DamageType_EnemyMelee.BP_DamageType_EnemyMelee_C")))

(event `/Game/Interfaces/IF_EnemyBehaviourPass.DashAttack`)

(event `/Game/Interfaces/IF_EnemyBehaviourPass.AttackInterface`)

(fn `UserConstructionScript`
  (`parent.UserConstructionScript`))