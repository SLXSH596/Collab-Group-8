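; Basic AI enemy that chases the player on sight or when damaged by them, feeding its state to a Behavior Tree through the Blackboard.
; PawnSensing and damage events set the player as chase target, updating Blackboard target and visibility keys.
; A health component processes damage; health is mirrored to the Blackboard, and the actor is destroyed at zero.
; A delayed event clears the attack cooldown for a task; the CheckPlayer range check is unused.
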(event `Toggle Attack Cooldown`
  (params (Cooldown :type "Float (double-precision)"))
  (bind _returnvalue (`AIBlueprintHelperLibrary.GetBlackboard` (`AIBlueprintHelperLibrary.GetAIController` self)))
  ;[1 0.004025 0.7835] Sets Attack Cooldown - Called from toggle cooldown task
  (`KismetSystemLibrary.Delay` Cooldown)
  (`/Engine/EditorBlueprintResources/StandardMacros.IsValid` _returnvalue
    (:`Is Valid`
      (`BlackboardComponent.SetValueAsBool` _returnvalue "AttackCooldown" false))))

(event `self.PawnSensing.OnSeePawn`
  (params (Pawn :type "Pawn Object Reference"))
  ;[1 0.004025 0.7835] Trigger Chase On Sight
  (`self.Set Chase Target` Pawn))

(event `Check Player`
  (bind _returnvalue (`AIBlueprintHelperLibrary.GetBlackboard` (`AIBlueprintHelperLibrary.GetAIController` self)))
  ; Not Used
  (if (<= (`KismetMathLibrary.Vector_Distance` (`self.K2_GetActorLocation`) (`self.K2_GetActorLocation` (`self.ChaseTarget`))) (`BlackboardComponent.GetValueAsFloat` (`AIBlueprintHelperLibrary.GetBlackboard` (`AIBlueprintHelperLibrary.GetAIController` self)) "Attack Range"))
    (`BlackboardComponent.SetValueAsBool` _returnvalue "CanSeePl" true)
    (else
      (`BlackboardComponent.SetValueAsBool` _returnvalue "CanSeePl" false))))

(event `self.ReceiveBeginPlay`
  (bind _ac_enemyhealthcomponent (`self.AC_EnemyHealthComponent`))
  (bind _maxhealth (`/Game/Blueprints/Components/AC_HealthComponent.MaxHealth` _ac_enemyhealthcomponent))
  (bind _returnvalue (`AIBlueprintHelperLibrary.GetBlackboard` (`AIBlueprintHelperLibrary.GetAIController` self)))
  ;[1 0.004025 0.7835] Initializes Health Values
  (`/Game/Blueprints/Components/AC_HealthComponent.HealthCompInit` _ac_enemyhealthcomponent)
  (`BlackboardComponent.SetValueAsFloat` _returnvalue "MaxHealth" _maxhealth)
  (`BlackboardComponent.SetValueAsFloat` _returnvalue "CurrentHealth" _maxhealth))

(event `self.ReceiveAnyDamage`
  (params (Damage :type "Float (single-precision)") (DamageType :type "DamageType Object Reference") (InstigatedBy :type "Controller Object Reference") (DamageCauser :type "Actor Object Reference"))
  (bind _currenthealth (`/Game/Blueprints/Components/AC_HealthComponent.CurrentHealth` (`self.AC_EnemyHealthComponent`)))
  ;[1 0.004025 0.7835] Handles Damage
  (`/Game/Blueprints/Components/AC_HealthComponent.TakeDamage` (`self.AC_EnemyHealthComponent`) self Damage DamageType InstigatedBy DamageCauser)
  (`self.Set Chase Target` DamageCauser)
  (`KismetSystemLibrary.DelayUntilNextTick`)
  (`BlackboardComponent.SetValueAsFloat` (`AIBlueprintHelperLibrary.GetBlackboard` (`AIBlueprintHelperLibrary.GetAIController` self)) "CurrentHealth" _currenthealth)
  (if (<= _currenthealth 0.0)
    (`self.K2_DestroyActor`)))

(event `Set Chase Target`
  (params (Player :type "Actor Object Reference"))
  (bind (_asbp_player _bsuccess) (cast `/Game/Blueprints/BP_Player` Player :!pure true))
  (bind _returnvalue (`AIBlueprintHelperLibrary.GetBlackboard` (`AIBlueprintHelperLibrary.GetAIController` self)))
  ;[1 0.004025 0.7835] Sets chase target and values for the BT
  (bind _output_get (set `self.ChaseTarget` _asbp_player))
  (if _bsuccess
    (`BlackboardComponent.SetValueAsObject` _returnvalue "Player" _output_get)
    (`BlackboardComponent.SetValueAsBool` _returnvalue "CanSeePlayer" true)
    (`BlackboardComponent.SetValueAsBool` _returnvalue "FarFromPlayer" false)))

(fn `UserConstructionScript`)