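; BP_ChimeraSnake is the snake part of a Chimera enemy, an AI actor with a ranged attack.
; On possession it runs the BT_ChimeraParts behavior tree, and its attack interface event spawns a BP_SnakeProjectile at the Mouth's transform.
; An overlap on the HasBeenAlerted component sets the matching blackboard bool, while DecideTarget and GetClosestPlayer are stubs that return no target.
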(event `self.ReceivePossessed`
  (params (NewController :type "Controller Object Reference"))
  (`AIController.RunBehaviorTree` (`AIBlueprintHelperLibrary.GetAIController` self) "/Game/AI/BehaviourTree/BT_ChimeraParts.BT_ChimeraParts"))

(event `self.AttackInterface`
  (bind _mouth (`self.Mouth`))
  (`|SpawnActorFromClass` "/Game/AI/EnemyProjectiles/BossProjectiles/BP_SnakeProjectile.BP_SnakeProjectile_C" (`KismetMathLibrary.MakeTransform` (`SceneComponent.K2_GetComponentLocation` _mouth) (`SceneComponent.K2_GetComponentRotation` _mouth)) "Undefined" "MultiplyWithRoot" null null))

(event `self.HasBeenAlerted?.OnComponentBeginOverlap`
  (params (OverlappedComponent :type "PrimitiveComponent Object Reference") (OtherActor :type "Actor Object Reference") (OtherComp :type "PrimitiveComponent Object Reference") (OtherBodyIndex :type Integer) (bFromSweep :type Boolean) (SweepResult :type "HitResult Structure (by ref)"))
  (`BlackboardComponent.SetValueAsBool` (`AIBlueprintHelperLibrary.GetBlackboard` null) "HasBeenAlerted" true))

(fn `DecideTarget`
  (params (`TargetRanged?` :type Boolean))
  (returns (`Has Target?` :type Boolean) (Player :type "Actor Object Reference"))
  (return false null))

(fn `GetClosestPlayer`
  (params (`TargetRanged?` :type Boolean))
  (returns (ClosestPlayer :type "Actor Object Reference"))
  (return null))

(fn `UserConstructionScript`)