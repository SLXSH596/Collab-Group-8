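; Player component that plays controller force feedback for attacks, dashes, damage, death and joining the game.
; Initialise caches the pawn and controller, then binds to health, damage, dash and current-weapon events.
; Damage amount and explosive damage type pick light, heavy or explosive effects, with stored values reused to choose the death rumble.
; Tagged effects let higher-priority rumbles stop attack or damage feedback; a comment flags the death binding as needing a fix.
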(event `Light Attack FF`
  (bind _playerref (`self.PlayerRef`))
  ;[0.06301 0.6939 0.1441] Attack
  (if (and (`/Game/Components/Weapons/AC_WeaponBase.bCanAttack` (`/Game/Blueprints/Player/BP_Player.CurrentWeapon` _playerref)) (not (`/Game/Components/Pawns/AC_DashAbility.IsDashing?` (`/Game/Blueprints/Player/BP_Player.AC_DashAbility` _playerref))))
    (`PlayerController.K2_ClientPlayForceFeedback` (`self.PlayerController`) "/Game/JUICE/ForceFeedback/FF_LightAttack.FF_LightAttack" "Attack" false false false)))

(event `Heavy Attack FF`
  (bind _playerref (`self.PlayerRef`))
  ;[0.06301 0.6939 0.1441] Attack
  (if (and (`/Game/Components/Weapons/AC_WeaponBase.bCanAttack` (`/Game/Blueprints/Player/BP_Player.CurrentWeapon` _playerref)) (not (`/Game/Components/Pawns/AC_DashAbility.IsDashing?` (`/Game/Blueprints/Player/BP_Player.AC_DashAbility` _playerref))))
    (`PlayerController.K2_ClientPlayForceFeedback` (`self.PlayerController`) "/Game/JUICE/ForceFeedback/FF_HeavyAttack.FF_HeavyAttack" "Attack" false false false)))

(event `Death_Light FF`
  (bind _playercontroller (`self.PlayerController`))
  ;[0.06301 0.6939 0.1441] Death (need to fix the dead bind)
  (`PlayerController.ClientStopForceFeedback` _playercontroller null "Attack")
  (`PlayerController.ClientStopForceFeedback` _playercontroller null "TakeDamage")
  (`PlayerController.K2_ClientPlayForceFeedback` _playercontroller "/Game/JUICE/ForceFeedback/FF_Death_Light.FF_Death_Light" "Death" false false false))

(event `Explosive FF`
  (bind _playercontroller (`self.PlayerController`))
  ;[0.06301 0.6939 0.1441] Modifiers
  (`PlayerController.ClientStopForceFeedback` _playercontroller null "TakeDamage")
  (`PlayerController.K2_ClientPlayForceFeedback` _playercontroller "/Game/JUICE/ForceFeedback/FF_Explosive.FF_Explosive" "TakeDamage" false false false))

(event `Choose Death FF`
  ;[0.06301 0.6939 0.1441] Death (need to fix the dead bind)
  (if (`/Game/Components/Player/AC_HealthComponent.IsDead?` (`/Game/Blueprints/Player/BP_Player.AC_Health` (`self.PlayerRef`)))
    (if (or (>= (`self.Damage`) 15.0) (`GameplayStatics.ObjectIsA` (`self.Damage Type`) "/Game/Blueprints/WeaponDamageTypes/BP_DamageType_Explosive.BP_DamageType_Explosive_C"))
      (`self.Death_Heavy FF`)
      (else
        (`self.Death_Light FF`)))))

(event `Death_Heavy FF`
  (bind _playercontroller (`self.PlayerController`))
  ;[0.06301 0.6939 0.1441] Death (need to fix the dead bind)
  (`PlayerController.ClientStopForceFeedback` _playercontroller null "Attack")
  (`PlayerController.ClientStopForceFeedback` _playercontroller null "TakeDamage")
  (`PlayerController.K2_ClientPlayForceFeedback` _playercontroller "/Game/JUICE/ForceFeedback/FF_Death_Heavy.FF_Death_Heavy" "Death" false false false))

(event `Player Joined FF`
  ;[0.06301 0.6939 0.1441] Join Game
  (`PlayerController.K2_ClientPlayForceFeedback` (`self.PlayerController`) "/Game/JUICE/ForceFeedback/FF_JoinGame.FF_JoinGame" "PlayerJoin" false false false))

(event `TakeDamage Light FF`
  (bind _playercontroller (`self.PlayerController`))
  ;[0.06301 0.6939 0.1441] Take damage
  (`PlayerController.ClientStopForceFeedback` _playercontroller null "Attack")
  (`PlayerController.K2_ClientPlayForceFeedback` _playercontroller "/Game/JUICE/ForceFeedback/FF_TakeDamage_Light.FF_TakeDamage_Light" "TakeDamage" false false false))

(event `Choose TakeDamage FF`
  (params (DamagedActor :type "Actor Object Reference") (Damage :type "Float (single-precision)") (DamageType :type "DamageType Object Reference") (InstigatedBy :type "Controller Object Reference") (DamageCauser :type "Actor Object Reference"))
  ;[0.06301 0.6939 0.1441] Take damage
  (set `self.Damage` Damage)
  (set `self.Damage Type` DamageType)
  (if (not (`/Game/Components/Player/AC_HealthComponent.IsDead?` (`/Game/Blueprints/Player/BP_Player.AC_Health` (`self.PlayerRef`))))
    (`/Engine/EditorBlueprintResources/StandardMacros.IsValid` DamageCauser
      (:`Is Valid`
        (`/Engine/EditorBlueprintResources/StandardMacros.IsValid` (`Actor.GetComponentByClass` DamageCauser "/Game/Components/Modifiers/AC_Explosive.AC_Explosive_C")
          (:`Is Valid`
            (if (`GameplayStatics.ObjectIsA` (`self.Damage Type`) "/Game/Blueprints/WeaponDamageTypes/BP_DamageType_Explosive.BP_DamageType_Explosive_C")
              (`self.Explosive FF`)
              (else
                (if (>= (`self.Damage`) 15.0) :!label _label
                  (`self.TakeDamage Heavy FF`)
                  (else
                    (`self.TakeDamage Light FF`))))))
          (:`Is Not Valid`
            (goto _label))))
      (:`Is Not Valid`
        (goto _label)))))

(event `TakeDamage Heavy FF`
  (bind _playercontroller (`self.PlayerController`))
  ;[0.06301 0.6939 0.1441] Take damage
  (`PlayerController.ClientStopForceFeedback` _playercontroller null "Attack")
  (`PlayerController.K2_ClientPlayForceFeedback` _playercontroller "/Game/JUICE/ForceFeedback/FF_TakeDamage_Heavy.FF_TakeDamage_Heavy" "TakeDamage" false false false))

(event `Dash FF`
  (bind _playercontroller (`self.PlayerController`))
  ;[0.06301 0.6939 0.1441] Dash
  (`PlayerController.ClientStopForceFeedback` _playercontroller null "Attack")
  (`PlayerController.K2_ClientPlayForceFeedback` _playercontroller "/Game/JUICE/ForceFeedback/FF_Dash.FF_Dash" "Dash" false false false))

(event `Initialise`
  (params (PlayerPawn :type "/Game/Blueprints/Player/BP_Player Object Reference") (`Player Controller` :type "/Game/Blueprints/Player/PC_PlayerController Object Reference"))
  (bind _playerref (`self.PlayerRef`))
  (bind _playerref_2 (`self.PlayerRef`))
  (bind _ac_dashability (`/Game/Blueprints/Player/BP_Player.AC_DashAbility` _playerref_2))
  (bind _currentweapon (`/Game/Blueprints/Player/BP_Player.CurrentWeapon` (`self.PlayerRef`)))
  (bind _ac_health (`/Game/Blueprints/Player/BP_Player.AC_Health` _playerref))
  ;[0.06301 0.6939 0.1441] Initialise
  (`/Engine/EditorBlueprintResources/StandardMacros.IsValid` `Player Controller`
    (:`Is Valid`
      (set `self.PlayerController` `Player Controller`)
      (`/Engine/EditorBlueprintResources/StandardMacros.IsValid` PlayerPawn
        (:`Is Valid`
          (bind _output_get (set `self.PlayerRef` PlayerPawn))
          (bind _returnvalue (`Actor.GetComponentByClass` _output_get "/Game/Components/Player/AC_HealthComponent.AC_HealthComponent_C"))
          (`/Engine/EditorBlueprintResources/StandardMacros.IsValid` _returnvalue
            (:`Is Valid`
              (set `self.Health Component` _returnvalue)
              ;[0.06301 0.6939 0.1441] Setup Binds
              (`/Engine/EditorBlueprintResources/StandardMacros.IsValid` _playerref
                (:`Is Valid`
                  (`/Engine/EditorBlueprintResources/StandardMacros.IsValid` _ac_health
                    (:`Is Valid`
                      (add `/Game/Components/Player/AC_HealthComponent.OnDeath` _ac_health (`|CreateDelegate` :!event `Choose Death FF`)))
                    (:`Is Not Valid`
                      _))
                  (`/Engine/EditorBlueprintResources/StandardMacros.IsValid` _playerref_2
                    (:`Is Valid`
                      (add `Actor.OnTakeAnyDamage` _playerref_2 (`|CreateDelegate` :!event `Choose TakeDamage FF`)))
                    (:`Is Not Valid`
                      _))
                  (`/Engine/EditorBlueprintResources/StandardMacros.IsValid` _ac_dashability
                    (:`Is Valid`
                      (add `/Game/Components/Pawns/AC_DashAbility.OnDash` _ac_dashability (`|CreateDelegate` :!event `Dash FF`)))
                    (:`Is Not Valid`
                      _))
                  (`/Engine/EditorBlueprintResources/StandardMacros.IsValid` _currentweapon
                    (:`Is Valid`
                      (add `/Game/Components/Weapons/AC_WeaponBase.OnLightAttack` _currentweapon (`|CreateDelegate` :!event `Test 1`))
                      (add `/Game/Components/Weapons/AC_WeaponBase.OnHeavyAttack` _currentweapon (`|CreateDelegate` :!event `Test 2`)))))))))
        (:`Is Not Valid`
          (`KismetSystemLibrary.RaiseScriptError` "Rumble references are borked" :!label _label_2))))
    (:`Is Not Valid`
      (goto _label_2))))

(event `Test 1`
  (`KismetSystemLibrary.PrintString` "L attack ff"))

(event `Test 2`
  (`KismetSystemLibrary.PrintString` "R attack ff"))