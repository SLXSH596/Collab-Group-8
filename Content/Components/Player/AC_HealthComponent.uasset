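; Health component that gives its owner health, a widget health bar, damage handling, death and optional timed regen.
; Damage triggers the indicator, enemy aggro swap, brief i-frames and damage-type knockback; bar updates, death and regen scheduling run only with a knockback component.
; Death broadcasts an event and grants vampiric healing to buffed attackers.
; AC_Respawn's event restores full health and resets the player's face texture.
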(event `HealthCompInit`
  (params (Player :type "/Game/Blueprints/Player/BP_Player Object Reference"))
  (bind _returnvalue (`self.GetOwner`))
  (bind _returnvalue_2 (`Actor.GetComponentByClass` (`self.GetOwner`) "/Game/Components/Player/AC_Respawn.AC_Respawn_C"))
  (bind _returnvalue_3 (`Actor.GetComponentByClass` (`self.GetOwner`) "/Game/Components/Pawns/AC_DamageIndicator.AC_DamageIndicator_C"))
  (set `self.I_FrameActive?` false)
  (set `self.Refforplayerface` Player)
  (`/Engine/EditorBlueprintResources/StandardMacros.DoOnce` false
    (:`Completed`
      (add `Actor.OnTakeAnyDamage` _returnvalue (`|CreateDelegate` :!event `TakeDamage`))
      (set `self.CurrentHealth` (`self.MaxHealth`))
      (bind _returnvalue_4 (`|AddComponentByClass` _returnvalue (`self.WidgetClass`) false (`KismetMathLibrary.MakeTransform` (`self.HealthBarLocation`))))
      (bind _aswbp_health_parent (cast `/Game/UI/WBP_HealthPARENT` (`WidgetComponent.GetWidget` _returnvalue_4)))
      (bind _output_get (set `self.HealthBarComponent` _aswbp_health_parent))
      (`/Game/UI/WBP_HealthPARENT.Init` _output_get (`self.MaxHealth`))
      (`/Engine/EditorBlueprintResources/StandardMacros.IsValid` _returnvalue_2
        (:`Is Valid`
          (bind _output_get_2 (set `self.Respawn Component` _returnvalue_2))
          (add `/Game/Components/Player/AC_Respawn.OnRespawn` _output_get_2 (`|CreateDelegate` :!event `On Respawn`)))
        (:`Is Not Valid`
          _))
      ;[0.06301 0.6939 0.1441] Damage Indicator
      (`/Engine/EditorBlueprintResources/StandardMacros.IsValid` _returnvalue_3
        (:`Is Valid`
          (set `self.AC Damage Indicator` _returnvalue_3))))))

(event `On Respawn`
  (bind _maxhealth (`self.MaxHealth`))
  ;[0.06301 0.6939 0.1441] Heal owner On Respawn
  (bind _output_get (set `self.CurrentHealth` _maxhealth))
  (`/Game/UI/WBP_HealthPARENT.SetHealthPercent` (`self.HealthBarComponent`) _output_get)
  (`self.OnHealthChange` _output_get _maxhealth)
  (set `self.IsDead?` false)
  (`MaterialInstanceDynamic.SetTextureParameterValue` (`/Game/Blueprints/Player/BP_Player.FaceMaterial` (`self.Refforplayerface`)) "FaceTexture" "/Game/Textures/T_Player_Face_Regular.T_Player_Face_Regular"))

(event `TakeDamage`
  (params (DamagedActor :type "Actor Object Reference") (Damage :type "Float (single-precision)") (DamageType :type "DamageType Object Reference") (InstigatedBy :type "Controller Object Reference") (DamageCauser :type "Actor Object Reference"))
  (bind _returnvalue (`self.GetOwner`))
  (bind _maxhealth (`self.MaxHealth`))
  (bind _knockbackvalues (`self.KnockbackValues`))
  (bind _returnvalue_2 (`Actor.GetComponentByClass` _returnvalue "/Game/Components/Pawns/AC_KnockbackComponent.AC_KnockbackComponent_C"))
  (if (`self.I_FrameActive?`)
    _
    (elif (not (`self.IsDead?`))
      (`self.Stop Health Regen`)
      (`self.EnemyAgroCheck` DamageCauser)
      (bind _asbp_damage_type_parent (cast `/Game/Blueprints/WeaponDamageTypes/BP_DamageType_Parent` DamageType))
      (set `self.KnockbackValues` _asbp_damage_type_parent)
      ;[0.06301 0.6939 0.1441] Damage Indicator
      (`/Game/Components/Pawns/AC_DamageIndicator.Damage Indicator` (`self.AC Damage Indicator`) DamagedActor Damage)
      ;[1 0.5271 0] apply the weapon types knockback values to then be applied to the damaged actor
      (bind _output_get (set `self.CurrentHealth` (`KismetMathLibrary.FClamp` (- (`self.CurrentHealth`) Damage) 0.0 _maxhealth)))
      (`self.StartIFrames` 0.1)
      (`/Engine/EditorBlueprintResources/StandardMacros.IsValid` _returnvalue_2
        (:`Is Valid`
          (`/Game/Components/Pawns/AC_KnockbackComponent.ApplyKnockback` _returnvalue_2 _returnvalue DamageCauser (`/Game/Blueprints/WeaponDamageTypes/BP_DamageType_Parent.KnockbackStrength` _knockbackvalues) (`/Game/Blueprints/WeaponDamageTypes/BP_DamageType_Parent.UpwardKnockback` _knockbackvalues))
          (`/Game/UI/WBP_HealthPARENT.SetHealthPercent` (`self.HealthBarComponent`) _output_get)
          (`self.OnHealthChange` _output_get _maxhealth)
          (if (<= (`self.CurrentHealth`) 0.0)
            (`self.Start Vampiric Heal` DamageCauser)
            ;[0.06301 0.6939 0.1441] Set owner to be dead
            (set `self.IsDead?` true)
            (`self.OnDeath`)
            (else
              ;[0.06301 0.6939 0.1441] Start Health Regen
              (if (`self.RegenHealth?`)
                (bind _returnvalue_3 (`KismetSystemLibrary.K2_SetTimerDelegate` (`|CreateDelegate` :!event `Start Health Regen`) (`self.Regen Start Timer`)))
                (set `self.Start Health Regen Handle` _returnvalue_3)))))))))

(event `StartIFrames`
  (params (`I frame Duration` :type "Float (double-precision)" :default 0.1))
  (set `self.I_FrameActive?` true)
  (`KismetSystemLibrary.K2_SetTimerDelegate` (delegate `EndIFrames`) `I frame Duration`))

(event `Start Vampiric Heal`
  (params (`Damage Causer` :type "Actor Object Reference"))
  (bind _returnvalue (`Actor.GetComponentByClass` `Damage Causer` "/Game/Components/Player/AC_StatComponent.AC_StatComponent_C"))
  ;[0.06301 0.6939 0.1441] Vampiric Heal
  (`/Engine/EditorBlueprintResources/StandardMacros.IsValid` _returnvalue
    (:`Is Valid`
      (if (> (`.Vampiric_16_BBF88A3E47C11B4656DA02B2102A83CD` (break `/Game/Blueprints/Data/F_PlayerBuffs` (`/Game/Components/Player/AC_StatComponent.GetPlayerBuffs` _returnvalue))) 0)
        (`/Game/Components/Player/AC_StatComponent.VampiricHeal` _returnvalue)))))

(event `Stop Health Regen`
  ;[0.06301 0.6939 0.1441] Stop Health Regen
  (`KismetSystemLibrary.K2_ClearAndInvalidateTimerHandle` (`self.Start Health Regen Handle`))
  (`KismetSystemLibrary.K2_ClearAndInvalidateTimerHandle` (`self.Regen Health Handle`)))

(event `EndIFrames`
  (set `self.I_FrameActive?` false))

(event `Start Health Regen`
  ;[0.06301 0.6939 0.1441] Health Regen Timer
  (bind _returnvalue (`KismetSystemLibrary.K2_SetTimerDelegate` (`|CreateDelegate` :!event `Health Regen`) (`self.Regen Timer`) true))
  (set `self.Regen Health Handle` _returnvalue))

(event `EnemyAgro`
  (params (`Player Reference` :type "/Game/Blueprints/Player/BP_Player Object Reference"))
  ;[1 0.004025 0.7835] Initialises Enemy Agro
  (set `self.Player` `Player Reference`)
  (set `self.EnemyAgroActive` true))

(event `Health Regen`
  (bind _maxhealth (`self.MaxHealth`))
  ;[0.06301 0.6939 0.1441] Health Regen
  (bind _output_get (set `self.CurrentHealth` (`KismetMathLibrary.FClamp` (+ (`self.CurrentHealth`) (`self.RegenAmount`)) 0.0 _maxhealth)))
  (`/Game/UI/WBP_HealthPARENT.SetHealthPercent` (`self.HealthBarComponent`) _output_get)
  (`self.OnHealthChange` _output_get _maxhealth)
  (if (== (`self.CurrentHealth`) (`self.MaxHealth`))
    (`self.Stop Health Regen`)))

(fn `EnemyAgroCheck`
  (params (Instigator :type "Actor Object Reference"))
  (bind (_asbp_player _bsuccess) (cast `/Game/Blueprints/Player/BP_Player` Instigator :!pure true))
  ;[1 0.004025 0.7835] Checks and swaps Enemy Agro Target
  (if (and (`self.EnemyAgroActive`) _bsuccess)
    (if (`/Game/Blueprints/Player/BP_Player.ModifierTarget` _asbp_player)
      (`/Game/Blueprints/Player/BP_Player.SwapEnemyAgroTarget` _asbp_player (`self.Player`))
      (return))
    (else
      (return))))