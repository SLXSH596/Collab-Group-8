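; Player component that colors a ring under or on a player by controller index, so players can be told apart.
; Init stores the target primitive and the player controller's ID, then triggers SetRingColor.
; SetRingColor creates a dynamic instance of M_PlayerRing, applies it to the target's first material slot and sets its Color parameter to one of four fixed per-player colors.
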(event `Init`
  (params (`Material Target` :type "StaticMeshComponent Object Reference") (`Player Controller` :type "PlayerController Object Reference"))
  ;[0.06301 0.6939 0.1441] Initiate Player Ring
  (set `self.Material Target` `Material Target`)
  (set `self.Controller ID` (`GameplayStatics.GetPlayerControllerID` `Player Controller`))
  (`self.Set Ring Color`))

(event `Set Ring Color`
  ;[0.06301 0.6939 0.1441] Set Ring Color
  (bind _returnvalue (`KismetMaterialLibrary.CreateDynamicMaterialInstance` "/Game/Materials/M_PlayerRing.M_PlayerRing"))
  (bind _output_get (set `self.Ring Material` _returnvalue))
  (`PrimitiveComponent.SetMaterial` (`self.Material Target`) 0 _output_get)
  (`MaterialInstanceDynamic.SetVectorParameterValue` (`self.Ring Material`) "Color" (select `int` (`self.Controller ID`) :`0` (struct :`R` 1.0 :`A` 1.0) :`1` (struct :`R` 1.0 :`G` 0.75 :`A` 1.0) :`2` (struct :`G` 1.0 :`A` 1.0) :`3` (struct :`B` 1.0 :`A` 1.0) :!type "LinearColor Structure")))