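; AC_Interacting is a player component that lets its owner interact with objects in the world.
; On the IA_Interact press it sphere-traces from InteractRange ahead of the owner back to the owner's location, ignoring the owner and drawing debug shapes.
; If the hit actor has an AC_Interactable component, it calls Interact on it, passing the Owner set in Initialise and the hit actor.
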(event `EnhancedInput|/Game/Input/IA_Interact`
  (params (ActionValue :type Boolean) (ElapsedSeconds :type "Float (double-precision)") (TriggeredSeconds :type "Float (double-precision)") (InputAction :type "InputAction Object Reference" :default "/Game/Input/IA_Interact.IA_Interact"))
  (:`Started`
    ;[0.4793 0.05127 0.0648] Create a Sphere Trace for Interaction
    (bind (_trace_start _trace_end _defaultobjecttype _array) (`self.Get_TraceValues`))
    (bind (_outhit _returnvalue) (`KismetSystemLibrary.SphereTraceSingleForObjects` _trace_start _trace_end 120.0 _defaultobjecttype false _array "ForDuration"))
    ;[0.4793 0.05127 0.0648] Checks the "Hit Actor" has the Interactable Component
    (if _returnvalue
      (bind (_bblockinghit _binitialoverlap _time _distance _location _impactpoint _normal _impactnormal _physmat _hitactor) (`GameplayStatics.BreakHitResult` _outhit))
      (bind _returnvalue_2 (`Actor.GetComponentByClass` _hitactor "/Game/Components/Objects/AC_Interactable.AC_Interactable_C"))
      (`/Engine/EditorBlueprintResources/StandardMacros.IsValid` _returnvalue_2
        (:`Is Valid`
          ;[0.4793 0.05127 0.0648] Interact with Object
          (`/Game/Components/Objects/AC_Interactable.Interact` _returnvalue_2 (`self.Owner`) _hitactor))))))

(event `Initialise`
  (params (Owner :type "/Game/Blueprints/Player/BP_Player Object Reference"))
  (set `self.Owner` Owner))

(fn `Get_TraceValues`
  (returns (`Trace Start` :type "Vector Structure") (`Trace End` :type "Vector Structure") (DefaultObjectType :type "Array of EObjectTypeQuery Enum") (Array :type "Array of Actor Object Reference (by ref)"))
  (bind _returnvalue (`self.GetOwner`))
  (bind _returnvalue_2 (`Actor.K2_GetActorLocation` _returnvalue))
  (return (+ (* (`Actor.GetActorForwardVector` _returnvalue) (`self.InteractRange`)) _returnvalue_2) _returnvalue_2 (`self.DefaultObjectType`) (`|MakeArray` _returnvalue)))