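; Player stat component for BP_Player that applies stackable buffs to health, move speed, damage, attack speed and dash distance.
; Increase functions multiply or divide owner stats and save stack counts in the GameInstance, keyed by controller ID.
; Initialise replays saved stacks without incrementing; ResetPlayerBuffs attempts reversal but divides attack cooldown again.
; It also restores health and spawns an attached healing aura; knockback and health-based attack scaling are unfinished.
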(fn `ActivateHealingAura`
  (params (Radius :type "Float (double-precision)") (`Heal Amount` :type "Float (double-precision)") (`Healing Rate` :type "Float (double-precision)") (Duration :type "Float (double-precision)"))
  (bind _returnvalue (`self.GetOwner`))
  (bind _returnvalue_2 (`|SpawnActorFromClass` "/Game/Blueprints/Pickup/BP_HealingAura.BP_HealingAura_C" (`KismetMathLibrary.Conv_VectorToTransform` (`Actor.K2_GetActorLocation` _returnvalue)) "Undefined" "MultiplyWithRoot" null null))
  (`Actor.K2_AttachToActor` _returnvalue_2 _returnvalue "None" "KeepRelative" "KeepRelative" "KeepRelative" true))

(fn `BuffPersistenceGet`
  (bind (_health _attackspeed _damage _knockback _dashdistance _speed) (break `/Game/Blueprints/Data/F_PlayerBuffs` (`self.GetPlayerBuffs`)))
  (`|ExecutionSequence`
    (:`then_0`
      (if (> _health 0)
        (for _ (range 1 (+ _health 1))
          (`self.IncreaseMaxHealth` false))))
    (:`then_1`
      (if (> _attackspeed 0)
        (for _ (range 1 (+ _attackspeed 1))
          (`self.IncreaseAttackSpeed` false))))
    (:`then_2`
      (if (> _damage 0)
        (for _ (range 1 (+ _damage 1))
          (`self.IncreaseDamage` false))))
    (:`then_3`
      (if (> _knockback 0)
        (for _ (range 1 (+ _knockback 1))
          (`self.IncreaseKnockback`))))
    (:`then_4`
      (if (> _dashdistance 0)
        (for _ (range 1 (+ _dashdistance 1))
          (`self.IncreaseDashDistance` false))))
    (:`then_5`
      (if (> _speed 0)
        (for _ (range 1 (+ _speed 1))
          (`self.IncreaseSpeed` false))))))

(fn `CreatePlayerBuffData`
  (`BlueprintMapLibrary.Map_Add` (`/Game/Blueprints/GI_GameInstance.PlayerBuffData` (`self.Game Instance`)) (`GameplayStatics.GetPlayerControllerID` (`/Game/Blueprints/Player/BP_Player.PlayerController` (`self.Owner`))) (make `/Game/Blueprints/Data/F_PlayerBuffs` 0)))

(fn `GetPlayerBuffs`
  (returns (PlayerBuffs :type "/Game/Blueprints/Data/F_PlayerBuffs Structure"))
  (bind (_value _returnvalue) (`BlueprintMapLibrary.Map_Find` (`/Game/Blueprints/GI_GameInstance.PlayerBuffData` (`self.Game Instance`)) (`GameplayStatics.GetPlayerControllerID` (`/Game/Blueprints/Player/BP_Player.PlayerController` (`self.Owner`)))))
  (if _returnvalue
    (return _value)))

(fn `IncreaseAttackSpeed`
  (params (bShouldIncrement :type Boolean))
  (bind _playerbuffs (`self.GetPlayerBuffs`))
  (bind _currentweapon (`/Game/Blueprints/Player/BP_Player.CurrentWeapon` (`self.Owner`)))
  (set `/Game/Components/Weapons/AC_WeaponBase.AttackCooldown` (/ (`/Game/Components/Weapons/AC_WeaponBase.AttackCooldown` _currentweapon) (`self.AttackSpeedIncreaseValue`)) _currentweapon)
  (if bShouldIncrement
    (`/Engine/EditorBlueprintResources/StandardMacros.IncrementInt` (`.AttackSpeed_6_86AE96EB41D2465F4E1E22910A388069` (break `/Game/Blueprints/Data/F_PlayerBuffs` _playerbuffs))
      (:`  `
        _)))
  (`BlueprintMapLibrary.Map_Add` (`/Game/Blueprints/GI_GameInstance.PlayerBuffData` (`self.Game Instance`)) (`GameplayStatics.GetPlayerControllerID` (`/Game/Blueprints/Player/BP_Player.PlayerController` (`self.Owner`))) _playerbuffs)
  (return))

(fn `IncreaseDamage`
  (params (bShouldIncrement :type Boolean))
  (returns (NewDamageValue :type "Float (double-precision)"))
  (bind _playerbuffs (`self.GetPlayerBuffs`))
  (bind _currentweapon (`/Game/Blueprints/Player/BP_Player.CurrentWeapon` (`self.Owner`)))
  (bind _output_get (set `/Game/Components/Weapons/AC_WeaponBase.BaseDamage` (* (`/Game/Components/Weapons/AC_WeaponBase.BaseDamage` _currentweapon) (`self.DamageIncreaseValue`)) _currentweapon))
  (if bShouldIncrement
    (`/Engine/EditorBlueprintResources/StandardMacros.IncrementInt` (`.Damage_7_F7E6D403466A141E8A1823B3105E92F3` (break `/Game/Blueprints/Data/F_PlayerBuffs` _playerbuffs))
      (:`  `
        _)))
  (`BlueprintMapLibrary.Map_Add` (`/Game/Blueprints/GI_GameInstance.PlayerBuffData` (`self.Game Instance`)) (`GameplayStatics.GetPlayerControllerID` (`/Game/Blueprints/Player/BP_Player.PlayerController` (`self.Owner`))) _playerbuffs)
  (return _output_get))

(fn `IncreaseDashDistance`
  (params (bShouldIncrement :type Boolean))
  (bind _playerbuffs (`self.GetPlayerBuffs`))
  (bind _ac_dashability (`/Game/Blueprints/Player/BP_Player.AC_DashAbility` (`self.Owner`)))
  (set `/Game/Components/Pawns/AC_DashAbility.Dash Distance` (* (`/Game/Components/Pawns/AC_DashAbility.Dash Distance` _ac_dashability) (`self.DashIncreaseValue`)) _ac_dashability)
  (if bShouldIncrement
    (`/Engine/EditorBlueprintResources/StandardMacros.IncrementInt` (`.DashDistance_11_26E189C948AE9FFAA96C0BBF6B144114` (break `/Game/Blueprints/Data/F_PlayerBuffs` _playerbuffs))
      (:`  `
        _)))
  (`BlueprintMapLibrary.Map_Add` (`/Game/Blueprints/GI_GameInstance.PlayerBuffData` (`self.Game Instance`)) (`GameplayStatics.GetPlayerControllerID` (`/Game/Blueprints/Player/BP_Player.PlayerController` (`self.Owner`))) _playerbuffs)
  (return))

(fn `IncreaseKnockback`)

(fn `IncreaseMaxHealth`
  (params (bShouldIncrement :type Boolean))
  (returns (NewMaxHealth :type "Float (double-precision)"))
  (bind _playerbuffs (`self.GetPlayerBuffs`))
  (bind _ac_health (`/Game/Blueprints/Player/BP_Player.AC_Health` (`self.Owner`)))
  (bind _output_get (set `/Game/Components/Player/AC_HealthComponent.MaxHealth` (* (`/Game/Components/Player/AC_HealthComponent.MaxHealth` _ac_health) (`self.MaxHealthIncreasevalue`)) _ac_health))
  (if bShouldIncrement
    (`/Engine/EditorBlueprintResources/StandardMacros.IncrementInt` (`.Health_2_D01783FC4AEB58C0706B05B0D7AEDF1C` (break `/Game/Blueprints/Data/F_PlayerBuffs` _playerbuffs))
      (:`  `
        _)))
  (`BlueprintMapLibrary.Map_Add` (`/Game/Blueprints/GI_GameInstance.PlayerBuffData` (`self.Game Instance`)) (`GameplayStatics.GetPlayerControllerID` (`/Game/Blueprints/Player/BP_Player.PlayerController` (`self.Owner`))) _playerbuffs)
  (return _output_get))

(fn `IncreaseSpeed`
  (params (bShouldIncrement :type Boolean))
  (returns (NewSpeed :type "Float (double-precision)"))
  (bind _playerbuffs (`self.GetPlayerBuffs`))
  (bind _charactermovement (`Character.CharacterMovement` (`self.Owner`)))
  (bind _output_get (set `CharacterMovementComponent.MaxWalkSpeed` (* (`MovementComponent.GetMaxSpeed` _charactermovement) (`self.SpeedIncreaseValue`)) _charactermovement))
  (if bShouldIncrement
    (`/Engine/EditorBlueprintResources/StandardMacros.IncrementInt` (`.Speed_13_501616FD434C1EA3FF676F8187E0C2BF` (break `/Game/Blueprints/Data/F_PlayerBuffs` _playerbuffs))
      (:`  `
        _)))
  (`BlueprintMapLibrary.Map_Add` (`/Game/Blueprints/GI_GameInstance.PlayerBuffData` (`self.Game Instance`)) (`GameplayStatics.GetPlayerControllerID` (`/Game/Blueprints/Player/BP_Player.PlayerController` (`self.Owner`))) _playerbuffs)
  (return _output_get))

(fn `Initialise`
  (bind _asbp_player (cast `/Game/Blueprints/Player/BP_Player` (`self.GetOwner`)))
  (bind _output_get (set `self.Owner` _asbp_player))
  (set `self.Game Instance` (`/Game/Blueprints/Player/BP_Player.GameInstance` _output_get))
  (`self.BuffPersistenceGet`))

(fn `RecoverHealth`
  (returns (NewCurrentHealth :type "Float (double-precision)"))
  (bind _ac_health (`/Game/Blueprints/Player/BP_Player.AC_Health` (`self.Owner`)))
  (bind _maxhealth (`/Game/Components/Player/AC_HealthComponent.MaxHealth` _ac_health))
  (bind _output_get (set `/Game/Components/Player/AC_HealthComponent.CurrentHealth` (`KismetMathLibrary.FClamp` (+ (`/Game/Components/Player/AC_HealthComponent.CurrentHealth` _ac_health) (mod _maxhealth 20.0)) 0.0 _maxhealth) _ac_health))
  (return _output_get))

(fn `ResetPlayerBuffs`
  (bind ((`Health_2_D01783FC4AEB58C0706B05B0D7AEDF1C` _health)) (break `/Game/Blueprints/Data/F_PlayerBuffs` (`self.GetPlayerBuffs`)))
  (bind ((`Speed_13_501616FD434C1EA3FF676F8187E0C2BF` _speed)) (break `/Game/Blueprints/Data/F_PlayerBuffs` (`self.GetPlayerBuffs`)))
  (bind ((`DashDistance_11_26E189C948AE9FFAA96C0BBF6B144114` _dashdistance)) (break `/Game/Blueprints/Data/F_PlayerBuffs` (`self.GetPlayerBuffs`)))
  (bind ((`Damage_7_F7E6D403466A141E8A1823B3105E92F3` _damage)) (break `/Game/Blueprints/Data/F_PlayerBuffs` (`self.GetPlayerBuffs`)))
  (bind ((`AttackSpeed_6_86AE96EB41D2465F4E1E22910A388069` _attackspeed)) (break `/Game/Blueprints/Data/F_PlayerBuffs` (`self.GetPlayerBuffs`)))
  (bind _charactermovement (`Character.CharacterMovement` (`self.Owner`)))
  (bind _ac_health (`/Game/Blueprints/Player/BP_Player.AC_Health` (`self.Owner`)))
  (bind _currentweapon (`/Game/Blueprints/Player/BP_Player.CurrentWeapon` (`self.Owner`)))
  (bind _ac_dashability (`/Game/Blueprints/Player/BP_Player.AC_DashAbility` (`self.Owner`)))
  (bind _currentweapon_2 (`/Game/Blueprints/Player/BP_Player.CurrentWeapon` (`self.Owner`)))
  (`|ExecutionSequence`
    (:`then_0`
      (if (>= _health 1)
        (for _ (range _health)
          (set `/Game/Components/Player/AC_HealthComponent.MaxHealth` (/ (`/Game/Components/Player/AC_HealthComponent.MaxHealth` _ac_health) (`self.MaxHealthIncreasevalue`)) _ac_health))))
    (:`then_1`
      (if (>= _attackspeed 1)
        (for _ (range _attackspeed)
          (set `/Game/Components/Weapons/AC_WeaponBase.AttackCooldown` (/ (`/Game/Components/Weapons/AC_WeaponBase.AttackCooldown` _currentweapon) (`self.AttackSpeedIncreaseValue`)) _currentweapon))))
    (:`then_2`
      (if (>= _damage 1)
        (for _ (range _damage)
          (set `/Game/Components/Weapons/AC_WeaponBase.BaseDamage` (/ (`/Game/Components/Weapons/AC_WeaponBase.BaseDamage` _currentweapon_2) (`self.DamageIncreaseValue`)) _currentweapon_2))))
    (:`then_3`
      (if (>= (`.Knockback_9_8B604A0A42C812C2C3199DB3407D5BCA` (break `/Game/Blueprints/Data/F_PlayerBuffs` (`self.GetPlayerBuffs`))) 1)
        _))
    (:`then_4`
      (if (>= _dashdistance 1)
        (for _ (range _dashdistance)
          (set `/Game/Components/Pawns/AC_DashAbility.Dash Distance` (/ (`/Game/Components/Pawns/AC_DashAbility.Dash Distance` _ac_dashability) (`self.DashIncreaseValue`)) _ac_dashability))))
    (:`then_5`
      (if (>= _speed 1)
        (for _ (range _speed)
          (set `CharacterMovementComponent.MaxWalkSpeed` (/ (`MovementComponent.GetMaxSpeed` _charactermovement) (`self.SpeedIncreaseValue`)) _charactermovement))))))

(fn `ScaleAttackFromHealth`
  (locals (LocalCurrentHealth :type Integer) (LocalCurrentDamage :type Integer))
  (bind ((`Health_2_D01783FC4AEB58C0706B05B0D7AEDF1C` _health) (`Damage_7_F7E6D403466A141E8A1823B3105E92F3` _damage)) (break `/Game/Blueprints/Data/F_PlayerBuffs` (`self.GetPlayerBuffs`)))
  (set `local.LocalCurrentHealth` _health)
  (set `local.LocalCurrentDamage` _damage))