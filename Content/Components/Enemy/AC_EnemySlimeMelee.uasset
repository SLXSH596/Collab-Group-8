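; Actor component for the slime enemy's melee attack, dealing damage in front of its owner.
; LightAttack, gated by CanAttack, runs a multi sphere object trace along the owner's forward vector, offset by AttackRange, with debug drawing on.
; Each hit receives BaseDamage as enemy melee damage type, with no deduplication of actors.
; A timer then calls MeleeCooldown to re-enable attacking after AttackCooldown.
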(event `self.LightAttack`
  (bind _returnvalue (`self.GetOwner`))
  (bind _returnvalue_2 (`Actor.K2_GetActorLocation` _returnvalue))
  (bind _returnvalue_3 (`Actor.GetActorForwardVector` _returnvalue))
  ;[0 0.15 0.147 0.502] Enemy Attack Logic
  (if (`self.bCanAttack`)
    (set `self.bCanAttack` false)
    (bind _outhits (`KismetSystemLibrary.SphereTraceMultiForObjects` :`Start` (+ (* (`Actor.GetActorForwardVector` _returnvalue) (`self.AttackRange`)) _returnvalue_2 (* _returnvalue_3 150.0)) :`End` (+ _returnvalue_2 (* _returnvalue_3 75.0)) :`Radius` 50.0 :`ObjectTypes` (`self.DefaultObjectType`) :`DrawDebugType` "ForDuration"))
    (if true
      (for _array_element _outhits
        (`GameplayStatics.ApplyDamage` (`.HitActor` (`GameplayStatics.BreakHitResult` _array_element)) (`self.BaseDamage`) null (`self.GetOwner`) "/Game/Blueprints/WeaponDamageTypes/BP_DamageType_EnemyMelee.BP_DamageType_EnemyMelee_C")))
    (`KismetSystemLibrary.K2_SetTimerDelegate` (delegate `MeleeCooldown`) (`self.AttackCooldown`))))

(event `MeleeCooldown`
  ;[0 0.15 0.147 0.502] Enemy Attack Logic
  (set `self.bCanAttack` true))