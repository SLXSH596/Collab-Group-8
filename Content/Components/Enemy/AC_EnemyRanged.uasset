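; Enemy ranged attack component that fires a projectile from its owner on a light attack, limited by a cooldown.
; LightAttack resets the heavy attack multiplier, then, if attacking is allowed, spawns BP_EnemyProjectile just ahead of the owner, facing the same way and carrying BaseDamage.
; Firing clears CanAttack and starts an AttackCooldown timer, whose RangedCooldown event re-enables attacking.
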(event `self.LightAttack`
  (bind _returnvalue (`self.GetOwner`))
  ;[1 0.004025 0.7835] Enemy Ranged Attack
  (set `self.HeavyAttackMultiplier` 1.0)
  (if (`self.bCanAttack`)
    (set `self.bCanAttack` false)
    (`|SpawnActorFromClass` "/Game/Blueprints/WeaponProjectiles/BP_EnemyProjectile.BP_EnemyProjectile_C" (`KismetMathLibrary.MakeTransform` (+ (* (`Actor.GetActorForwardVector` _returnvalue) 80.0) (`Actor.K2_GetActorLocation` _returnvalue)) (`Actor.K2_GetActorRotation` _returnvalue)) "Undefined" "MultiplyWithRoot" (`self.GetOwner`) (`self.BaseDamage`) null)
    (`KismetSystemLibrary.K2_SetTimerDelegate` (delegate `RangedCooldown`) (`self.AttackCooldown`))))

(event `RangedCooldown`
  ;[1 0.004025 0.7835] Enemy Ranged Attack
  (set `self.bCanAttack` true))