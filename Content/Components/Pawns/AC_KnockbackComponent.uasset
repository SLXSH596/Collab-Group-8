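; Pawn component that knocks a target Character away from an instigating actor.
; One tick after BeginPlay it caches the global knockback multiplier from BP_GameMode.
; ApplyKnockback scales the normalized instigator-to-target direction by strength and multiplier, adds scaled upward strength, and clamps vertical velocity between the multiplier and a fixed cap.
; The result goes to LaunchCharacter without overrides, so it adds to existing velocity.
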(event `self.ReceiveBeginPlay`
  (`KismetSystemLibrary.DelayUntilNextTick`)
  (bind _asbp_game_mode (cast `/Game/Blueprints/Player/BP_Gamemode` (`GameplayStatics.GetGameMode`)))
  (bind _output_get (set `self.As BP Gamemode` _asbp_game_mode))
  (set `self.KnockbackMultiplier` (`/Game/Blueprints/Player/BP_Gamemode.GlobalKnockbackMultiplier` _output_get)))

(event `Initialise`
  (params (Owner :type "/Game/Blueprints/Player/BP_Player Object Reference"))
  (set `self.Owner` Owner))

(fn `ApplyKnockback`
  (params (TargetActor :type "Actor Object Reference") (InstigatorActor :type "Actor Object Reference") (Strength :type "Float (double-precision)") (UpwardStrength :type "Float (double-precision)"))
  (bind _knockbackmultiplier (`self.KnockbackMultiplier`))
  (`/Engine/EditorBlueprintResources/StandardMacros.IsValid` InstigatorActor
    (:`Is Valid`
      (bind _ascharacter (cast `Character` TargetActor))
      (`Character.LaunchCharacter` _ascharacter (`KismetMathLibrary.MakeVector` (.x (* (`KismetMathLibrary.Normal` (- (`Actor.K2_GetActorLocation` TargetActor) (`Actor.K2_GetActorLocation` InstigatorActor))) (* _knockbackmultiplier Strength))) (.y (* (`KismetMathLibrary.Normal` (- (`Actor.K2_GetActorLocation` TargetActor) (`Actor.K2_GetActorLocation` InstigatorActor))) (* _knockbackmultiplier Strength))) (`KismetMathLibrary.FClamp` (+ (.z (* (`KismetMathLibrary.Normal` (- (`Actor.K2_GetActorLocation` TargetActor) (`Actor.K2_GetActorLocation` InstigatorActor))) (* _knockbackmultiplier Strength))) (* _knockbackmultiplier UpwardStrength)) _knockbackmultiplier 300.0)) false false))))