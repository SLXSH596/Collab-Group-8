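; Actor component that gives hit feedback on its owning pawn with a damage overlay material and a spawned damage number.
; Initiate creates a dynamic material with configurable thickness and binds to the owner's any-damage event.
; Damage on a living actor applies the overlay, spawns BP_DamageNumber with offset start and end points, and starts a removal timer.
; Hits while the overlay is visible trigger neither effect again.
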(event `Initiate`
  (params (Mesh :type "MeshComponent Object Reference") (`Mat Thickness` :type "Float (double-precision)" :default 1.2))
  ;[0.06301 0.6939 0.1441] Initialise
  (set `self.Mesh` Mesh)
  (bind _returnvalue (`KismetMaterialLibrary.CreateDynamicMaterialInstance` "/Game/Materials/M_DamageMaterial.M_DamageMaterial"))
  (bind _output_get (set `self.Damage Material` _returnvalue))
  (`MaterialInstanceDynamic.SetScalarParameterValue` _output_get "Thickness" `Mat Thickness`)
  (add `Actor.OnTakeAnyDamage` (`self.GetOwner`) (`|CreateDelegate` :!event `AnyDamage`)))

(event `Damage Indicator`
  (params (`Damaged Actor` :type "Actor Object Reference") (Damage :type "Float (double-precision)"))
  ;[0.06301 0.6939 0.1441] Activate Damage Indicator
  (set `self.Damage` Damage)
  (bind _isdead (message `/Game/Interfaces/BPI_PlayerInterface.IsDead` `Damaged Actor`))
  (if _isdead
    _
    (elif (not (`self.Material Visible?`))
      (`self.Apply Mat`))))

(event `AnyDamage`
  (params (DamagedActor :type "Actor Object Reference") (Damage :type "Float (single-precision)") (DamageType :type "DamageType Object Reference") (InstigatedBy :type "Controller Object Reference") (DamageCauser :type "Actor Object Reference"))
  ;[0.06301 0.6939 0.1441] Activate Damage Indicator
)

(event `Apply Mat`
  ;[0.06301 0.6939 0.1441] Apply / Remove Damage Material
  (`/Engine/EditorBlueprintResources/StandardMacros.IsValid` (`self.Damage Material`)
    (:`Is Valid`
      (`MeshComponent.SetOverlayMaterial` (`self.Mesh`) (`self.Damage Material`)))
    (:`Is Not Valid`
      _))
  (set `self.Material Visible?` true)
  (`self.Spawn Dmg Widget`)
  (bind _returnvalue (`KismetSystemLibrary.K2_SetTimerDelegate` (`|CreateDelegate` :!event `Remove Material`) 0.45))
  (set `self.Remove Mat Handle` _returnvalue))

(event `Spawn Dmg Widget`
  (bind _returnvalue (`self.GetOwner`))
  ;[0.06301 0.6939 0.1441] Spawn Damage Number
  (bind _output_get (set `self.Start Loc` (`Actor.K2_GetActorLocation` _returnvalue)))
  (set `self.End Loc` (+ _output_get (-25.0 -25.0 50.0)))
  (`|SpawnActorFromClass` "/Game/Blueprints/LevelActors/BP_DamageNumber.BP_DamageNumber_C" (`Actor.GetTransform` _returnvalue) "Undefined" "MultiplyWithRoot" null (`self.Damage`) (`self.Start Loc`) (`self.End Loc`) null))

(event `Remove Material`
  ;[0.06301 0.6939 0.1441] Apply / Remove Damage Material
  (`MeshComponent.SetOverlayMaterial` (`self.Mesh`) (`self.ResetOverlay`))
  (set `self.Material Visible?` false))