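; AC_DashAbility is a pawn component that gives its owning character a ground-only directional dash with a cooldown and knockback on impact.
; Dash input plays a montage whose notify launches the owner along its velocity, or forward vector when nearly still, and starts the cooldown timer.
; While dashing, owner hits trigger AC_KnockbackComponent on the other actor once, via a DoOnce that resets when the cooldown ends.
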(event `EnhancedInput|/Game/Input/IA_Dash`
  (params (ActionValue :type Boolean) (ElapsedSeconds :type "Float (double-precision)") (TriggeredSeconds :type "Float (double-precision)") (InputAction :type "InputAction Object Reference" :default "/Game/Input/IA_Dash.IA_Dash"))
  (bind _owner (`self.Owner`))
  (bind _returnvalue (`Actor.GetVelocity` _owner))
  (bind (_returnvalue_x _returnvalue_y) (`KismetMathLibrary.BreakVector` (* (`KismetMathLibrary.SelectVector` (`KismetMathLibrary.Normal` _returnvalue) (`Actor.GetActorForwardVector` (`self.GetOwner`)) (> (`KismetMathLibrary.VSize` _returnvalue) 25.0)) (`self.Dash Distance`))))
  (:`Triggered`
    (if (not (`NavMovementComponent.IsFalling` (`Character.CharacterMovement` _owner)))
      (if (and (not (`self.IsDashing?`)) (not (`self.DashCooldownActive?`)))
        (set `self.IsDashing?` true)
        (set `self.DashCooldownActive?` true)
        (`self.OnDash`)
        (`|PlayMontage` (`Character.Mesh` _owner) "/Game/Animation/Player/AM_PlayerDash.AM_PlayerDash"
          (:`OnCompleted`
            (set `self.IsDashing?` false :!label _label))
          (:`OnInterrupted`
            (goto _label))
          (:`OnNotifyBegin`
            (`Character.LaunchCharacter` _owner (`KismetMathLibrary.MakeVector` _returnvalue_x _returnvalue_y) false false)
            ;[0 0.15 0.147 0.502] Set timer (instead of delay)
            (`KismetSystemLibrary.K2_SetTimerDelegate` (delegate `SetNotDashing`) (`self.Dash Cooldown`))))))))

(event `SetNotDashing`
  ;[0.06301 0.6939 0.1441] Reset dash knockback
  (set `self.DashCooldownActive?` false)
  (`self.Reset Knockback`))

(event `Initialise`
  (params (Owner :type "/Game/Blueprints/Player/BP_Player Object Reference"))
  (bind _output_get (set `self.Owner` Owner))
  ;[0.06301 0.6939 0.1441] Bind On Hit
  (add `Actor.OnActorHit` _output_get (`|CreateDelegate` :!event `OnActorHit`)))

(event `OnActorHit`
  (params (SelfActor :type "Actor Object Reference") (OtherActor :type "Actor Object Reference") (NormalImpulse :type "Vector Structure") (Hit :type "HitResult Structure (by ref)"))
  (bind _returnvalue (`Actor.GetComponentByClass` OtherActor "/Game/Components/Pawns/AC_KnockbackComponent.AC_KnockbackComponent_C"))
  ;[0.06301 0.6939 0.1441] Dash Knockback
  (if (`self.IsDashing?`)
    (`/Engine/EditorBlueprintResources/StandardMacros.IsValid` _returnvalue
      (:`Is Valid`
        (`/Engine/EditorBlueprintResources/StandardMacros.DoOnce` false :!label _label_2
          (:`Completed`
            (`/Game/Components/Pawns/AC_KnockbackComponent.ApplyKnockback` _returnvalue OtherActor SelfActor (`self.Knockback Strength`) (`self.Knockback Upward Strength`))))))))

(event `Reset Knockback`
  ;[0.06301 0.6939 0.1441] Dash Knockback
  (goto _label_2 :!via `Reset`))