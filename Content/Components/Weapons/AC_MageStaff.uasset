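; Mage staff weapon component that gives its owner light and heavy ranged attacks by spawning BP_MagicBall projectiles.
; Light attack fires one ball from in front of the owner along its facing.
; Heavy attack spawns a symmetric fan sized by SpellAmount around the owner's Arrow component, offset sideways and in yaw, passing a boosted multiplier to each ball.
; Both attacks share a CanAttack gate that timer events reopen after AttackCooldown.
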(event `self.LightAttack`
  (bind _returnvalue (`self.GetOwner`))
  ;[0 0.15 0.147 0.502] Staff Attack Logic
  (set `self.HeavyAttackMultiplier` 1.0)
  (if (`self.bCanAttack`)
    (set `self.bCanAttack` false)
    (`|SpawnActorFromClass` "/Game/Blueprints/WeaponProjectiles/BP_MagicBall.BP_MagicBall_C" (`KismetMathLibrary.MakeTransform` (+ (* (`Actor.GetActorForwardVector` _returnvalue) 80.0) (`Actor.K2_GetActorLocation` _returnvalue)) (`Actor.K2_GetActorRotation` _returnvalue)) "Undefined" "MultiplyWithRoot" _returnvalue 1.0 null)
    (`KismetSystemLibrary.K2_SetTimerDelegate` (delegate `RangedCooldown`) (`self.AttackCooldown`))))

(event `RangedCooldown`
  ;[0 0.15 0.147 0.502] Staff Attack Logic
  (set `self.bCanAttack` true))

(event `self.HeavyAttack`
  (bind _returnvalue (`self.GetOwner`))
  (bind _spellamount (`self.SpellAmount`))
  (bind _returnvalue_2 (`Actor.GetComponentByClass` _returnvalue "/Script/Engine.ArrowComponent"))
  (bind (_returnvalue_roll _returnvalue_pitch _returnvalue_yaw) (`KismetMathLibrary.BreakRotator` (`SceneComponent.K2_GetComponentRotation` _returnvalue_2)))
  ;[0 0.15 0.147 0.502] Heavy Attack - Logic inspired by Lich
  (set `self.HeavyAttackMultiplier` 1.5)
  (if (`self.bCanAttack`)
    (set `self.bCanAttack` false)
    (for _index (range (* _spellamount -1) (+ _spellamount 1))
      (`|SpawnActorFromClass` "/Game/Blueprints/WeaponProjectiles/BP_MagicBall.BP_MagicBall_C" (`KismetMathLibrary.MakeTransform` (+ (* (`Actor.GetActorForwardVector` _returnvalue) 80.0) (+ (`SceneComponent.K2_GetComponentLocation` _returnvalue_2) (* (`SceneComponent.GetRightVector` _returnvalue_2) (* _index 50)))) (`KismetMathLibrary.MakeRotator` _returnvalue_roll _returnvalue_pitch (+ _returnvalue_yaw (* _index 10)))) "Undefined" "MultiplyWithRoot" _returnvalue (`self.HeavyAttackMultiplier`) null)
      (`KismetSystemLibrary.K2_SetTimerDelegate` (delegate `HeavyCooldown`) (`self.AttackCooldown`)))))

(event `HeavyCooldown`
  ;[0 0.15 0.147 0.502] Heavy Attack - Logic inspired by Lich
  (set `self.bCanAttack` true))