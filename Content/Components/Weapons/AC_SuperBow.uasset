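; AC_SuperBow is a weapon component that gives its owner a ranged bow light attack.
; LightAttack spawns a BP_BulletArrow a short distance in front of the owner, facing the owner's rotation, as a placeholder for the bow's own location.
; A CanAttack flag gates firing, and a timer calls RangedCooldown to re-enable it after AttackCooldown.
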(event `self.LightAttack`
  (bind _returnvalue (`self.GetOwner`))
  ;[0 0.15 0.147 0.502] Bow Attack Logic
  (if (`self.bCanAttack`)
    (set `self.bCanAttack` false)
    (`|SpawnActorFromClass` "/Game/Blueprints/WeaponProjectiles/BP_BulletArrow.BP_BulletArrow_C" (`KismetMathLibrary.MakeTransform` (+ (* (`Actor.GetActorForwardVector` _returnvalue) 80.0) (`Actor.K2_GetActorLocation` _returnvalue)) (`Actor.K2_GetActorRotation` _returnvalue)) "Undefined" "MultiplyWithRoot" (`self.GetOwner`) null)
    (`KismetSystemLibrary.K2_SetTimerDelegate` (delegate `RangedCooldown`) (`self.AttackCooldown`))))

(event `RangedCooldown`
  (set `self.bCanAttack` true))