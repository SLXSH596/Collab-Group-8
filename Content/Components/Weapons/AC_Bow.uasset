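; AC_Bow is a weapon component that gives its owning actor ranged bow attacks.
; Light and heavy attacks share one firing path, differing only in a damage-style multiplier passed to the spawned BP_Arrow.
; The arrow spawns just ahead of the owner along its forward vector, a placeholder until a bow location exists.
; A timer-driven cooldown gates firing through a CanAttack flag.
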(event `self.LightAttack`
  (bind _returnvalue (`self.GetOwner`))
  ;[0 0.15 0.147 0.502] Bow Attack Logic
  (set `self.HeavyAttackMultiplier` 1.0)
  (if (`self.bCanAttack`) :!label _label
    (set `self.bCanAttack` false)
    (`|SpawnActorFromClass` "/Game/Blueprints/WeaponProjectiles/BP_Arrow.BP_Arrow_C" (`KismetMathLibrary.MakeTransform` (+ (* (`Actor.GetActorForwardVector` _returnvalue) 80.0) (`Actor.K2_GetActorLocation` _returnvalue)) (`Actor.K2_GetActorRotation` _returnvalue)) "Undefined" "MultiplyWithRoot" (`self.GetOwner`) (`self.HeavyAttackMultiplier`) null)
    (`KismetSystemLibrary.K2_SetTimerDelegate` (delegate `RangedCooldown`) (`self.AttackCooldown`))))

(event `self.HeavyAttack`
  ;[0 0.15 0.147 0.502] Bow Attack Logic
  (set `self.HeavyAttackMultiplier` 3.0)
  (goto _label))

(event `RangedCooldown`
  ;[0 0.15 0.147 0.502] Bow Attack Logic
  (set `self.bCanAttack` true))