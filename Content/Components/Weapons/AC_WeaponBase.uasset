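; Base weapon component for players, providing shared light and heavy attack events intended for child weapons to inherit.
; Initialisation caches the player and controller; staff and sword triggers share paths that play controller rumble, then fire the matching attack event.
; Attack events broadcast OnLightAttack or OnHeavyAttack, while StopAttack is an empty hook for ending auto or charge attacks.
; FriendlyFireCheck flags hits on actors whose class is exactly BP_Player.
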(event `Initialisation`
  (params (Player :type "/Game/Blueprints/Player/BP_Player Object Reference"))
  (bind _output_get (set `self.Player` Player))
  (set `self.Player Controller` (`/Game/Blueprints/Player/BP_Player.PlayerController` _output_get)))

(event `HeavyAttack`
  (`self.OnHeavyAttack`))

(event `/Game/Interfaces/BPI_PlayerCombatPass.StaffLightTrigger`
  (`/Game/Components/Controllers/AC_ControllerRumble.Light Attack FF` (`/Game/Blueprints/Player/PC_PlayerController.AC_ControllerRumble` (`self.Player Controller`)) :!label _label)
  (`self.LightAttack`))

(event `/Game/Interfaces/BPI_PlayerCombatPass.SwordLightTrigger`
  (goto _label))

(event `LightAttack`
  ;[0 0.15 0.147 0.502] Inherited Attack Event
  (`self.OnLightAttack`))

(event `/Game/Interfaces/BPI_PlayerCombatPass.StaffHeavyTrigger`
  (`/Game/Components/Controllers/AC_ControllerRumble.Heavy Attack FF` (`/Game/Blueprints/Player/PC_PlayerController.AC_ControllerRumble` (`self.Player Controller`)) :!label _label_2)
  (`self.HeavyAttack`))

(event `/Game/Interfaces/BPI_PlayerCombatPass.SwordHeavyTrigger`
  (goto _label_2))

(event `StopAttack`
  ;[0 0.15 0.147 0.502] For stopping auto attacks OR charge attacks
)

(fn `FriendlyFireCheck`
  (params (Hit :type "HitResult Structure (by ref)"))
  (returns (HitActor :type "Actor Object Reference") (bWasFriendlyFire :type Boolean))
  (bind (_bblockinghit _binitialoverlap _time _distance _location _impactpoint _normal _impactnormal _physmat _hitactor) (`GameplayStatics.BreakHitResult` Hit))
  (if (== (`GameplayStatics.GetObjectClass` _hitactor) "/Game/Blueprints/Player/BP_Player.BP_Player_C")
    (return _hitactor true)
    (else
      (return _hitactor false))))