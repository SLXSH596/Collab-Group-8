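; Sword weapon component that gives its owning actor light and heavy melee attacks.
; Each attack spawns a Niagara slash, then sphere-traces ahead of the owner, with heavy attacks using a larger area and doubled damage.
; Hits deal sword-type damage with an impact effect, while friendly-fire hits take scaled damage without one.
; A shared CanAttack flag and timer enforce the cooldown between attacks.
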(event `self.HeavyAttack`
  (bind _returnvalue (`self.GetOwner`))
  (bind _returnvalue_2 (`self.GetOwner`))
  (bind _returnvalue_3 (`self.GetOwner`))
  (bind _returnvalue_4 (`Actor.K2_GetActorLocation` _returnvalue))
  ;[0 0.15 0.147 0.502] Sword Attack Logic
  (set `self.HeavyAttackMultiplier` 2.0)
  (if (`self.bCanAttack`)
    (set `self.bCanAttack` false)
    (`NiagaraFunctionLibrary.SpawnSystemAttached` "/Game/VFX/NiagaraSystem/NS_SwordSlash_Giant.NS_SwordSlash_Giant" (`Actor.RootComponent` _returnvalue_3) "None" (- (+ (`Actor.K2_GetActorLocation` _returnvalue_3) (* (`Actor.GetActorForwardVector` _returnvalue_3) 50.0)) (0.0 0.0 40.0)) (`Actor.K2_GetActorRotation` _returnvalue_3) "KeepWorldPosition" true)
    (bind (_outhits _returnvalue_5) (`KismetSystemLibrary.SphereTraceMultiForObjects` (+ (* (`Actor.GetActorForwardVector` _returnvalue) (* (`self.AttackRange`) 1.75)) _returnvalue_4) _returnvalue_4 225.0 (`self.DefaultObjectType`) false (`|MakeArray` _returnvalue) "ForOneFrame"))
    (if _returnvalue_5
      (for _array_element _outhits
        (bind (_hitactor _bwasfriendlyfire) (`self.FriendlyFireCheck` _array_element))
        (if (not _bwasfriendlyfire)
          (`GameplayStatics.ApplyDamage` _hitactor (* (`self.HeavyAttackMultiplier`) (`self.BaseDamage`)) null _returnvalue_2 "/Game/Blueprints/WeaponDamageTypes/BP_DamageType_Sword.BP_DamageType_Sword_C")
          (`NiagaraFunctionLibrary.SpawnSystemAtLocation` "/Game/VFX/NiagaraSystem/NS_Sword_Impact.NS_Sword_Impact" (`.ImpactPoint` (`GameplayStatics.BreakHitResult` _array_element)) (`Actor.K2_GetActorRotation` (`self.GetOwner`)))
          (else
            (`GameplayStatics.ApplyDamage` _hitactor (* (* (`self.HeavyAttackMultiplier`) (`self.BaseDamage`)) (`self.FriendlyFireMultiplier`)) null _returnvalue_2 "/Game/Blueprints/WeaponDamageTypes/BP_DamageType_Sword.BP_DamageType_Sword_C")))))
    (`KismetSystemLibrary.K2_SetTimerDelegate` (delegate `MeleeCooldown`) (`self.AttackCooldown`))))

(event `MeleeCooldown`
  ;[0 0.15 0.147 0.502] Sword Attack Logic
  (set `self.bCanAttack` true))

(event `self.LightAttack`
  (bind _returnvalue (`self.GetOwner`))
  (bind _returnvalue_2 (`self.GetOwner`))
  (bind _returnvalue_3 (`self.GetOwner`))
  (bind _returnvalue_4 (`Actor.K2_GetActorLocation` _returnvalue_3))
  ;[0 0.15 0.147 0.502] Sword Attack Logic
  (set `self.HeavyAttackMultiplier` 1.0)
  (if (`self.bCanAttack`)
    (set `self.bCanAttack` false)
    (`NiagaraFunctionLibrary.SpawnSystemAttached` "/Game/VFX/NiagaraSystem/NS_SwordSlash_Slowed.NS_SwordSlash_Slowed" (`Actor.RootComponent` _returnvalue_2) "None" (- (+ (`Actor.K2_GetActorLocation` _returnvalue_2) (* (`Actor.GetActorForwardVector` _returnvalue_2) 50.0)) (0.0 0.0 40.0)) (`Actor.K2_GetActorRotation` _returnvalue_2) "KeepWorldPosition" true)
    (bind (_outhits _returnvalue_5) (`KismetSystemLibrary.SphereTraceMultiForObjects` (+ (* (`Actor.GetActorForwardVector` _returnvalue_3) (`self.AttackRange`)) _returnvalue_4) (+ _returnvalue_4 (* (`Actor.GetActorForwardVector` _returnvalue_3) 90.0)) 100.0 (`self.DefaultObjectType`) false (`|MakeArray` _returnvalue_3)))
    (if _returnvalue_5
      (for _array_element _outhits
        (bind (_hitactor _bwasfriendlyfire) (`self.FriendlyFireCheck` _array_element))
        (if (not _bwasfriendlyfire)
          (`GameplayStatics.ApplyDamage` _hitactor (* (`self.HeavyAttackMultiplier`) (`self.BaseDamage`)) null _returnvalue "/Game/Blueprints/WeaponDamageTypes/BP_DamageType_Sword.BP_DamageType_Sword_C")
          (`NiagaraFunctionLibrary.SpawnSystemAtLocation` "/Game/VFX/NiagaraSystem/NS_Sword_Impact.NS_Sword_Impact" (`.ImpactPoint` (`GameplayStatics.BreakHitResult` _array_element)) (`Actor.K2_GetActorRotation` (`self.GetOwner`)))
          (else
            (`GameplayStatics.ApplyDamage` _hitactor (* (* (`self.HeavyAttackMultiplier`) (`self.BaseDamage`)) (`self.FriendlyFireMultiplier`)) null _returnvalue "/Game/Blueprints/WeaponDamageTypes/BP_DamageType_Sword.BP_DamageType_Sword_C")))))
    (`KismetSystemLibrary.K2_SetTimerDelegate` (delegate `CustomEvent`) (`self.AttackCooldown`))))

(event `CustomEvent`
  ;[0 0.15 0.147 0.502] Sword Attack Logic
  (set `self.bCanAttack` true))