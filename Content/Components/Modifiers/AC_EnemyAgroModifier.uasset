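; AC_EnemyAgroModifier is a modifier component that manages which player the enemies target for aggro.
; On initialisation it stores the enemy manager, gathers all BP_Player actors and picks one at random as the target.
; It notifies every player, passing itself and whether that player is the target.
; A change-target event stores the new target and forwards it to the enemy manager.
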(event `InitialiseEnemyAgro`
  (params (EnemyManager :type "/Game/Components/GameMode/AC_EnemyManager Object Reference"))
  (set `self.EnemyManager` EnemyManager)
  (bind _outactors (`GameplayStatics.GetAllActorsOfClass` "/Game/Blueprints/Player/BP_Player.BP_Player_C"))
  (bind _output_get (set `self.Players` _outactors))
  (set `self.PlayerTarget` (`KismetArrayLibrary.Array_Random` _output_get))
  (for _array_element (`self.Players`)
    (`/Game/Blueprints/Player/BP_Player.EnemyAgroModifier` _array_element self (== _array_element (`self.PlayerTarget`)))))

(event `ChangeEnemyTarget`
  (params (`New Target` :type "Actor Object Reference"))
  (bind _output_get (set `self.PlayerTarget` `New Target`))
  (`/Game/Components/GameMode/AC_EnemyManager.ChangeEnemyTarget` (`self.EnemyManager`) _output_get))