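; Arrow Hell modifier component that replaces every player's weapon with a super bow.
; Shortly after BeginPlay, it gathers all BP_Player actors, overrides their chosen weapon type and rebuilds the equipped weapon.
; It binds to the game mode's OnEndPlay to restore weapons from each player's ModifierSaveWeapon, which this component reads but never writes.
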(event `self.ReceiveBeginPlay`
  ;[0 0.15 0.147 0.502] Begin Play Logic - Replaces the player weapon with a super bow, returns weapon on game mode end play called
  (bind _asbp_gamemode (cast `/Game/Blueprints/Player/BP_Gamemode` (`GameplayStatics.GetGameMode`)))
  (bind _output_get (set `self.As BP Gamemode` _asbp_gamemode))
  (add `Actor.OnEndPlay` _output_get (delegate `Return Weapons`))
  (`KismetSystemLibrary.Delay` 0.2)
  (bind _outactors (`GameplayStatics.GetAllActorsOfClass` "/Game/Blueprints/Player/BP_Player.BP_Player_C"))
  (bind _output_get_2 (set `self.Players` _outactors))
  (for _array_element _output_get_2
    (set `/Game/Blueprints/Player/BP_Player.ChosenWeaponType` "NewEnumerator4" _array_element)
    (`/Game/Blueprints/Player/BP_Player.Remove Current Weapon` _array_element)
    (`/Game/Blueprints/Player/BP_Player.CheckWeapon` _array_element)
    (`/Game/Blueprints/Player/BP_Player.SetCurrentWeapon` _array_element)))

(event `Return Weapons`
  (params (Actor :type "Actor Object Reference") (EndPlayReason :type "EEndPlayReason Enum" :default "Destroyed"))
  ;[0 0.15 0.147 0.502] Begin Play Logic - Replaces the player weapon with a super bow, returns weapon on game mode end play called
  (for _array_element _
    (set `/Game/Blueprints/Player/BP_Player.ChosenWeaponType` (`/Game/Blueprints/Player/BP_Player.ModifierSaveWeapon` _array_element) _array_element)
    (`/Game/Blueprints/Player/BP_Player.Remove Current Weapon` _array_element)
    (`/Game/Blueprints/Player/BP_Player.CheckWeapon` _array_element)
    (`/Game/Blueprints/Player/BP_Player.SetCurrentWeapon` _array_element)))