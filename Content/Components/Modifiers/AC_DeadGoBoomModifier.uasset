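; AC_DeadGoBoomModifier is a gameplay modifier component for the Game Mode that makes enemies leave a bomb when destroyed.
; On BeginPlay it looks for AC_EnemyManager on its owner and, if present, binds to its enemy-spawned event.
; Each spawned enemy gets its OnDestroyed event bound, which spawns a BP_Bomb at the destroyed actor's transform.
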(event `self.ReceiveBeginPlay`
  (bind _returnvalue (`Actor.GetComponentByClass` (`self.GetOwner`) "/Game/Components/GameMode/AC_EnemyManager.AC_EnemyManager_C"))
  ;[0 0.15 0.147 0.502] Begin Play Logic - Checks Enemy Spawning in the Enemy Manager, this attaches to Game Mode
  (`/Engine/EditorBlueprintResources/StandardMacros.IsValid` _returnvalue
    (:`Is Valid`
      (add `/Game/Components/GameMode/AC_EnemyManager.OnEnemySpawned` _returnvalue (`|CreateDelegate` :!event `Enemy Spawned`)))))

(event `Enemy Spawned`
  (params (SpawnedEnemy :type "/Game/AI/AIActors/BP_BaseEnemy Object Reference"))
  ;[0 0.15 0.147 0.502] Attaches the Explosive Component to the enemy
  (add `Actor.OnDestroyed` SpawnedEnemy (`|CreateDelegate` :!event `Spawn Bomb`)))

(event `Spawn Bomb`
  (params (DestroyedActor :type "Actor Object Reference"))
  ;[0 0.15 0.147 0.502] Attaches the Explosive Component to the enemy
  (`|SpawnActorFromClass` "/Game/Blueprints/Hazards/BP_Bomb.BP_Bomb_C" (`Actor.GetTransform` DestroyedActor) "Undefined" "MultiplyWithRoot" null null))