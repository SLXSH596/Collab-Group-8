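; AC_PoisonBomb is a modifier component that makes enemies leave a poison bomb where they are destroyed.
; On BeginPlay it looks for an AC_EnemyManager on its owner and subscribes to that manager's enemy-spawned event.
; Each newly spawned enemy gets its OnDestroyed event bound, which spawns a BP_PosionBomb at the destroyed actor's transform.
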(event `self.ReceiveBeginPlay`
  (bind _returnvalue (`Actor.GetComponentByClass` (`self.GetOwner`) "/Game/Components/GameMode/AC_EnemyManager.AC_EnemyManager_C"))
  (`/Engine/EditorBlueprintResources/StandardMacros.IsValid` _returnvalue
    (:`Is Valid`
      (add `/Game/Components/GameMode/AC_EnemyManager.OnEnemySpawned` _returnvalue (`|CreateDelegate` :!event `EnemySpawned`)))))

(event `EnemySpawned`
  (params (SpawnedEnemy :type "/Game/AI/AIActors/BP_BaseEnemy Object Reference"))
  (add `Actor.OnDestroyed` SpawnedEnemy (`|CreateDelegate` :!event `Spawn Bomb`)))

(event `Spawn Bomb`
  (params (DestroyedActor :type "Actor Object Reference"))
  (`|SpawnActorFromClass` "/Game/Blueprints/Hazards/BP_PosionBomb.BP_PosionBomb_C" (`Actor.GetTransform` DestroyedActor) "Undefined" "MultiplyWithRoot" null null))