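; AC_AutoDashModifier is a game modifier component that makes players dash automatically.
; On BeginPlay it caches all BP_Player actors and sets the auto-dash and cooldown-active flags on each one's dash ability.
; A looping timer, with its interval randomized once at start, then triggers an auto dash on every living cached player at the same time.
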(event `self.ReceiveBeginPlay`
  (bind _outactors (`GameplayStatics.GetAllActorsOfClass` "/Game/Blueprints/Player/BP_Player.BP_Player_C"))
  (bind _output_get (set `self.Players` _outactors))
  (for _array_element _output_get
    (bind _ac_dashability (`/Game/Blueprints/Player/BP_Player.AC_DashAbility` _array_element))
    (set `/Game/Components/Pawns/AC_DashAbility.DashCooldownActive?` true _ac_dashability)
    (set `/Game/Components/Pawns/AC_DashAbility.AutoDash?` true _ac_dashability))
  (`KismetSystemLibrary.K2_SetTimerDelegate` (delegate `CallDash`) (`KismetMathLibrary.RandomFloatInRange` 2.0 8.0) true))

(event `CallDash`
  (for _array_element (`self.Players`)
    (bind _isdead (`/Game/Interfaces/BPI_PlayerInterface.IsDead` _array_element))
    (if (not _isdead)
      (`/Game/Components/Pawns/AC_DashAbility.Activate Auto Dash` (`/Game/Blueprints/Player/BP_Player.AC_DashAbility` _array_element)))))