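; AC_DoubleTroubleModifier is a wave modifier component that scales enemy health and enemy counts on its owner's AC_EnemyManager.
; InitialiseOnEM multiplies the manager's SpawnedHealthMult by the health multiplier, then scales each spawn entry's EnemyCount in DEBUGWaves by a separate multiplier.
; Nested loops edit each wave struct and write it back into the manager's array, followed by a leftover "Hello" debug print.
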(event `InitialiseOnEM`
  (bind _returnvalue (`Actor.GetComponentByClass` (`self.GetOwner`) "/Game/Components/GameMode/AC_EnemyManager.AC_EnemyManager_C"))
  (bind _debug_waves (`/Game/Components/GameMode/AC_EnemyManager.DEBUG_Waves` _returnvalue))
  ;[0.162 0.02956 0.3515] Change the health multiplier
  (`/Engine/EditorBlueprintResources/StandardMacros.IsValid` _returnvalue
    (:`Is Valid`
      (set `/Game/Components/GameMode/AC_EnemyManager.SpawnedHealthMult` (* (`/Game/Components/GameMode/AC_EnemyManager.SpawnedHealthMult` _returnvalue) (`self.ModifierHealthMultiplier`)) _returnvalue)
      ;[0.162 0.02956 0.3515] Loop through each wave
      (for (_array_element _array_index) _debug_waves
        (bind _output_get (set `self.CurrentWave` _array_element))
        (bind ((`EnemySpawnInfo_14_BF26838A45C7CF396F4185A1AC63EDEF` _enemyspawninfo)) (break `/Game/Blueprints/Data/EnemySpawning/F_EnemyWaveData` _output_get))
        ;[0.162 0.02956 0.3515] Multiply the enemy count of each enemy type for the wave
        (for (_array_element_2 _array_index_2) _enemyspawninfo
          (bind _structout (setmembers `/Game/Blueprints/Data/EnemySpawning/F_EnemySpawnInfo` :`StructRef` _array_element_2 :`Enemy Count` (* (`.EnemyCount_14_8DBA91B14E65D1458EAE12AF7376EF0B` (break `/Game/Blueprints/Data/EnemySpawning/F_EnemySpawnInfo` _array_element_2)) (`self.ModifierMultiplier`))))
          (`KismetArrayLibrary.Array_Set` _enemyspawninfo _array_index_2 _structout))
        (`KismetArrayLibrary.Array_Set` _debug_waves _array_index _output_get))
      (`KismetSystemLibrary.PrintString` "Hello"))))