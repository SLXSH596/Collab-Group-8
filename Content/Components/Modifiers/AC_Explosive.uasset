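; AC_Explosive is a modifier component attached to enemies on spawn that makes them explode when destroyed.
; On BeginPlay it binds to the owner's OnDestroyed event to trigger DeathSplosion.
; The explosion runs a zero-length multi sphere trace at the owner's location and applies explosive-type damage to each blocking hit, with the destroyed actor as causer.
; The trace's debug drawing is left on persistent.
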(event `self.ReceiveBeginPlay`
  ;[0 0.15 0.147 0.502] ACM_Explosive: Attached to enemies on spawn
  ;;[0 0.15 0.147 0.502] Binds to destroy event
  (add `Actor.OnDestroyed` (`self.GetOwner`) (`|CreateDelegate` :!event `DeathSplosion`)))

(event `DeathSplosion`
  (params (DestroyedActor :type "Actor Object Reference"))
  (bind _returnvalue (`Actor.K2_GetActorLocation` (`self.GetOwner`)))
  ;[0 0.15 0.147 0.502] ACM_Explosive: Attached to enemies on spawn
  ;;[0 0.15 0.147 0.502] Explosion triggers on death
  (bind _outhits (`KismetSystemLibrary.SphereTraceMultiForObjects` :`Start` _returnvalue :`End` _returnvalue :`Radius` 300.0 :`ObjectTypes` (`self.DefaultObjects`) :`DrawDebugType` "Persistent"))
  (for _array_element _outhits
    (bind (_bblockinghit _binitialoverlap _time _distance _location _impactpoint _normal _impactnormal _physmat _hitactor) (`GameplayStatics.BreakHitResult` _array_element))
    (if _bblockinghit
      (`GameplayStatics.ApplyDamage` _hitactor 1.0 null DestroyedActor "/Game/Blueprints/WeaponDamageTypes/BP_DamageType_Explosive.BP_DamageType_Explosive_C"))))