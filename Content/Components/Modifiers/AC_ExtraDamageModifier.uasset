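; AC_ExtraDamageModifier is a modifier component that scales both enemy and player damage by a shared multiplier.
; On BeginPlay, if its owner has an AC_EnemyManager, it multiplies that manager's spawned damage multiplier by the modifier value.
; Within the same check, it finds every BP_Player and multiplies the base damage of their current weapon.
; The change is applied once, with no update for later weapons and no revert.
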(event `self.ReceiveBeginPlay`
  (bind _returnvalue (`Actor.GetComponentByClass` (`self.GetOwner`) "/Game/Components/GameMode/AC_EnemyManager.AC_EnemyManager_C"))
  (`/Engine/EditorBlueprintResources/StandardMacros.IsValid` _returnvalue
    (:`Is Valid`
      (set `/Game/Components/GameMode/AC_EnemyManager.SpawnedDmgMult` (* (`/Game/Components/GameMode/AC_EnemyManager.SpawnedDmgMult` _returnvalue) (`self.ModifierDamageMultiplier`)) _returnvalue)
      (bind _outactors (`GameplayStatics.GetAllActorsOfClass` "/Game/Blueprints/Player/BP_Player.BP_Player_C"))
      (for _array_element _outactors
        (bind _currentweapon (`/Game/Blueprints/Player/BP_Player.CurrentWeapon` _array_element))
        (`/Engine/EditorBlueprintResources/StandardMacros.IsValid` _currentweapon
          (:`Is Valid`
            (set `/Game/Components/Weapons/AC_WeaponBase.BaseDamage` (* (`/Game/Components/Weapons/AC_WeaponBase.BaseDamage` _currentweapon) (`self.ModifierDamageMultiplier`)) _currentweapon)))))))