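; Modifier component that speeds up both enemies and players by a shared speed multiplier.
; On InitialiseOnEM it finds the owner's AC_EnemyManager and scales its spawned-enemy speed multiplier.
; If that manager exists, it also scales every BP_Player's max walk speed, stores the result as WalkSpeed, and divides the current weapon's attack cooldown by the same factor.
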(event `InitialiseOnEM`
  (bind _returnvalue (`Actor.GetComponentByClass` (`self.GetOwner`) "/Game/Components/GameMode/AC_EnemyManager.AC_EnemyManager_C"))
  (`/Engine/EditorBlueprintResources/StandardMacros.IsValid` _returnvalue
    (:`Is Valid`
      (set `/Game/Components/GameMode/AC_EnemyManager.SpawnedSpeedMult` (* (`/Game/Components/GameMode/AC_EnemyManager.SpawnedSpeedMult` _returnvalue) (`self.ModifierSpeedMultiplier`)) _returnvalue)
      (bind _outactors (`GameplayStatics.GetAllActorsOfClass` "/Game/Blueprints/Player/BP_Player.BP_Player_C"))
      (for _array_element _outactors
        (bind _charactermovement (`Character.CharacterMovement` _array_element))
        (`/Engine/EditorBlueprintResources/StandardMacros.IsValid` _charactermovement
          (:`Is Valid`
            (bind _output_get (set `CharacterMovementComponent.MaxWalkSpeed` (* (`CharacterMovementComponent.MaxWalkSpeed` _charactermovement) (`self.ModifierSpeedMultiplier`)) _charactermovement))
            (set `/Game/Blueprints/Player/BP_Player.WalkSpeed` _output_get _array_element)
            (bind _currentweapon (`/Game/Blueprints/Player/BP_Player.CurrentWeapon` _array_element))
            (`/Engine/EditorBlueprintResources/StandardMacros.IsValid` _currentweapon
              (:`Is Valid`
                (set `/Game/Components/Weapons/AC_WeaponBase.AttackCooldown` (/ (`/Game/Components/Weapons/AC_WeaponBase.AttackCooldown` _currentweapon) (`self.ModifierSpeedMultiplier`)) _currentweapon)))))))))