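; Actor component that marks an object as interactable and broadcasts when a player interacts with it.
; On BeginPlay it casts its owner to BP_BasePickup and caches that as its Pickup reference.
; Interact prints a debug message naming the owner of the passed Player, then fires the OnInteracted dispatcher with that Player, leaving the response to bound listeners.
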(event `self.ReceiveBeginPlay`
  ;[0.4793 0.05127 0.0648] Initalises Pickup References
  (`self.Initialise`))

(fn `Initialise`
  ;[0.4793 0.05127 0.0648] Function called
  ;[0.4793 0.05127 0.0648] Create reference to the Pickup Class
  (bind _asbp_base_pickup (cast `/Game/Blueprints/Pickup/BP_BasePickup` (`self.GetOwner`)))
  (set `self.Pickup` _asbp_base_pickup))

(fn `Interact`
  (params (Player :type "/Game/Blueprints/Player/BP_Player Object Reference"))
  ;[0.4793 0.05127 0.0648] Function called
  ;[0.4793 0.05127 0.0648] DEBUG: Prints which Player Character sucessfully interacted
  (`KismetSystemLibrary.PrintString` (`KismetStringLibrary.Concat_StrStr` "Player: " (`KismetSystemLibrary.GetDisplayName` (`Actor.GetOwner` Player)) " interacted!"))
  ;[0.4793 0.05127 0.0648] Calls the Event Dispatcher "OnInteracted"
  (`self.OnInteracted` Player))