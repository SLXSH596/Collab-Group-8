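; Transition component that handles the loading screen and fades the level's directional light in and out around level changes.
; Initialise caches the light's intensity then dims it, and the loading screen shows for a given duration before collecting garbage, notifying the Gamemode and starting the entry fade.
; Looping timers step the intensity, with a ratio-scaled ramp up on entry and a linear drop on exit before GameInstance selects the next level.
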(event `Initialise`
  (params (GameInstance :type "/Game/Blueprints/GI_GameInstance Object Reference") (Gamemode :type "/Game/Blueprints/Player/BP_Gamemode Object Reference"))
  ;[1 0.004025 0.7835] Initialiser
  (set `self.Gamemode` Gamemode)
  (set `self.Game Instance` GameInstance)
  (bind _returnvalue (`GameplayStatics.GetActorOfClass` "/Script/Engine.DirectionalLight"))
  (bind _output_get (set `self.Light` _returnvalue))
  (bind _lightcomponent (`Light.LightComponent` _output_get))
  (set `self.Intensity` (`LightComponentBase.Intensity` _lightcomponent))
  (`KismetSystemLibrary.DelayUntilNextTick`)
  (`LightComponent.SetIntensity` _lightcomponent 0.25))

(event `StartEntryTransition`
  ;[1 0.004025 0.7835] Start Entry Transition
  (bind _returnvalue (`KismetSystemLibrary.K2_SetTimerDelegate` (delegate `EntryTransition`) 0.1 true))
  (set `self.StartTimer` _returnvalue))

(event `StartLoadScreen`
  (params (duration :type "Float (double-precision)"))
  (bind _gamemode (`self.Gamemode`))
  ;[1 0.004025 0.7835] Create Loading Screen
  (bind _returnvalue (`|CreateWidget` "/Game/UI/WBP_LoadingScreen.WBP_LoadingScreen_C" (`GameplayStatics.GetPlayerController` 0)))
  (`UserWidget.AddToViewport` _returnvalue 0)
  (`KismetSystemLibrary.Delay` duration)
  (`Widget.RemoveFromParent` _returnvalue)
  (`KismetSystemLibrary.CollectGarbage`)
  (`/Engine/EditorBlueprintResources/StandardMacros.IsValid` _gamemode
    (:`Is Valid`
      (`/Game/Blueprints/Player/BP_Gamemode.FinishedLoad` _gamemode (`self.Initialise Delay`)))
    (:`Is Not Valid`
      _))
  (`self.LoadFinished`)
  (`self.StartEntryTransition`))

(event `EntryTransition`
  (bind _lightcomponent (`Light.LightComponent` (`self.Light`)))
  (bind _intensity (`LightComponentBase.Intensity` _lightcomponent))
  ;[1 0.004025 0.7835] Entry Transition
  (if (>= _intensity (`self.Intensity`))
    (`KismetSystemLibrary.K2_ClearAndInvalidateTimerHandle` (`self.StartTimer`))
    (else
      (`LightComponent.SetIntensity` _lightcomponent (+ _intensity (* (`KismetMathLibrary.FClamp` (* (/ _intensity (`self.Intensity`)) 2.0) 0.1) (`KismetMathLibrary.Abs` 0.25)))))))

(event `StartExitTransition`
  ;[1 0.004025 0.7835] Start Exit Transition
  (bind _returnvalue (`KismetSystemLibrary.K2_SetTimerDelegate` (delegate `Exit Transition`) 0.1 true))
  (set `self.ExitTimer` _returnvalue))

(event `Exit Transition`
  (bind _lightcomponent (`Light.LightComponent` (`self.Light`)))
  (bind _intensity (`LightComponentBase.Intensity` _lightcomponent))
  ;[1 0.004025 0.7835] Exist Transition
  (if (<= _intensity 0.5)
    (`KismetSystemLibrary.K2_ClearAndInvalidateTimerHandle` (`self.ExitTimer`))
    (`KismetSystemLibrary.Delay` 1.0)
    ;[1 0.004025 0.7835] Load Next Level
    (`/Game/Blueprints/GI_GameInstance.SelectNewLevel` (`self.Game Instance`))
    (else
      (`LightComponent.SetIntensity` _lightcomponent (- _intensity 0.5)))))