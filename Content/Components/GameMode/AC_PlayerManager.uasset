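; Game mode component that tracks how many players are alive and triggers game over when none remain.
; Initialise seeds the count from the GameInstance join count and binds to every BP_Player's health and respawn component events.
; Decrease and increase events adjust the clamped count, broadcasting OnGameOver at zero.
; The game-over sequence resets buffs and clears saved buff data through PlayerRef, a single reference rather than every player.
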(event `Initialise`
  ;[0.06301 0.6939 0.1441] Initialise
  (`self.AlivePlayers`)
  (bind _outactors (`GameplayStatics.GetAllActorsOfClass` "/Game/Blueprints/Player/BP_Player.BP_Player_C"))
  (for _array_element _outactors
    (bind _output_get (set `self.Player Ref` (cast `/Game/Blueprints/Player/BP_Player` _array_element :!pure true)))
    (set `self.Health Component` (`Actor.GetComponentByClass` _output_get "/Game/Components/Player/AC_HealthComponent.AC_HealthComponent_C"))
    (set `self.Respawn Component` (`Actor.GetComponentByClass` (`self.Player Ref`) "/Game/Components/Player/AC_Respawn.AC_Respawn_C"))
    (add `/Game/Components/Player/AC_HealthComponent.OnDeath` (`self.Health Component`) (`|CreateDelegate` :!event `Decrease Alive Players`))
    (add `/Game/Components/Player/AC_Respawn.OnRespawn` (`self.Respawn Component`) (`|CreateDelegate` :!event `Increase Alive Players`))
    (add `self.OnGameOver` (`|CreateDelegate` :!event `Game Over Sequence`))))

(event `Decrease Alive Players`
  (bind _alive_players (`self.Alive Players`))
  ;[0.06301 0.6939 0.1441] Update number of alive players
  (if (not (<= _alive_players 0))
    (bind _output_get (set `self.Alive Players` (`KismetMathLibrary.Clamp` (- _alive_players 1) 0 (`self.Player Num`))))
    (`KismetSystemLibrary.PrintString` (`KismetStringLibrary.Concat_StrStr` "Players Alive: " (`KismetStringLibrary.Conv_IntToString` _output_get)) true true (struct :`G` 0.66 :`B` 1.0 :`A` 1.0) 2.0 "5")
    ;[0.06301 0.6939 0.1441] Game Over
    (if (<= (`self.Alive Players`) 0)
      (`KismetSystemLibrary.PrintString` "GAME OVER" true true (struct :`R` 1.0 :`G` 0.813439 :`A` 1.0) 2.0 "6")
      (`self.OnGameOver`))))

(event `Increase Alive Players`
  ;[0.06301 0.6939 0.1441] Update number of alive players
  (bind _output_get (set `self.Alive Players` (`KismetMathLibrary.Clamp` (+ (`self.Alive Players`) 1) 0 (`self.Player Num`))))
  (`KismetSystemLibrary.PrintString` (`KismetStringLibrary.Concat_StrStr` "Players Alive: " (`KismetStringLibrary.Conv_IntToString` _output_get)) true true (struct :`G` 0.66 :`B` 1.0 :`A` 1.0) 2.0 "5"))

(event `Game Over Sequence`
  (bind _player_ref (`self.Player Ref`))
  ;[0.06301 0.6939 0.1441] Renamed: Game Over Sequence - Reset Player Stats (Note: Test with multiple players)
  (`/Game/Components/Player/AC_StatComponent.ResetPlayerBuffs` (`/Game/Blueprints/Player/BP_Player.AC_StatComponent` _player_ref))
  (`BlueprintMapLibrary.Map_Clear` (`/Game/Blueprints/GI_GameInstance.PlayerBuffData` (`/Game/Blueprints/Player/BP_Player.GameInstance` _player_ref))))

(fn `AlivePlayers`
  (bind _currentjoincount (`/Game/Blueprints/GI_GameInstance.CurrentJoinCount` (`/Game/Blueprints/Player/BP_Gamemode.GameInstance` (cast `/Game/Blueprints/Player/BP_Gamemode` (`GameplayStatics.GetGameMode`) :!pure true))))
  ;[0.06301 0.6939 0.1441] Number of players alive
  (set `self.Player Num` _currentjoincount)
  (bind _output_get (set `self.Alive Players` _currentjoincount))
  (`KismetSystemLibrary.PrintString` (`KismetStringLibrary.Concat_StrStr` "Players Alive: " (`KismetStringLibrary.Conv_IntToString` _output_get)) true true (struct :`G` 0.66 :`B` 1.0 :`A` 1.0) 2.0 "5"))