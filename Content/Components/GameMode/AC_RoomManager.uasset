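; AC_RoomManager is a game mode component, going by its folder, that handles what happens when a room is completed.
; Initialise stores the game mode and room exit references.
; RoomCompleted opens the exit through OpenDoor, then calls CallPickupEvent to look up the game mode's AC_PickupSpawning component.
; The SpawnPickups call at CentralPickupLocation is disconnected, so completing a room spawns no pickups from here.
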(event `Initialise`
  (params (Gamemode :type "/Game/Blueprints/Player/BP_Gamemode Object Reference") (RoomExit :type "/Game/Blueprints/LevelManagement/BP_RoomExitDoor Object Reference"))
  ;[0.162 0.02956 0.3515] Init
  (set `self.Gamemode` Gamemode)
  (set `self.RoomExit` RoomExit))

(event `Room Completed`
  ;[0.06301 0.6939 0.1441] On Room Completed
  (`self.Open Door`)
  (`self.Call Pickup Event`))

(event `Open Door`
  (bind _roomexit (`self.RoomExit`))
  ;[0.06301 0.6939 0.1441] Open Exit
  (`/Engine/EditorBlueprintResources/StandardMacros.IsValid` _roomexit
    (:`Is Valid`
      (`/Game/Blueprints/LevelManagement/BP_RoomExitDoor.Open Exit` _roomexit))))

(event `Call Pickup Event`
  ;[0.06301 0.6939 0.1441] Spawn Pickup
  (`/Engine/EditorBlueprintResources/StandardMacros.IsValid` (`Actor.GetComponentByClass` (`self.Gamemode`) "/Game/Components/GameMode/AC_PickupSpawning.AC_PickupSpawning_C")))