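; Game mode component that spawns pickups around a given location, one per local player controller.
; SpawnPickups places each BP_SpeedPickup at a point from GetRandomPointInRadius and prints its location; a TODO marks the fixed class for random selection.
; The random point offsets X and Y independently at a fixed height, so the spawn area is a square rather than a circle.
; Initialise only stores the GameMode reference.
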(event `Initialise`
  (params (GameMode :type "/Game/Blueprints/Player/BP_Gamemode Object Reference"))
  ;[0.162 0.02956 0.3515] Init
  (set `self.GameMode` GameMode))

(event `SpawnPickups`
  (params (SpawnLocation :type "Vector2D Structure") (SpawnRadius :type "Float (double-precision)"))
  ;[0.4793 0.05127 0.0648] Pickup spawning
  (for _index (range (`GameplayStatics.GetNumLocalPlayerControllers`))
    (bind _random_point (`self.GetRandomPointInRadius` SpawnLocation SpawnRadius))
    ;;[0.162 0.02956 0.3515] TODO: Replace with random logic
    (`|SpawnActorFromClass` "/Game/Blueprints/Pickup/BP_SpeedPickup.BP_SpeedPickup_C" (`KismetMathLibrary.MakeTransform` _random_point) "Undefined" "MultiplyWithRoot" null null)
    (`KismetSystemLibrary.PrintString` (`KismetStringLibrary.Concat_StrStr` "Pickup: " (`KismetStringLibrary.Conv_IntToString` _index) " , spawned at: " (`KismetStringLibrary.Conv_VectorToString` _random_point)))))

(fn `GetRandomPointInRadius`
  (params (Origin :type "Vector2D Structure") (Radius :type "Float (double-precision)"))
  (returns (`Random Point` :type "Vector Structure"))
  (bind (_x _y) (`KismetMathLibrary.BreakVector2D` Origin))
  (bind _returnvalue (* Radius -1.0))
  ;[0.162 0.02956 0.3515] Finds a random point in a 2D radius to spawn a pickup
  (return (`KismetMathLibrary.MakeVector` (+ _x (`KismetMathLibrary.RandomFloatInRange` _returnvalue Radius)) (+ _y (`KismetMathLibrary.RandomFloatInRange` _returnvalue Radius)) 150.0)))