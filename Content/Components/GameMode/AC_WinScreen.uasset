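; AC_WinScreen is a game mode component that shows the victory screen when a level is completed.
; On BeginPlay it creates and stores the WBP_WinScreen widget, then binds an event to OnLevelCompleted.
; DisplayWinScreen sets LevelCompleted and adds the widget to the viewport through a DoOnce gate.
; ResetOnLevelCompleted clears the flag and resets the gate, without removing the widget.
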(event `self.ReceiveBeginPlay`
  ;[0.06301 0.6939 0.1441] Win Screen Setup
  (bind _returnvalue (`|CreateWidget` "/Game/UI/WBP_WinScreen.WBP_WinScreen_C"))
  (set `self.WBP_WinScreen` _returnvalue)
  (add `self.OnLevelCompleted` (`|CreateDelegate` :!event `Display Win Screen`)))

(event `Display Win Screen`
  ;[0.06301 0.6939 0.1441] Display Victory Screen
  (`/Engine/EditorBlueprintResources/StandardMacros.DoOnce` false :!label _label
    (:`Completed`
      (set `self.LevelCompleted?` true)
      (`UserWidget.AddToViewport` (`self.WBP_WinScreen`) 0))))

(event `Reset On Level Completed`
  ;[0.06301 0.6939 0.1441] Reset Level Completed
  (set `self.LevelCompleted?` false)
  (goto _label :!via `Reset`))