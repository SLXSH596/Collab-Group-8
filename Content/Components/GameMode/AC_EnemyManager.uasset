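; Game mode component that runs a room's enemy waves and signals room completion when the last one dies.
; Init applies the first modifier component found, then scales enemy health and wave budget by room and player count.
; It pre-builds waves from random cost-weighted picks, with leaders bringing minions.
; A timer spawns each queue at navmesh points near placed markers or a fallback origin, and death events advance waves.
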(event `Init`
  ; Spawner Initialiser
  (`self.CheckModifiers`)
  (`self.CaculateEnemyMultiplier`)
  (`self.Build Waves`)
  (`self.GetSpawnLocations`)
  (`self.StartWave`))

(event `CheckModifiers`
  (bind _returnvalue (`Actor.GetComponentByClass` (`self.GetOwner`) "/Game/Components/Modifiers/AC_DoubleTroubleModifier.AC_DoubleTroubleModifier_C"))
  (bind _returnvalue_2 (`Actor.GetComponentByClass` (`self.GetOwner`) "/Game/Components/Modifiers/AC_EnemyAgroModifier.AC_EnemyAgroModifier_C"))
  (bind _returnvalue_3 (`Actor.GetComponentByClass` (`self.GetOwner`) "/Game/Components/Modifiers/AC_SuperSpeedModifier.AC_SuperSpeedModifier_C"))
  ; Handles Modifier Data
  (`/Engine/EditorBlueprintResources/StandardMacros.IsValid` (`Actor.GetComponentByClass` (`self.GetOwner`) "/Game/Components/Modifiers/AC_DeadGoBoomModifier.AC_DeadGoBoomModifier_C")
    (:`Is Valid`
      (set `self.bExplosiveEnemies` true))
    (:`Is Not Valid`
      (`/Engine/EditorBlueprintResources/StandardMacros.IsValid` (`Actor.GetComponentByClass` (`self.GetOwner`) "/Game/Components/Modifiers/AC_PoisonBombModifier.AC_PoisonBombModifier_C")
        (:`Is Valid`
          (set `self.bExplosiveEnemies` true))
        (:`Is Not Valid`
          (`/Engine/EditorBlueprintResources/StandardMacros.IsValid` _returnvalue
            (:`Is Valid`
              (`/Game/Components/Modifiers/AC_DoubleTroubleModifier.InitialiseOnEM` _returnvalue)
              (set `self.DoubleTroubleMult` 2.0))
            (:`Is Not Valid`
              (`/Engine/EditorBlueprintResources/StandardMacros.IsValid` _returnvalue_3
                (:`Is Valid`
                  (`/Game/Components/Modifiers/AC_SuperSpeedModifier.InitialiseOnEM` _returnvalue_3))
                (:`Is Not Valid`
                  (`/Engine/EditorBlueprintResources/StandardMacros.IsValid` _returnvalue_2
                    (:`Is Valid`
                      (set `self.EnemyAgroActive` true)
                      (`/Game/Components/Modifiers/AC_EnemyAgroModifier.InitialiseEnemyAgro` _returnvalue_2 self)
                      (set `self.PlayerTarget` (`/Game/Components/Modifiers/AC_EnemyAgroModifier.PlayerTarget` _returnvalue_2)))))))))))))

(event `SpawnNextEnemy`
  (bind _spawn_queue (`self.Spawn Queue`))
  (bind _current_spawn_index (`self.Current Spawn Index`))
  (bind _returnvalue (not (<= (`KismetArrayLibrary.Array_Length` (`self.EnemySpawnLocations`)) 0)))
  ;[0.4793 0.05127 0.0648] Spawn Enemy Wave (with spawn rate)
  (if (>= _current_spawn_index (`KismetArrayLibrary.Array_Length` _spawn_queue))
    ;;[0.4793 0.05127 0.0648] Stop Timer once Spawn Queue has been spawned
    (`KismetSystemLibrary.K2_ClearAndInvalidateTimerHandle` (`self.SpawnTimerHandle`))
    (else
      (if _returnvalue
        (bind _spawnlocation (`self.GetRandomPre-setSpawnLocation` 25.0))
        (else
          ;;[0.4793 0.05127 0.0648] Generate Random Spawn Point
          (bind _random_point (`self.GetRandomPointInRadius` (`self.SpawnOrigin`) (`self.SpawnRadius`)))))
      ;;[0.4793 0.05127 0.0648] Spawn next Enemy from the Spawn Queue, assign an OnEnemyDeath and add to list of Alive Enemies
      (bind _returnvalue_2 (`|SpawnActorFromClass` (`|GetArrayItem` _spawn_queue _current_spawn_index) (`KismetMathLibrary.MakeTransform` (`KismetMathLibrary.SelectVector` _spawnlocation _random_point _returnvalue)) "AdjustIfPossibleButAlwaysSpawn" "MultiplyWithRoot" null (* (`self.SpawnedHealthMult`) (`self.DifficultyHealthMult`)) (`self.SpawnedDmgMult`) (`self.SpawnedSpeedMult`) null))
      (bind _output_get (set `self.SpawnedEnemy` _returnvalue_2))
      (`/Engine/EditorBlueprintResources/StandardMacros.IsValid` _output_get
        (:`Is Valid`
          (add `/Game/AI/AIActors/BP_BaseEnemy.OnEnemyDeath` _output_get (`|CreateDelegate` :!event `EnemyDied`))
          (`KismetArrayLibrary.Array_Add` (`self.Alive Enemies`) _output_get)
          (`/Engine/EditorBlueprintResources/StandardMacros.IncrementInt` (`self.Current Spawn Index`)
            (:`  `
              ; Modifier Checks
              (`|ExecutionSequence`
                (:`then_0`
                  (if (`self.bExplosiveEnemies`)
                    (`self.OnEnemySpawned` (`self.SpawnedEnemy`))))
                (:`then_1`
                  ;;[1 0.004025 0.7835] Enemy Agro Modifier
                  (if (`self.EnemyAgroActive`)
                    (`/Game/AI/AIActors/BP_BaseEnemy.EnemyAgroActive` (`self.SpawnedEnemy`) (`self.PlayerTarget`))))))))))))

(event `EnemyDied`
  (params (Enemy :type "/Game/AI/AIActors/BP_BaseEnemy Object Reference"))
  ;[0.4793 0.05127 0.0648] Remove Dead Enemy from the Array of Alive Enemies -> Then check if theres any still alive before progressing to the next Wave.
  (`KismetArrayLibrary.Array_RemoveItem` (`self.Alive Enemies`) Enemy)
  (`self.CheckWaveCompletion`))

(event `OnWaveCompleted`
  (bind _currentwaveindex (`self.CurrentWaveIndex`))
  ;[0.4793 0.05127 0.0648] A Wave has been Completed -> Check if there is another and start that wave if so
  ;;[0.4793 0.05127 0.0648] No wave in progress
  (set `self.IsWaveInProgress?` false)
  ;;[0.4793 0.05127 0.0648] Increment Wave Count
  (`/Engine/EditorBlueprintResources/StandardMacros.IncrementInt` _currentwaveindex
    (:`  `
      (if (< _currentwaveindex (`KismetArrayLibrary.Array_Length` (`self.All Enemy Waves`)))
        ;;[0.4793 0.05127 0.0648] Start the Next Wave
        (`self.StartWave`)
        (else
          ;;[0.4793 0.05127 0.0648] LOGIC FOR ROOM COMPLETION HERE
          (`self.OnRoomComplete`))))))

(event `ChangeEnemyTarget`
  (params (NewTarget :type "Actor Object Reference"))
  ;[1 0.004025 0.7835] Swaps Enemy Agro Target
  (set `self.PlayerTarget` NewTarget)
  (for _array_element (`self.Alive Enemies`)
    (`/Game/AI/AIActors/BP_BaseEnemy.ChangeModiferPlayerTarget` _array_element (`self.PlayerTarget`))))

(event `Build Waves`
  ;[1 0.004025 0.7835] Build Enemy Waves
  (for _ (range 3)
    (bind _generatedwave (`self.Generate Wave`))
    (`KismetArrayLibrary.Array_Add` (`self.All Enemy Waves`) _generatedwave)))

(event `CaculateEnemyMultiplier`
  (bind _asgi_game_instance (cast `/Game/Blueprints/GI_GameInstance` (`GameplayStatics.GetGameInstance`) :!pure true))
  (bind _currentjoincount (`/Game/Blueprints/GI_GameInstance.CurrentJoinCount` _asgi_game_instance))
  (bind _returnvalue (- _currentjoincount 1))
  (bind _returnvalue_2 (- (`/Game/Blueprints/GI_GameInstance.CurrentRoomCount` _asgi_game_instance) 1))
  ;[1 0.004025 0.7835] Calculate Health Multiplier Based off Level Count + Player Count
  (set `self.DifficultyHealthMult` (+ (* _returnvalue_2 0.2) (* _returnvalue 0.5) 1.0))
  (set `self.PlayerCount` _currentjoincount)
  (set `self.MaxWaveCost` (`KismetMathLibrary.Conv_IntToDouble` (`KismetMathLibrary.FTrunc` (* 7.0 (+ (* _returnvalue_2 0.25) (* _returnvalue 0.5) 1.0) (`self.DoubleTroubleMult`))))))

(event `GetSpawnLocations`
  ;[1 0.004025 0.7835] Gets empty spawns
  (bind _outactors (`GameplayStatics.GetAllActorsOfClass` "/Game/Blueprints/LevelActors/BP_EnemySpawnLocation.BP_EnemySpawnLocation_C"))
  (set `self.EnemySpawnLocations` _outactors))

(fn `CheckWaveCompletion`
  ;[0.4793 0.05127 0.0648] Both true?
  (if (and (== (`KismetArrayLibrary.Array_Length` (`self.Alive Enemies`)) 0) (>= (`self.Current Spawn Index`) (`KismetArrayLibrary.Array_Length` (`self.Spawn Queue`))))
    (`KismetSystemLibrary.K2_ClearAndInvalidateTimerHandle` (`self.EnemyCheck`))
    ;[0.4793 0.05127 0.0648] Wave has been completed
    (`self.OnWaveCompleted`)))

(fn `ClearSpawnData`
  ;[0.4793 0.05127 0.0648] Resets all Spawn Info
  (`KismetArrayLibrary.Array_Clear` (`self.Spawn Queue`))
  (`KismetArrayLibrary.Array_Clear` (`self.Alive Enemies`))
  (set `self.Current Spawn Index` 0))

(fn `Generate Wave`
  (returns (GeneratedWave :type "/Game/Blueprints/Data/EnemySpawning/F_EnemyWaveData Structure"))
  (locals (CurrentWaveCost :type "Float (double-precision)") (EnemyWave :type "Array of /Game/Blueprints/Data/EnemySpawning/F_EnemySpawnInfo Structure") (SmallestCost :type "Float (double-precision)" :default 10.0) (RandomEnemy :type "/Game/AI/AIActors/BP_BaseEnemy Class Reference"))
  (bind _randomenemy (`local.RandomEnemy`))
  (bind _value (`BlueprintMapLibrary.Map_Find` (`self.EnemyCosts`) _randomenemy))
  ;[1 0.004025 0.7835] Enemy Wave Generator
  ;;[1 0.004025 0.7835] Gets Value of smallest Cost Enemy
  (for _array_element (`self.Enemies`)
    (bind _value_2 (`BlueprintMapLibrary.Map_Find` (`self.EnemyCosts`) _array_element))
    (if (and (< _value_2 (`local.SmallestCost`)) (!= _value_2 0.5))
      (set `local.SmallestCost` _value_2)))
  ;;[1 0.004025 0.7835] Generates Random Enemy from list and adds it to the wave
  (while (and (< (`local.CurrentWaveCost`) (`self.MaxWaveCost`)) (>= (- (`self.MaxWaveCost`) (`local.CurrentWaveCost`)) (`local.SmallestCost`)))
    (bind _output_get (set `local.RandomEnemy` (`KismetArrayLibrary.Array_Random` (`self.Enemies`))))
    (bind _value_3 (`BlueprintMapLibrary.Map_Find` (`self.EnemyCosts`) _output_get))
    (if (<= _value_3 (- (`self.MaxWaveCost`) (`local.CurrentWaveCost`)))
      (if (== _output_get "/Game/AI/AIActors/BP_BaseMeleeLeaderEnemy.BP_BaseMeleeLeaderEnemy_C")
        ;;[1 0.004025 0.7835] Enemy Leader Handling to spawn in minions
        (if (>= (- (`self.MaxWaveCost`) (`local.CurrentWaveCost`)) (+ _value_3 (* (`BlueprintMapLibrary.Map_Find` (`self.EnemyCosts`) (`KismetArrayLibrary.Array_Random` (`self.LeaderMinions`))) 2.0)))
          (bind _returnvalue (+ (`local.CurrentWaveCost`) _value_3))
          (set `local.CurrentWaveCost` _returnvalue)
          (`KismetArrayLibrary.Array_Add` (`local.EnemyWave`) (make `/Game/Blueprints/Data/EnemySpawning/F_EnemySpawnInfo` _output_get 1))
          (for _ (range (+ (`KismetMathLibrary.RandomIntegerInRange` 2 5) 1))
            (set `local.RandomEnemy` (`KismetArrayLibrary.Array_Random` (`self.LeaderMinions`)))
            (if (and (< (`local.CurrentWaveCost`) (`self.MaxWaveCost`)) (>= (- (`self.MaxWaveCost`) (`local.CurrentWaveCost`)) _value))
              (set `local.CurrentWaveCost` (+ (`local.CurrentWaveCost`) _value))
              (`KismetArrayLibrary.Array_Add` (`local.EnemyWave`) (make `/Game/Blueprints/Data/EnemySpawning/F_EnemySpawnInfo` _randomenemy 1)))))
        (else
          (set `local.CurrentWaveCost` _returnvalue)
          (`KismetArrayLibrary.Array_Add` (`local.EnemyWave`) (make `/Game/Blueprints/Data/EnemySpawning/F_EnemySpawnInfo` _output_get 1))))))
  ;;[1 0.004025 0.7835] Returns Generated Wave
  (return (make `/Game/Blueprints/Data/EnemySpawning/F_EnemyWaveData` (`local.EnemyWave`) "None" 0.5)))

(fn `GetRandomPointInRadius`
  (params (Origin :type "Vector2D Structure") (Radius :type "Float (double-precision)"))
  (returns (`Random Point` :type "Vector Structure"))
  (locals (SpawnLocation :type "Vector Structure" :default (0.0 0.0 0.0)) (InvalidLocation :type Boolean :default true) (SpawnRadi :type "Float (double-precision)" :default 5.0))
  (bind (_x _y) (`KismetMathLibrary.BreakVector2D` Origin))
  (bind _returnvalue (* Radius -1.0))
  ;[0.162 0.02956 0.3515] TODO: Account for navmesh TO ensure movement
  (set `local.SpawnLocation` (`KismetMathLibrary.MakeVector` (+ _x (`KismetMathLibrary.RandomFloatInRange` _returnvalue Radius)) (+ _y (`KismetMathLibrary.RandomFloatInRange` _returnvalue Radius)) 150.0))
  (while (`local.InvalidLocation`)
    (bind (_randomlocation _returnvalue_2) (`NavigationSystemV1.K2_GetRandomLocationInNavigableRadius` (`local.SpawnLocation`) (`local.SpawnRadi`) null null))
    (if _returnvalue_2
      (set `local.SpawnLocation` _randomlocation)
      (set `local.InvalidLocation` false)
      (else
        (set `local.SpawnRadi` (+ (`local.SpawnRadi`) 5.0)))))
  (return (`local.SpawnLocation`)))

(fn `GetRandomPre-setSpawnLocation`
  (params (SpawnRadi :type "Float (double-precision)"))
  (returns (SpawnLocation :type "Vector Structure"))
  (bind (_randomlocation _returnvalue) (`NavigationSystemV1.K2_GetRandomLocationInNavigableRadius` (`Actor.K2_GetActorLocation` (`KismetArrayLibrary.Array_Random` (`self.EnemySpawnLocations`))) SpawnRadi null null))
  (if _returnvalue
    (return _randomlocation)
    (else
      (bind _spawnlocation (`self.GetRandomPre-setSpawnLocation` SpawnRadi))
      (return _spawnlocation))))

(fn `SpawnAllEnemies`
  ;[0.4793 0.05127 0.0648] Spawns all Enemies in a Wave - Better for debugging
  ;;[0.4793 0.05127 0.0648] Clear List of Alive Enemies
  (`KismetArrayLibrary.Array_Clear` (`self.Alive Enemies`))
  ;;[0.4793 0.05127 0.0648] Loop through the Spawn Queue
  (for _index (range (`KismetArrayLibrary.Array_Length` (`self.Spawn Queue`)))
    ;;[0.4793 0.05127 0.0648] Get spawn origin and generate a random spawn point with it
    (bind _random_point (`self.GetRandomPointInRadius` (`self.SpawnOrigin`) (`self.SpawnRadius`)))
    ;;[0.4793 0.05127 0.0648] Spawn next Enemy from the Spawn Queue, assign an OnEnemyDeath and add to list of Alive Enemies
    (bind _returnvalue (`|SpawnActorFromClass` (`|GetArrayItem` (`self.Spawn Queue`) _index) (`KismetMathLibrary.MakeTransform` _random_point) "AdjustIfPossibleButAlwaysSpawn" "MultiplyWithRoot" null (`self.SpawnedHealthMult`) (`self.SpawnedDmgMult`) (`self.SpawnedSpeedMult`) null))
    (add `/Game/AI/AIActors/BP_BaseEnemy.OnEnemyDeath` _returnvalue (`|CreateDelegate` :!event `EnemyDied`))
    (`KismetArrayLibrary.Array_Add` (`self.Alive Enemies`) _returnvalue))
  ;;[0.4793 0.05127 0.0648] Current amount of Enemies that are Spawned
  (set `self.Current Spawn Index` (`KismetArrayLibrary.Array_Length` (`self.Alive Enemies`))))

(fn `StartWave`
  ;[0.4793 0.05127 0.0648] Only Start new Wave if one isn't in progress
  (if (not (`self.IsWaveInProgress?`))
    (set `self.IsWaveInProgress?` true)
    ;[0.4793 0.05127 0.0648] Reset Spawn Data
    (`self.ClearSpawnData`)
    ;[0.4793 0.05127 0.0648] Gets Info of incoming Wave
    (bind _output_get (set `self.Current Wave` (`|GetArrayItem` (`self.All Enemy Waves`) (`self.CurrentWaveIndex`))))
    (bind (_enemyspawninfo _wavename _spawnrate _spawnallatonce_) (break `/Game/Blueprints/Data/EnemySpawning/F_EnemyWaveData` _output_get))
    ;[0.4793 0.05127 0.0648] Build Spawn Queue (a list of all the enemies to spawn based on Wave Data)
    (for _array_element _enemyspawninfo
      (bind (_enemyclass _enemycount) (break `/Game/Blueprints/Data/EnemySpawning/F_EnemySpawnInfo` _array_element))
      (for _ (range _enemycount)
        (`KismetArrayLibrary.Array_Add` (`self.Spawn Queue`) _enemyclass)))
    ;[0.4793 0.05127 0.0648] Once Spawn Queue is built, should enemies spawn spawn all at once or on a timer?
    (if _spawnallatonce_
      ;[0.4793 0.05127 0.0648] Debug Purposes
      (`self.SpawnAllEnemies`)
      (else
        ;[0.4793 0.05127 0.0648] Start Spawning Enemies based on Spawn Rate
        (bind _returnvalue (`KismetSystemLibrary.K2_SetTimerDelegate` (`|CreateDelegate` :!event `SpawnNextEnemy`) _spawnrate true))
        (set `self.SpawnTimerHandle` _returnvalue)
        (bind _returnvalue_2 (`KismetSystemLibrary.K2_SetTimerDelegate` (`|CreateDelegate` :!event `CheckWaveCompletion`) 10.0 true))
        (set `self.EnemyCheck` _returnvalue_2)))))