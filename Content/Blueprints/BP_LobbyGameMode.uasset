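; Lobby game mode that sets up local multiplayer by creating a player and controller for each connected input device.
; On BeginPlay it creates the players, then caches player controllers up to the game instance's PlayerNum.
; It points the first controller's view at a camera actor found in the level.
; SpawnPlayer is an empty stub, and the player manager initialisation is disconnected and noted as not working.
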(event `self.ReceiveBeginPlay`
  ;[1 1 1] Add a character for each connected device
  (bind (_outinputdevices _returnvalue) (`InputDeviceLibrary.GetAllConnectedInputDevices`))
  (set `self.Game Instance` (cast `/Game/Blueprints/GI_GameInstance` (`GameplayStatics.GetGameInstance`) :!pure true))
  (`/Engine/EditorBlueprintResources/StandardMacros.IsValid` (`self.Game Instance`)
    (:`Is Valid`
      (for _ (range _returnvalue)
        (`GameplayStatics.CreatePlayer` -1))
      (for _index (range (`/Game/Blueprints/GI_GameInstance.PlayerNum` (`self.Game Instance`)))
        (`KismetArrayLibrary.Array_Add` (`self.PlayerControllers`) (cast `/Game/Blueprints/BPC_PlayerController` (`GameplayStatics.GetPlayerController` _index) :!pure true)))
      ;;[1 1 1 0.5] Set camera
      (bind _returnvalue_2 (`GameplayStatics.GetActorOfClass` "/Script/Engine.CameraActor"))
      (`PlayerController.SetViewTargetWithBlend` (`GameplayStatics.GetPlayerController` 0) _returnvalue_2 0.0 "VTBlend_Linear" 0.0 false))))

(fn `SpawnPlayer`)

(fn `UserConstructionScript`)