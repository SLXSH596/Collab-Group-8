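; Procedural map generator actor that builds a room layout from a TileSet at BeginPlay using a seeded random stream.
; It picks weighted repeating or singular rooms, attaches each at a random open exit and destroys any that overlap.
; If the room count falls short, it retries recursively.
; On success, it attempts to place leftover singular rooms, caps open exits and destroys itself.
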(event `self.ReceiveBeginPlay`
  (bind _tileset_startroom (break `/Vindustry_Procedural_Map_Creation/testingstuff/Core/ST_TileSet` (`self.TileSet`)))
  (if (`KismetSystemLibrary.IsValidClass` _tileset_startroom)
    (`self.BeginGeneration`)
    (else
      (`KismetSystemLibrary.PrintString` "ERROR: No StartRoom set within current TileSet!"))))

(fn `BeginGeneration`
  (locals (i :type Integer) (Failsafe :type Integer) (MaxSpawnAttempts :type Integer))
  (`self.SpawnStartRoom`)
  (set `local.Failsafe` 0)
  (set `local.MaxSpawnAttempts` (* (`self.AmountOfRooms`) 2))
  (if (and (`KismetArrayLibrary.Array_IsEmpty` (`self.RepeatingTilesCache`)) (`KismetArrayLibrary.Array_IsEmpty` (`self.SingularTilesCache`)))
    (`KismetSystemLibrary.PrintString` "NO ROOM CLASSES SET! Ending Generation")
    (return)
    (else
      (while (and (< (`local.i`) (`self.AmountOfRooms`)) (< (`local.Failsafe`) (`local.MaxSpawnAttempts`)) (`KismetArrayLibrary.Array_IsNotEmpty` (`self.ExitList`)))
        (`/Engine/EditorBlueprintResources/StandardMacros.IncrementInt` (`local.Failsafe`)
          (:`  `
            (bind _roomclasschosen (`self.GetRoomClass`))
            (if _roomclasschosen
              (`/Engine/EditorBlueprintResources/StandardMacros.IncrementInt` (`local.i`)
                (:`  `
                  (`self.SpawnRoomClass`)
                  (`self.RoomCollisionCheck`)))
              (else
                (`KismetSystemLibrary.PrintString` "Room was not able to be selected"))))))
      (bind _mapgensuccessful (`self.CheckMapGenSuccess`))
      (if _mapgensuccessful
        (`self.MapGenCleanup`)
        (else
          (`self.CacheTileSet`)
          (`self.BeginGeneration`))))))

(fn `CacheTileSet`
  (bind (_tileset_startroom _tileset_exitcap _tileset_repeatingtiles _tileset_singulartiles) (break `/Vindustry_Procedural_Map_Creation/testingstuff/Core/ST_TileSet` (`self.TileSet`)))
  (for _array_element _tileset_repeatingtiles
    (`KismetArrayLibrary.Array_Add` (`self.RepeatingTilesCache`) _array_element))
  (for _array_element_2 _tileset_singulartiles
    (`KismetArrayLibrary.Array_Add` (`self.SingularTilesCache`) _array_element_2)))

(fn `CheckMapGenSuccess`
  (returns (MapGenSuccessful :type Boolean))
  (bind _spawnedmaprooms (`self.SpawnedMapRooms`))
  (if (== (`self.AmountOfRooms`) (`KismetArrayLibrary.Array_Length` _spawnedmaprooms))
    (`KismetSystemLibrary.PrintString` "Map gen successful!")
    (return true)
    (elif (`KismetArrayLibrary.Array_IsNotEmpty` _spawnedmaprooms)
      (for _array_element (`self.SpawnedMapRooms`)
        (`self.K2_DestroyActor` _array_element))
      (`self.K2_DestroyActor` (`self.StartRoomRef`))
      (set `self.StartRoomRef` null)
      (`KismetArrayLibrary.Array_Clear` (`self.SpawnedMapRooms`))
      (`KismetArrayLibrary.Array_Clear` (`self.SingularTilesCache`))
      (`KismetArrayLibrary.Array_Clear` (`self.RepeatingTilesCache`))
      (`KismetArrayLibrary.Array_Clear` (`self.ExitList`))
      (return false)
      (else
        (return false)))))

(fn `GetRoomClass`
  (returns (RoomClassChosen :type Boolean))
  (locals (SingularTile :type "/Vindustry_Procedural_Map_Creation/testingstuff/Core/ST_SingularTiles Structure" :default (struct)) (SingularTileIndex :type Integer) (RepeatingTile :type "/Vindustry_Procedural_Map_Creation/testingstuff/Core/ST_RepeatingTiles Structure") (RepeatingTileIndex :type Integer))
  (bind (_repeatingtile_roomclass _repeatingtile_abundance) (break `/Vindustry_Procedural_Map_Creation/testingstuff/Core/ST_RepeatingTiles` (`local.RepeatingTile`)))
  (bind _singulartile_roomasset (break `/Vindustry_Procedural_Map_Creation/testingstuff/Core/ST_SingularTiles` (`local.SingularTile`)))
  (set `self.SelectedRoom` null)
  (while (not (`KismetSystemLibrary.IsValidClass` (`self.SelectedRoom`)))
    (if (`KismetMathLibrary.RandomBoolFromStream` (`self.RandomSeed`))
      (if (`KismetArrayLibrary.Array_IsNotEmpty` (`self.RepeatingTilesCache`))
        (bind _output_get (set `local.RepeatingTileIndex` (`KismetMathLibrary.RandomIntegerInRangeFromStream` (`self.RandomSeed`) 0 (- (`KismetArrayLibrary.Array_Length` (`self.RepeatingTilesCache`)) 1))))
        (bind _output_get_2 (set `local.RepeatingTile` (`|GetArrayItem` (`self.RepeatingTilesCache`) _output_get)))
        (if (and (`KismetSystemLibrary.IsValidClass` _repeatingtile_roomclass) (> _repeatingtile_abundance (`KismetMathLibrary.RandomFloatFromStream` (`self.RandomSeed`))))
          (set `self.SelectedRoom` (break `/Vindustry_Procedural_Map_Creation/testingstuff/Core/ST_RepeatingTiles` _output_get_2))
          (return true)))
      (elif (`KismetArrayLibrary.Array_IsNotEmpty` (`self.SingularTilesCache`))
        (bind _output_get_3 (set `local.SingularTileIndex` (`KismetMathLibrary.RandomIntegerInRangeFromStream` (`self.RandomSeed`) 0 (- (`KismetArrayLibrary.Array_Length` (`self.SingularTilesCache`)) 1))))
        (bind _output_get_4 (set `local.SingularTile` (`|GetArrayItem` (`self.SingularTilesCache`) _output_get_3)))
        (if (`.SpawnAtEndOfGeneration_3_73D9FC5A423677F13B51079661ECE462` (break `/Vindustry_Procedural_Map_Creation/testingstuff/Core/ST_SingularTiles` _output_get_4))
          _
          (elif (and (`KismetSystemLibrary.IsValidClass` (break `/Vindustry_Procedural_Map_Creation/testingstuff/Core/ST_SingularTiles` _output_get_4)) (> (`.ChanceToSpawn_6_11EEDEE54971C0CCDDF345B1358ACD0A` (break `/Vindustry_Procedural_Map_Creation/testingstuff/Core/ST_SingularTiles` _output_get_4)) (`KismetMathLibrary.RandomFloatFromStream` (`self.RandomSeed`))))
            (set `self.SelectedRoom` _singulartile_roomasset)
            (set `self.SingularRoomSetToSpawn` true)
            (set `self.SelectedTileIndex` (`local.SingularTileIndex`))
            (return true)
            (else
              (`KismetArrayLibrary.Array_Remove` (`self.SingularTilesCache`) (`local.SingularTileIndex`))))))))
  (return false))

(fn `MapGenCleanup`
  (bind _singulartilescache (`self.SingularTilesCache`))
  (bind (_tileset_startroom _tileset_exitcap) (break `/Vindustry_Procedural_Map_Creation/testingstuff/Core/ST_TileSet` (`self.TileSet`)))
  (`KismetSystemLibrary.PrintString` "Cleaning up...")
  (if (`KismetArrayLibrary.Array_IsNotEmpty` _singulartilescache)
    (for (_array_element _array_index) _singulartilescache
      (set `self.SelectedRoom` (break `/Vindustry_Procedural_Map_Creation/testingstuff/Core/ST_SingularTiles` _array_element))
      (set `self.SingularRoomSetToSpawn` true)
      (set `self.SelectedTileIndex` _array_index)
      (`self.SpawnRoomClass`)
      (`self.RoomCollisionCheck`)))
  (if (`KismetSystemLibrary.IsValidClass` _tileset_exitcap)
    (for _array_element_2 (`self.ExitList`)
      (bind _output_get (set `self.SelectedExit` _array_element_2))
      (bind (_returnvalue_location _returnvalue_rotation) (`KismetMathLibrary.BreakTransform` (`SceneComponent.K2_GetComponentToWorld` _output_get)))
      (`|SpawnActorFromClass` _tileset_exitcap (`KismetMathLibrary.MakeTransform` _returnvalue_location _returnvalue_rotation) "AlwaysSpawn" "MultiplyWithRoot" null null)))
  (`self.K2_DestroyActor`))

(fn `RoomCollisionCheck`
  (locals (CollisionComps :type "Array of SceneComponent Object Reference") (OverlappingRooms :type "Array of PrimitiveComponent Object Reference") (OverlappingComps :type "Array of PrimitiveComponent Object Reference"))
  (bind _lastspawnedroom (`self.LastSpawnedRoom`))
  (bind _exitlist (`self.ExitList`))
  (bind _output_get (set `local.CollisionComps` (`SceneComponent.GetChildrenComponents` (`/Vindustry_Procedural_Map_Creation/testingstuff/BP_RoomPARENT.Collisions` (`self.LastSpawnedRoom`)) true)))
  (for _array_element _output_get
    (bind _asprimitive_component (cast `PrimitiveComponent` _array_element))
    (`KismetArrayLibrary.Array_Append` (`local.OverlappingRooms`) (`PrimitiveComponent.GetOverlappingComponents` _asprimitive_component)))
  (if (`KismetArrayLibrary.Array_IsEmpty` (`local.OverlappingRooms`))
    (`KismetArrayLibrary.Array_RemoveItem` _exitlist (`self.SelectedExit`))
    (`KismetArrayLibrary.Array_Append` _exitlist (`SceneComponent.GetChildrenComponents` (`/Vindustry_Procedural_Map_Creation/testingstuff/BP_RoomPARENT.RoomExits` _lastspawnedroom) true))
    (`KismetArrayLibrary.Array_Add` (`self.SpawnedMapRooms`) (`self.LastSpawnedRoom`))
    (if (`self.SingularRoomSetToSpawn`)
      (`KismetArrayLibrary.Array_Remove` (`self.SingularTilesCache`) (`self.SelectedTileIndex`)))
    (set `self.SingularRoomSetToSpawn` false)
    (else
      (`self.K2_DestroyActor` _lastspawnedroom))))

(fn `SpawnRoomClass`
  (bind _exitlist (`self.ExitList`))
  (if (`KismetArrayLibrary.Array_IsEmpty` _exitlist)
    (`KismetSystemLibrary.PrintString` "NO MORE ROOM EXITS")
    (else
      (bind _output_get (set `self.SelectedExit` (`KismetArrayLibrary.Array_RandomFromStream` _exitlist (`self.RandomSeed`))))
      (bind (_returnvalue_location _returnvalue_rotation) (`KismetMathLibrary.BreakTransform` (`SceneComponent.K2_GetComponentToWorld` _output_get)))
      (bind _returnvalue (`|SpawnActorFromClass` (`self.SelectedRoom`) (`KismetMathLibrary.MakeTransform` _returnvalue_location _returnvalue_rotation) "AlwaysSpawn" "MultiplyWithRoot" null null))
      (set `self.LastSpawnedRoom` _returnvalue))))

(fn `SpawnStartRoom`
  (bind (_returnvalue_location _returnvalue_rotation) (`KismetMathLibrary.BreakTransform` (`self.GetTransform`)))
  (bind _exitlist (`self.ExitList`))
  (bind _tileset_startroom (break `/Vindustry_Procedural_Map_Creation/testingstuff/Core/ST_TileSet` (`self.TileSet`)))
  (bind _returnvalue (`|SpawnActorFromClass` _tileset_startroom (`KismetMathLibrary.MakeTransform` _returnvalue_location _returnvalue_rotation) "Undefined" "MultiplyWithRoot" null null))
  (bind _output_get (set `self.StartRoomRef` _returnvalue))
  (bind _output_get_2 (set `self.LastSpawnedRoom` _output_get))
  (`KismetArrayLibrary.Array_Append` _exitlist (`SceneComponent.GetChildrenComponents` (`/Vindustry_Procedural_Map_Creation/testingstuff/BP_RoomPARENT.RoomExits` _output_get_2) true))
  (set `self.SelectedExit` (`KismetArrayLibrary.Array_RandomFromStream` _exitlist (`self.RandomSeed`))))

(fn `UserConstructionScript`
  (`KismetArrayLibrary.Array_Clear` (`self.RepeatingTilesCache`))
  (`KismetArrayLibrary.Array_Clear` (`self.SingularTilesCache`))
  (`KismetArrayLibrary.Array_Clear` (`self.ExitList`))
  (`KismetMathLibrary.SeedRandomStream` (`self.RandomSeed`))
  (`self.CacheTileSet`)
  (`self.SetActorScale3D` (1.0 1.0 1.0)))