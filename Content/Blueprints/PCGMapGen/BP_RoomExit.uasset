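; BP_RoomExit is a room exit actor for the PCG map generator that opens by removing itself from the level.
; OpenExit destroys the actor outright, while CloseExit is an empty stub.
; BeginPlay stores the start location, which only an unconnected Timeline uses to lerp the Box downward.
; That animation and a delayed OpenExit call are never executed.
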(event Custom|Open%20Exit
  (Actor|DestroyActor))

(event Custom|Close%20Exit)

(event EventBeginPlay
  (Variables|Default|SetStart%20Location (Transformation|GetActorLocation)))

(fn ConstructionScript)