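; Blueprint function library with a helper that finds the player controller of the first joined player.
; Outside the lobby, it scans the keys of the GameInstance's JoinedPlayersMap, tracking the lowest, and uses that as the player index.
; In the lobby, it simply returns player zero's controller for simplicity.
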(fn `FindFirstPlayerController`
  (params (GameInstance :type "/Game/Blueprints/GI_GameInstance Object Reference") (bNotLobby :type Boolean))
  (returns (FirstPlayerController :type "PlayerController Object Reference"))
  (locals (Lowest :type Integer :default 3))
  (if bNotLobby
    (bind _keypin (`|MapForEach` (`/Game/Blueprints/GI_GameInstance.JoinedPlayersMap` GameInstance))
      (:`then`
        (if (< _keypin (`local.Lowest`))
          (set `local.Lowest` _keypin)))
      (:`CompletedPin`
        (return (`GameplayStatics.GetPlayerController` null (`local.Lowest`)))))
    (else
      ;[0.162 0.02956 0.3515] Return player zero for lobby - its just easiest
      (return (`GameplayStatics.GetPlayerController` null)))))