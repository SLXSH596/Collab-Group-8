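; Player controller that routes Enhanced Input movement and attack to the possessed BP_Player and manages game UI.
; On BeginPlay, only the first controller creates the HUD from the gamemode's controller list, prepares the death screen and binds to the player manager's game-over event.
; Pause toggles game pause, menu and input mode.
; Pause and death screens delay briefly before setting keyboard focus on their buttons.
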(event `self.ReceiveBeginPlay`
  (bind _asbp_gamemode (cast `/Game/Blueprints/BP_Gamemode` (`GameplayStatics.GetGameMode`)))
  (bind _output_get (set `self.Gamemode` _asbp_gamemode))
  ;[0.162 0.02956 0.3515] Only do UI setup etc. if this is the first player controller
  (if (== (`GameplayStatics.GetPlayerControllerID` self) 0)
    ;[0.162 0.02956 0.3515] HUD Setup
    (bind _returnvalue (`|CreateWidget` "/Game/UI/WBP_HUD.WBP_HUD_C"))
    (bind _output_get_2 (set `self.HUD` _returnvalue))
    (`/Game/UI/WBP_HUD.Init` _output_get_2 (`/Game/Blueprints/BP_Gamemode.PlayerControllers` _output_get))
    (`UserWidget.AddToViewport` _output_get_2 0)
    ;[0.06301 0.6939 0.1441] Death Setup
    (`self.Setup Death Screen`)
    (bind _ac_playermanager (`/Game/Blueprints/BP_Gamemode.AC_PlayerManager` _output_get))
    (`/Engine/EditorBlueprintResources/StandardMacros.IsValid` _ac_playermanager
      (:`Is Valid`
        (bind _output_get_3 (set `self.Player Manager` _ac_playermanager))
        (add `/Game/Blueprints/Components/AC_PlayerManager.OnGameOver` _output_get_3 (`|CreateDelegate` :!event `Display Death Screen`))))))

(event `EnhancedInput|/Game/Input/IA_PrimaryAttack`
  (params (ActionValue :type Boolean) (ElapsedSeconds :type "Float (double-precision)") (TriggeredSeconds :type "Float (double-precision)") (InputAction :type "InputAction Object Reference" :default "/Game/Input/IA_PrimaryAttack.IA_PrimaryAttack"))
  (:`Triggered`
    (`/Game/Blueprints/BP_Player.PrimaryAttack` (`self.PlayerPawn`))))

(event `Setup Death Screen`
  ;[0.06301 0.6939 0.1441] Initialise death screen
  (`/Engine/EditorBlueprintResources/StandardMacros.DoOnce` false
    (:`Completed`
      (bind _returnvalue (`|CreateWidget` "/Game/UI/WBP_DeathScreen.WBP_DeathScreen_C"))
      (set `self.DeathScreen` _returnvalue))))

(event `EnhancedInput|/Game/Input/IA_Movement`
  (params (ActionValue :type "Vector2D Structure") (ElapsedSeconds :type "Float (double-precision)") (TriggeredSeconds :type "Float (double-precision)") (InputAction :type "InputAction Object Reference" :default "/Game/Input/IA_Movement.IA_Movement"))
  (:`Triggered`
    (`Pawn.AddMovementInput` (`self.PlayerPawn`) (`KismetMathLibrary.Conv_Vector2DToVector` ActionValue) 100.0 false)))

(event `self.ReceivePossess`
  (params (PossessedPawn :type "Pawn Object Reference"))
  ;[0.162 0.02956 0.3515] Setup inputs
  (set `self.PlayerPawn` (cast `/Game/Blueprints/BP_Player` PossessedPawn :!pure true))
  (`EnhancedInputSubsystemInterface.AddMappingContext` (subsystem `EnhancedInputLocalPlayerSubsystem`) "/Game/Input/IMC_Controls.IMC_Controls" 0 (struct))
  (`WidgetBlueprintLibrary.SetInputMode_GameOnly` self true))

(event `EnhancedInput|/Game/Input/IA_Pause`
  (params (ActionValue :type Boolean) (ElapsedSeconds :type "Float (double-precision)") (TriggeredSeconds :type "Float (double-precision)") (InputAction :type "InputAction Object Reference" :default "/Game/Input/IA_Pause.IA_Pause"))
  (bind _pausemenu (`self.PauseMenu`))
  ;[1 1 1] Pause - TODO: DISCUSS AND CONSOLIDATE UI PLANNING WITH MULTIPLAYER FUNCTIONALITY
  (:`Started`
    (if (`GameplayStatics.IsGamePaused`)
      (`GameplayStatics.SetGamePaused` false)
      (`/Engine/EditorBlueprintResources/StandardMacros.IsValid` _pausemenu
        (:`Is Valid`
          (`/Game/UI/WBP_PauseMenu.Unpause` _pausemenu)
          (`WidgetBlueprintLibrary.SetInputMode_GameOnly` self)))
      (else
        (`GameplayStatics.SetGamePaused` true)
        (bind _returnvalue (`|CreateWidget` "/Game/UI/WBP_PauseMenu.WBP_PauseMenu_C"))
        (bind _output_get (set `self.PauseMenu` _returnvalue))
        (`UserWidget.AddToViewport` _output_get 0)
        (`WidgetBlueprintLibrary.SetInputMode_GameAndUIEx` self _output_get)
        (`KismetSystemLibrary.Delay` 0.2)
        (`Widget.SetKeyboardFocus` (`/Game/UI/WBP_PauseMenu.ResumeButton` _output_get))
        (`/Game/UI/WBP_PauseMenu.Init` _output_get self)))))

(event `Display Death Screen`
  (bind _deathscreen (`self.DeathScreen`))
  ;[0.06301 0.6939 0.1441] Display death screen
  (`/Engine/EditorBlueprintResources/StandardMacros.IsValid` _deathscreen
    (:`Is Valid`
      (`UserWidget.AddToViewport` _deathscreen 0)
      (`WidgetBlueprintLibrary.SetInputMode_GameAndUIEx` self _deathscreen)
      (`KismetSystemLibrary.Delay` 0.2)
      (`Widget.SetKeyboardFocus` (`/Game/UI/WBP_DeathScreen.ReturnButton` _deathscreen)))))

(fn `UserConstructionScript`)