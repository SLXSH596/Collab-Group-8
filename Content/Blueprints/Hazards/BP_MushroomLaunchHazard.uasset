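; A hazard Blueprint for a mushroom that launches characters that collide with it.
; Its HazardEffect override plays the mushroom sound with a Type parameter, then runs the parent effect.
; It then launches an overlapping player or base enemy along the Arrow component's forward vector, scaled much more horizontally than vertically, adding to existing velocity rather than overriding it.
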(event `self.Hazard Effect`
  (params (`Overlapped Actor` :type "Actor Object Reference"))
  (bind _returnvalue (* (`SceneComponent.GetForwardVector` (`self.Arrow`)) (2500.0 2500.0 300.0)))
  ; Mushroom launchers characters a set amount on collision
  (bind _returnvalue_2 (`GameplayStatics.SpawnSoundAtLocation` "/Game/Audio/MetaSounds/SFX/MS_Mushrooms.MS_Mushrooms" (`self.K2_GetActorLocation`) (struct) 1.0 1.0 0.0 null null))
  (`AudioParameterControllerInterface.SetIntParameter` _returnvalue_2 "Type" 0)
  (`parent.Hazard Effect` `Overlapped Actor`)
  (bind _asbp_player (cast `/Game/Blueprints/Player/BP_Player` `Overlapped Actor`)
    (:`then`
      (`Character.LaunchCharacter` _asbp_player _returnvalue false false))
    (:`CastFailed`
      (bind _asbp_base_enemy (cast `/Game/AI/AIActors/BP_BaseEnemy` `Overlapped Actor`))
      (`Character.LaunchCharacter` _asbp_base_enemy _returnvalue false false))))

(fn `UserConstructionScript`
  (`parent.UserConstructionScript`))