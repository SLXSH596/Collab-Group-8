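; Poison bomb hazard actor that spreads into a flat damaging area, then shrinks away and destroys itself.
; On spawn, a timeline scales the mesh out into a wide, thin shape, and a looping one-second timer is started, presumably driving Poison.
; Poison sphere-traces around the actor and applies explosive-type damage to blocking hits while ApplyDamage is set.
; After a delay, a second timeline shrinks the mesh and clears that flag.
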(event `self.ReceiveBeginPlay`
  (bind _staticmesh (`self.StaticMesh`))
  (`self.ScalePoison`)
  (`KismetSystemLibrary.K2_SetTimerDelegate` (`|CreateDelegate` :!event `Poison`) 1.0 true)
  (`KismetSystemLibrary.Delay` 8.0)
  (bind (_direction _alpha) (`Timeline|Timeline` :!via `PlayFromStart`)
    (:`Update`
      (`SceneComponent.SetRelativeScale3D` _staticmesh (`KismetMathLibrary.VLerp` (`SceneComponent.K2_GetComponentScale` _staticmesh) (0.0 0.0 0.0) _alpha)))
    (:`Finished`
      (`self.K2_DestroyActor`))
    (:`Event Alpha`
      (set `self.ApplyDamage?` false))))

(event `Poison`
  (bind _returnvalue (`self.K2_GetActorLocation`))
  (if (`self.ApplyDamage?`)
    (bind _outhits (`KismetSystemLibrary.SphereTraceMultiForObjects` _returnvalue _returnvalue 300.0 (`self.DefaultObjects`)))
    (for _array_element _outhits
      (bind (_bblockinghit _binitialoverlap _time _distance _location _impactpoint _normal _impactnormal _physmat _hitactor) (`GameplayStatics.BreakHitResult` _array_element))
      (if _bblockinghit
        (`GameplayStatics.ApplyDamage` _hitactor 0.5 null null "/Game/Blueprints/WeaponDamageTypes/BP_DamageType_Explosive.BP_DamageType_Explosive_C")))))

(event `ScalePoison`
  (bind _staticmesh (`self.StaticMesh`))
  (bind (_direction _alpha) (`Timeline|Timeline_0` :!via `PlayFromStart`)
    (:`Update`
      (`SceneComponent.SetRelativeScale3D` _staticmesh (`KismetMathLibrary.VLerp` (`SceneComponent.K2_GetComponentScale` _staticmesh) (6.0 6.0 0.1) _alpha)))))

(fn `UserConstructionScript`)