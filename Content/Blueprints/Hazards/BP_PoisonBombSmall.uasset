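; Small poison bomb hazard: a cloud that expands, damages what it touches, then shrinks away and destroys itself.
; Timelines lerp from the current actor scale to grow it on BeginPlay and shrink it after a delay.
; A looping timer is set alongside the Poison event, which sphere-traces at the actor's bounds extent and deals explosive-type damage to blocking hits.
; An event in the shrink timeline switches damage off.
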(event `self.ReceiveBeginPlay`
  (`self.ScalePoison`)
  (`KismetSystemLibrary.K2_SetTimerDelegate` (`|CreateDelegate` :!event `Poison`) 1.0 true)
  (`KismetSystemLibrary.Delay` 5.5)
  (bind (_direction _alpha) (`Timeline|Timeline` :!via `PlayFromStart`)
    (:`Update`
      (`self.SetActorScale3D` (`KismetMathLibrary.VLerp` (`self.GetActorScale3D`) (0.0 0.0 0.0) _alpha)))
    (:`Finished`
      (`self.K2_DestroyActor`))
    (:`Event Alpha`
      (set `self.ApplyDamage?` false))))

(event `Poison`
  (bind (_origin _boxextent) (`self.GetActorBounds` false))
  (bind _returnvalue (`self.K2_GetActorLocation`))
  (bind _x (.x _origin))
  (if (`self.ApplyDamage?`)
    (bind _outhits (`KismetSystemLibrary.SphereTraceMultiForObjects` _returnvalue _returnvalue (- (+ _x (.x _boxextent)) _x) (`self.DefaultObjects`)))
    (for _array_element _outhits
      (bind (_bblockinghit _binitialoverlap _time _distance _location _impactpoint _normal _impactnormal _physmat _hitactor) (`GameplayStatics.BreakHitResult` _array_element))
      (if _bblockinghit
        (`GameplayStatics.ApplyDamage` _hitactor 10.0 null null "/Game/Blueprints/WeaponDamageTypes/BP_DamageType_Explosive.BP_DamageType_Explosive_C")))))

(event `ScalePoison`
  (bind (_direction _alpha) (`Timeline|Timeline_0` :!via `PlayFromStart`)
    (:`Update`
      (`self.SetActorScale3D` (`KismetMathLibrary.VLerp` (`self.GetActorScale3D`) (3.0 3.0 3.0) _alpha)))))

(fn `UserConstructionScript`)