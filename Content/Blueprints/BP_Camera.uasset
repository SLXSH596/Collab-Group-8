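; Shared multiplayer camera that frames all player pawns by following the center of their bounds and zooming with their spread.
; Init caches pawns from the passed controllers and makes this actor player 0's view target.
; Each Tick, FindMinMaxPlayerCoords supplies X/Y extremes, whose midpoint sets actor location.
; The larger axis span, clamped, becomes the spring arm length.
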(event `Init`
  (params (PlayerControllers :type "Array of /Game/Blueprints/BPC_PlayerController Object Reference"))
  ;[0 1 0 0.5] Init - sets view target and gets references to player pawns
  (bind _output_get (set `self.PlayerControllers` PlayerControllers))
  (for _array_element _output_get
    (`KismetArrayLibrary.Array_AddUnique` (`self.PlayerPawns`) (`Controller.K2_GetPawn` _array_element)))
  (`PlayerController.SetViewTargetWithBlend` (`GameplayStatics.GetPlayerController` 0) self 0.0 "VTBlend_Linear" 0.0 false))

(event `self.ReceiveTick`
  (params (DeltaSeconds :type "Float (single-precision)"))
  (bind (_minx _maxx _miny _maxy) (`self.FindMinMaxPlayerCoords`))
  (bind _returnvalue (- _maxy _miny))
  (bind _returnvalue_2 (- _maxx _minx))
  ;[1 0 0 0.5] Average location of players to move camera to
  (`self.K2_SetActorLocation` (`KismetMathLibrary.MakeVector` (/ (+ _minx _maxx) 2.0) (/ (+ _miny _maxy) 2.0)))
  ;[1 0 0 0.5] Set spring arm length accordingly and clamp
  (set `SpringArmComponent.TargetArmLength` (`KismetMathLibrary.FClamp` (`KismetMathLibrary.SelectFloat` _returnvalue_2 _returnvalue (> _returnvalue_2 _returnvalue)) 1000.0 5000.0) (`self.SpringArm`)))

(fn `FindMinMaxPlayerCoords`
  (returns (MinX :type "Float (double-precision)") (MaxX :type "Float (double-precision)") (MinY :type "Float (double-precision)") (MaxY :type "Float (double-precision)"))
  (locals (MinXPos :type "Float (double-precision)" :default 99999.0) (MaxXPos :type "Float (double-precision)" :default -99999.0) (MinYPos :type "Float (double-precision)" :default 99999.0) (MaxYPos :type "Float (double-precision)" :default -99999.0))
  ;[0 0 1 0.5] Calculates the bounds of player coords for usage in camera operations
  (for _array_element (`self.PlayerPawns`)
    (`|ExecutionSequence`
      (:`then_0`
        (bind (_returnvalue_x _returnvalue_y) (`KismetMathLibrary.BreakVector` (`self.K2_GetActorLocation` _array_element)))
        (if (< _returnvalue_x (`local.MinXPos`))
          (set `local.MinXPos` _returnvalue_x)))
      (:`then_1`
        (if (> _returnvalue_x (`local.MaxXPos`))
          (set `local.MaxXPos` _returnvalue_x)))
      (:`then_2`
        (if (< _returnvalue_y (`local.MinYPos`))
          (set `local.MinYPos` _returnvalue_y)))
      (:`then_3`
        (if (> _returnvalue_y (`local.MaxYPos`))
          (set `local.MaxYPos` _returnvalue_y)))))
  (return (`local.MinXPos`) (`local.MaxXPos`) (`local.MinYPos`) (`local.MaxYPos`)))

(fn `UserConstructionScript`)