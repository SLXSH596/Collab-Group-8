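; Player controller for the main menu, which shows the menu UI and handles starting the game.
; On BeginPlay it caches the game instance, creates the main menu widget, binds to its nested start-button event and switches to UI-only input with a visible cursor.
; StartGame copies PlayerNum into the game instance so it persists across the level change, then opens the test level.
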(event `self.ReceiveBeginPlay`
  (set `self.GameInstance` (cast `/Game/Blueprints/GI_GameInstance` (`GameplayStatics.GetGameInstance`) :!pure true))
  (bind _returnvalue (`|CreateWidget` "/Game/UI/Menu/WBP_MainMenu.WBP_MainMenu_C" self))
  (bind _output_get (set `self.Menu` _returnvalue))
  (add `/Game/UI/Menu/WBP_MenuButtons.OnStartClicked` (`/Game/UI/Menu/WBP_TitleScreen.WBP_MenuButtons` (`/Game/UI/Menu/WBP_MainMenu.WBP_TitleScreen` _output_get)) (`|CreateDelegate` :!event `Start Game`))
  (`UserWidget.AddToViewport` _output_get 0)
  (`WidgetBlueprintLibrary.SetInputMode_UIOnlyEx` self null)
  (set `self.bShowMouseCursor` true))

(event `Start Game`
  (bind _gameinstance (`self.GameInstance`))
  (`/Engine/EditorBlueprintResources/StandardMacros.IsValid` _gameinstance
    (:`Is Valid`
      (set `/Game/Blueprints/GI_GameInstance.PlayerNum` (`self.PlayerNum`) _gameinstance)
      (`GameplayStatics.OpenLevelBySoftObjectPtr` "/Game/Maps/LVL_Test.LVL_Test"))))

(fn `UserConstructionScript`)