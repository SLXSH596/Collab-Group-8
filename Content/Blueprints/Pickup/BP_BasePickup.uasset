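; Base pickup actor that grants an effect to the interacting actor's AC_StatComponent, then destroys itself.
; LaunchDrop throws the mesh in an arc, and the first hit stops physics and adjusts a placeholder Niagara effect.
; ACInteractable's OnInteracted drives GrabPickup, which calls the empty ApplyPickupEffect hook.
; InteractionRange overlaps toggle a tooltip with fixed world rotation for actors that have a stat component.
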(event `self.Mesh.OnComponentHit`
  (params (HitComponent :type "PrimitiveComponent Object Reference") (OtherActor :type "Actor Object Reference") (OtherComp :type "PrimitiveComponent Object Reference") (NormalImpulse :type "Vector Structure") (Hit :type "HitResult Structure (by ref)"))
  (bind _ns_pickupplaceholder (`self.NS_PickUpPlaceHolder`))
  ;[1 1 1] Stop physics on hitting something
  (`PrimitiveComponent.SetSimulatePhysics` (`self.Mesh`) false)
  ;[1 1 1] Messing with placeholder particle effect
  (`NiagaraComponent.SetVariableVec3` _ns_pickupplaceholder "VelocityMax" (0.0 0.0 200.0))
  (`NiagaraComponent.SetVariableVec3` _ns_pickupplaceholder "VelocityMin" (0.0 0.0 200.0))
  (`NiagaraComponent.SetVariableFloat` _ns_pickupplaceholder "Lifetime" 1.5))

(event `Launch Drop`
  ;[1 1 1] Handle moving the drop in an arc
  (`PrimitiveComponent.AddImpulse` (`self.Mesh`) (* (`KismetMathLibrary.GreaterGreater_VectorRotator` (`self.GetActorForwardVector`) (`KismetMathLibrary.RotatorFromAxisAndAngle` (`KismetMathLibrary.NegateVector` (`self.GetActorRightVector`)) 60.0)) 500.0) "None" true))

(event `self.CollisionSphere.OnComponentBeginOverlap`
  (params (OverlappedComponent :type "PrimitiveComponent Object Reference") (OtherActor :type "Actor Object Reference") (OtherComp :type "PrimitiveComponent Object Reference") (OtherBodyIndex :type Integer) (bFromSweep :type Boolean) (SweepResult :type "HitResult Structure (by ref)")))

(event `self.ReceiveBeginPlay`
  ;[0.4793 0.05127 0.0648] Bind "Grab Pickup" to "On Interacted". When called elsewhere, it will now fire this Custom Event
  (add `/Game/Components/Objects/AC_Interactable.OnInteracted` (`self.AC_Interactable`) (delegate `Grab Pickup`)))

(event `Grab Pickup`
  (params (Owner :type "/Game/Blueprints/Player/BP_Player Object Reference"))
  (bind _returnvalue (`self.GetComponentByClass` Owner "/Game/Components/Player/AC_StatComponent.AC_StatComponent_C"))
  ;[0.4793 0.05127 0.0648] Bind "Grab Pickup" to "On Interacted". When called elsewhere, it will now fire this Custom Event
  (`/Engine/EditorBlueprintResources/StandardMacros.IsValid` _returnvalue
    (:`Is Valid`
      (`self.ApplyPickupEffect` _returnvalue)
      (`self.K2_DestroyActor`))))

(event `self.InteractionRange.OnComponentBeginOverlap`
  (params (OverlappedComponent :type "PrimitiveComponent Object Reference") (OtherActor :type "Actor Object Reference") (OtherComp :type "PrimitiveComponent Object Reference") (OtherBodyIndex :type Integer) (bFromSweep :type Boolean) (SweepResult :type "HitResult Structure (by ref)"))
  (bind _pickup_tooltip (`self.Pickup_Tooltip`))
  ;[0.4793 0.05127 0.0648] Has the player just reached the interaction range?
  ; Begin Overlap (Yes) -> Make the Pickup UI visible
  ; End Overlap (No longer) -> Make the Pickup UI invisible
  (`/Engine/EditorBlueprintResources/StandardMacros.IsValid` (`self.GetComponentByClass` OtherActor "/Game/Components/Player/AC_StatComponent.AC_StatComponent_C")
    (:`Is Valid`
      (`SceneComponent.SetVisibility` _pickup_tooltip true false)
      ;[1 1 1] Might need to make this face the camera instead of a har value
      (`SceneComponent.K2_SetWorldRotation` _pickup_tooltip (struct :`Yaw` 180.0) false false))))

(event `self.InteractionRange.OnComponentEndOverlap`
  (params (OverlappedComponent :type "PrimitiveComponent Object Reference") (OtherActor :type "Actor Object Reference") (OtherComp :type "PrimitiveComponent Object Reference") (OtherBodyIndex :type Integer))
  ;[0.4793 0.05127 0.0648] Has the player just reached the interaction range?
  ; Begin Overlap (Yes) -> Make the Pickup UI visible
  ; End Overlap (No longer) -> Make the Pickup UI invisible
  (`/Engine/EditorBlueprintResources/StandardMacros.IsValid` (`self.GetComponentByClass` OtherActor "/Game/Components/Player/AC_StatComponent.AC_StatComponent_C")
    (:`Is Valid`
      (`SceneComponent.SetVisibility` (`self.Pickup_Tooltip`) false false))))

(fn `ApplyPickupEffect`
  (params (ActorComp :type "/Game/Components/Player/AC_StatComponent Object Reference")))

(fn `Initialise`)

(fn `UserConstructionScript`)