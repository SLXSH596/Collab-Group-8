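; Loot chest that drops one upgrade pickup per connected player when a room is completed.
; DropLoot refreshes the count from GI_GameInstance's join count, then Launchupgrade shuffles the Upgrades list and spawns a random entry per player.
; Spawn yaws are spread evenly around 360 degrees so drops face outward, and each spawned class is removed to avoid repeats.
; Launch physics is delegated to each BP_BasePickup via LaunchDrop.
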(event `self.ReceiveBeginPlay`
  ;[1 1 1] Used to set how many item based on players connected
  (bind _asgi_game_instance (cast `/Game/Blueprints/GI_GameInstance` (`GameplayStatics.GetGameInstance`)))
  (bind _output_get (set `self.Game Instance` _asgi_game_instance))
  (set `self.Number of Items` (`/Game/Blueprints/GI_GameInstance.CurrentJoinCount` _output_get)))

(event `Launch upgrade`
  (bind _upgrades (`self.Upgrades`))
  (bind _number_of_items (`self.Number of Items`))
  ;[1 1 1] Drops loot for each player ingame
  (for _index (range 1 (+ _number_of_items 1))
    ;[1 1 1] Added this because the random didnt seem random enough
    (`KismetArrayLibrary.Array_Shuffle` _upgrades)
    (bind _returnvalue (`|SpawnActorFromClass` (`KismetArrayLibrary.Array_Random` _upgrades) (`KismetMathLibrary.MakeTransform` (`SceneComponent.K2_GetComponentLocation` (`self.Spawn Location`)) (`KismetMathLibrary.MakeRotator` 0.0 0.0 (- 360.0 (* (`KismetMathLibrary.Conv_IntToDouble` _index) (/ 360.0 (`KismetMathLibrary.Conv_IntToDouble` _number_of_items)))))) "Undefined" "MultiplyWithRoot" null null))
    ;[1 1 1] Doesnt allow repeats per level
    (`KismetArrayLibrary.Array_RemoveItem` (`self.Upgrades`) (`GameplayStatics.GetObjectClass` _returnvalue))
    ;[1 1 1] Physics of launch is handled on the drop itself
    (bind _asbp_base_pickup (cast `/Game/Blueprints/Pickup/BP_BasePickup` _returnvalue))
    (`/Game/Blueprints/Pickup/BP_BasePickup.Launch Drop` _asbp_base_pickup)))

(event `Drop Loot`
  ;[1 1 1 0.5] Drops loot when room is complete
  (set `self.Number of Items` (`/Game/Blueprints/GI_GameInstance.CurrentJoinCount` (`self.Game Instance`)))
  (`self.Launch upgrade`))

(fn `UserConstructionScript`)