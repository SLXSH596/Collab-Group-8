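; BP_WeaponSelector is a trigger actor that sets the player's weapon type when the player overlaps its box.
; On overlap with a BP_Player, it copies its WeaponType into the player's ChosenWeaponType and calls SetCurrentWeapon on that player.
; It also prints the selection and writes the weapon name to its WeaponText, while other actors only trigger debug prints.
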(event `self.ReceiveBeginPlay`)

(event `self.Box.OnComponentBeginOverlap`
  (params (OverlappedComponent :type "PrimitiveComponent Object Reference") (OtherActor :type "Actor Object Reference") (OtherComp :type "PrimitiveComponent Object Reference") (OtherBodyIndex :type Integer) (bFromSweep :type Boolean) (SweepResult :type "HitResult Structure (by ref)"))
  (bind _asbp_player (cast `/Game/Blueprints/BP_Player` OtherActor)
    (:`then`
      (bind _output_get (set `self.As BP Player` _asbp_player))
      (bind _output_get_2 (set `/Game/Blueprints/BP_Player.ChosenWeaponType` (`self.WeaponType`) _output_get))
      (bind _returnvalue (`|GetEnumeratorNameAsString` _output_get_2))
      (`KismetSystemLibrary.PrintString` (`KismetStringLibrary.Concat_StrStr` _returnvalue " selected."))
      (`TextRenderComponent.K2_SetText` (`self.WeaponText`) (`KismetTextLibrary.Conv_StringToText` _returnvalue))
      (`/Game/Blueprints/BP_Player.SetCurrentWeapon` _output_get))
    (:`CastFailed`
      (`KismetSystemLibrary.PrintString` "Unknown")
      (`KismetSystemLibrary.PrintString` "Hello"))))

(fn `UserConstructionScript`)