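; Game instance that drives random room progression and resets local multiplayer run state.
; SelectNewLevel opens a random regular level, or a boss level for the last room, removing a random pool entry and incrementing the room count.
; The random pick is re-evaluated, so the removed and opened levels can differ.
; ClearAll zeroes counters, removes extra local players and empties weapon, buff and joined-player maps.
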(event `SelectNewLevel`
  (bind _returnvalue (select `bool` (== (`self.CurrentRoomCount`) (- (`self.MaxRoomCount`) 1)) :`false` (`self.RegularLevels`) :`true` (`self.BossLevels`)))
  (bind _outitem (`KismetArrayLibrary.Array_Random` _returnvalue))
  ;[0.162 0.02956 0.3515] Only select new level if not in final room
  (if (< (`self.CurrentRoomCount`) (`self.MaxRoomCount`))
    ;[0.162 0.02956 0.3515] Open Random Level depending on room number
    ; TODO: Make it only choose previously unchosen levels
    (`KismetArrayLibrary.Array_RemoveItem` _returnvalue _outitem)
    (`GameplayStatics.OpenLevelBySoftObjectPtr` _outitem)
    (`/Engine/EditorBlueprintResources/StandardMacros.IncrementInt` (`self.CurrentRoomCount`))))

(event `Clear All`
  (set `self.CurrentJoinCount` 0)
  (set `self.CurrentRoomCount` 0)
  ;[0 0.15 0.147 0.502] Clears local players and players and maps
  (for _index (range 1 4)
    (bind _returnvalue (`GameplayStatics.GetPlayerControllerFromID` _index))
    (`/Engine/EditorBlueprintResources/StandardMacros.IsValid` _returnvalue
      (:`Is Valid`
        (`GameplayStatics.RemovePlayer` _returnvalue))))
  (`BlueprintMapLibrary.Map_Clear` (`self.EquippedWeaponsMap`))
  (`BlueprintMapLibrary.Map_Clear` (`self.PlayerBuffData`))
  (`BlueprintMapLibrary.Map_Clear` (`self.JoinedPlayersMap`)))