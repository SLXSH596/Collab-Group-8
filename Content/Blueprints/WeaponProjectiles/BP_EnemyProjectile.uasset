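; Enemy projectile actor that damages whatever its collision sphere hits, using the arrow damage type.
; On spawn it sets a short lifespan and makes the sphere ignore its owner while moving.
; On hit it stops projectile movement, disables collision, applies base damage credited to the owner, then shortens its lifespan so it disappears shortly after impact.
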(event `self.ReceiveBeginPlay`
  ;[0 0.15 0.147 0.502] Begin Play Logic
  (`self.SetLifeSpan` 2.0)
  (`PrimitiveComponent.IgnoreActorWhenMoving` (`self.Sphere`) (`self.GetOwner`) true))

(event `self.Sphere.OnComponentHit`
  (params (HitComponent :type "PrimitiveComponent Object Reference") (OtherActor :type "Actor Object Reference") (OtherComp :type "PrimitiveComponent Object Reference") (NormalImpulse :type "Vector Structure") (Hit :type "HitResult Structure (by ref)"))
  ;[0 0.15 0.147 0.502] Hit AnythingLogic
  (`ActorComponent.Deactivate` (`self.ProjectileMovement`))
  (`PrimitiveComponent.SetCollisionEnabled` (`self.Sphere`) "NoCollision")
  (`GameplayStatics.ApplyDamage` (`.HitActor` (`GameplayStatics.BreakHitResult` Hit)) (`self.BaseDamage`) null (`self.GetOwner`) "/Game/Blueprints/WeaponDamageTypes/BP_DamageType_Arrow.BP_DamageType_Arrow_C")
  (`self.SetLifeSpan` 0.2))

(fn `UserConstructionScript`)