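; Arrow projectile that damages whatever actor it hits and has a short lifespan in case it hits nothing.
; On sphere hit it stops projectile movement, disables collision, applies arrow-type damage credited to its owner, and briefly lingers before expiring.
; FriendlyFireCheck treats an exact BP_Player class match as friendly fire, scaling base damage by the friendly-fire multiplier.
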(event `self.ReceiveBeginPlay`
  ;[0 0.15 0.147 0.502] Begin Play Logic
  (`self.SetLifeSpan` 2.0))

(event `self.Sphere.OnComponentHit`
  (params (HitComponent :type "PrimitiveComponent Object Reference") (OtherActor :type "Actor Object Reference") (OtherComp :type "PrimitiveComponent Object Reference") (NormalImpulse :type "Vector Structure") (Hit :type "HitResult Structure (by ref)"))
  (bind _returnvalue (`self.GetOwner`))
  ;[0 0.15 0.147 0.502] Hit AnythingLogic
  (`ActorComponent.Deactivate` (`self.ProjectileMovement`))
  (`PrimitiveComponent.SetCollisionEnabled` (`self.Sphere`) "NoCollision")
  (bind (_hitactor _bwasfriendlyfire) (`self.FriendlyFireCheck` Hit))
  (if (not _bwasfriendlyfire)
    (`GameplayStatics.ApplyDamage` _hitactor (`self.BaseDamage`) null _returnvalue "/Game/Blueprints/WeaponDamageTypes/BP_DamageType_Arrow.BP_DamageType_Arrow_C")
    (else
      (`GameplayStatics.ApplyDamage` _hitactor (* (`self.BaseDamage`) (`self.FriendlyFireMultiplier`)) null _returnvalue "/Game/Blueprints/WeaponDamageTypes/BP_DamageType_Arrow.BP_DamageType_Arrow_C")))
  (`self.SetLifeSpan` 0.5))

(fn `FriendlyFireCheck`
  (params (Hit :type "HitResult Structure (by ref)"))
  (returns (HitActor :type "Actor Object Reference") (bWasFriendlyFire :type Boolean))
  (bind (_bblockinghit _binitialoverlap _time _distance _location _impactpoint _normal _impactnormal _physmat _hitactor) (`GameplayStatics.BreakHitResult` Hit))
  (if (== (`GameplayStatics.GetObjectClass` _hitactor) "/Game/Blueprints/Player/BP_Player.BP_Player_C")
    (return _hitactor true)
    (else
      (return _hitactor false))))

(fn `UserConstructionScript`)