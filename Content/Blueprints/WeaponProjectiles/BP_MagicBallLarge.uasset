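; Large magic projectile that deals magic damage on impact and sets off an explosion, with flight and impact sounds.
; A hit stops movement, then a sphere trace applies quarter splash damage, gated by DoOnce to one traced hit.
; Any BP_Player counts as friendly fire, taking multiplier-scaled damage, or negative damage as healing when the game mode's HealOnHit is set.
; A direct heal hit skips the explosion.
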(event `self.ReceiveDestroyed`
  ;[0 0.15 0.147 0.502] Looping sound so must be stopped on destroy
  (`/Engine/EditorBlueprintResources/StandardMacros.IsValid` (`self.FlyingProjSound`)
    (:`Is Valid`
      (`AudioComponent.Stop` (`self.FlyingProjSound`)))))

(event `self.ReceiveBeginPlay`
  ;[0 0.15 0.147 0.502] Begin Play Logic
  (bind _returnvalue (`GameplayStatics.SpawnSoundAttached` "/Game/Audio/MetaSounds/SFX/MS_Magic_Impacts.MS_Magic_Impacts" (`self.MagicBallMesh`) "None" (0.0 0.0 0.0) (struct) "KeepRelativeOffset" false 1.0 1.0 0.0 null "/Game/Audio/SoundConcs/CONC_Projectiles.CONC_Projectiles"))
  (`/Engine/EditorBlueprintResources/StandardMacros.IsValid` _returnvalue
    (:`Is Valid`
      (`AudioParameterControllerInterface.SetIntParameter` _returnvalue "State" 0))
    (:`Is Not Valid`
      _))
  (bind _returnvalue_2 (`GameplayStatics.SpawnSoundAttached` "/Game/Audio/MetaSounds/Weapons/MS_Spell_Fireball_Fly.MS_Spell_Fireball_Fly" (`self.MagicBallMesh`) "None" (0.0 0.0 0.0) (struct) "KeepRelativeOffset" false 1.0 1.0 0.0 null null))
  (set `self.FlyingProjSound` _returnvalue_2)
  (`self.SetLifeSpan` 5.0)
  (`PrimitiveComponent.IgnoreActorWhenMoving` (`self.Sphere`) (`self.GetOwner`) true))

(event `self.Sphere.OnComponentHit`
  (params (HitComponent :type "PrimitiveComponent Object Reference") (OtherActor :type "Actor Object Reference") (OtherComp :type "PrimitiveComponent Object Reference") (NormalImpulse :type "Vector Structure") (Hit :type "HitResult Structure (by ref)"))
  (bind _returnvalue (`self.GetOwner`))
  (bind _sphere (`self.Sphere`))
  ;[0 0.15 0.147 0.502] Hit Anything Logic
  (bind _returnvalue_2 (`GameplayStatics.SpawnSoundAtLocation` "/Game/Audio/MetaSounds/SFX/MS_Magic_Impacts.MS_Magic_Impacts" (`self.K2_GetActorLocation`) (struct) 1.0 1.0 0.0 null null))
  (`/Engine/EditorBlueprintResources/StandardMacros.IsValid` _returnvalue_2
    (:`Is Valid`
      (`AudioParameterControllerInterface.SetIntParameter` _returnvalue_2 "State" 1))
    (:`Is Not Valid`
      _))
  (`ActorComponent.Deactivate` (`self.ProjectileMovement`))
  (`PrimitiveComponent.SetCollisionEnabled` (`self.Sphere`) "NoCollision")
  (bind (_hitactor _bwasfriendlyfire) (`self.FriendlyFireCheck` Hit))
  (if (not _bwasfriendlyfire)
    (`GameplayStatics.ApplyDamage` _hitactor (* (`self.BaseDamage`) (`self.HAM`)) null _returnvalue "/Game/Blueprints/WeaponDamageTypes/BP_DamageType_Magic.BP_DamageType_Magic_C")
    (`self.SetLifeSpan` 0.1 :!label _label)
    (`self.Explosion Damage`)
    (`NiagaraFunctionLibrary.SpawnSystemAtLocation` "/Game/VFX/NiagaraSystem/Fire/NS_Shockwave_Red_Testing.NS_Shockwave_Red_Testing" (`SceneComponent.K2_GetComponentLocation` _sphere) (`SceneComponent.K2_GetComponentRotation` _sphere))
    (else
      (bind _asbp_game_mode (cast `/Game/Blueprints/Player/BP_Gamemode` (`GameplayStatics.GetGameMode`)))
      (if (`/Game/Blueprints/Player/BP_Gamemode.HealOnHit?` _asbp_game_mode)
        (`GameplayStatics.ApplyDamage` _hitactor -2.0 null _returnvalue "/Game/Blueprints/WeaponDamageTypes/BP_DamageType_Sword.BP_DamageType_Sword_C")
        (else
          (`GameplayStatics.ApplyDamage` _hitactor (* (* (`self.BaseDamage`) (`self.HAM`)) (`self.FriendlyFireMultiplier`)) null _returnvalue "/Game/Blueprints/WeaponDamageTypes/BP_DamageType_Magic.BP_DamageType_Magic_C")
          (goto _label))))))

(event `Explosion Damage`
  (bind _returnvalue (`self.GetOwner`))
  (bind _returnvalue_2 (`SceneComponent.K2_GetComponentLocation` (`self.Sphere`)))
  ;[0.06301 0.6939 0.1441] Explosion Damage
  (bind (_outhits _returnvalue_3) (`KismetSystemLibrary.SphereTraceMultiForObjects` _returnvalue_2 _returnvalue_2 200.0 (`self.Default Object Type`) false (`|MakeArray` (stale `self.Sphere.OnComponentHit` OtherActor)) "None" true (struct :`R` 1.0 :`A` 1.0) (struct :`G` 1.0 :`A` 1.0) 1.0))
  (if _returnvalue_3
    (for _array_element _outhits
      (`/Engine/EditorBlueprintResources/StandardMacros.DoOnce` false
        (:`Completed`
          (bind (_hitactor _bwasfriendlyfire) (`self.FriendlyFireCheck` _array_element))
          (if (not _bwasfriendlyfire)
            (`GameplayStatics.ApplyDamage` _hitactor (* (/ (`self.BaseDamage`) 4.0) (`self.HAM`)) null _returnvalue "/Game/Blueprints/WeaponDamageTypes/BP_DamageType_Magic.BP_DamageType_Magic_C")
            (else
              (bind _asbp_game_mode (cast `/Game/Blueprints/Player/BP_Gamemode` (`GameplayStatics.GetGameMode`)))
              (if (`/Game/Blueprints/Player/BP_Gamemode.HealOnHit?` _asbp_game_mode)
                (`GameplayStatics.ApplyDamage` null -3.0 null null "/Game/Blueprints/WeaponDamageTypes/BP_DamageType_Sword.BP_DamageType_Sword_C")
                (else
                  (`GameplayStatics.ApplyDamage` _hitactor (* (* (/ (`self.BaseDamage`) 4.0) (`self.HAM`)) (`self.FriendlyFireMultiplier`)) null _returnvalue "/Game/Blueprints/WeaponDamageTypes/BP_DamageType_Magic.BP_DamageType_Magic_C"))))))))))

(fn `FriendlyFireCheck`
  (params (Hit :type "HitResult Structure (by ref)"))
  (returns (HitActor :type "Actor Object Reference") (bWasFriendlyFire :type Boolean))
  (bind (_bblockinghit _binitialoverlap _time _distance _location _impactpoint _normal _impactnormal _physmat _hitactor) (`GameplayStatics.BreakHitResult` Hit))
  (if (== (`GameplayStatics.GetObjectClass` _hitactor) "/Game/Blueprints/Player/BP_Player.BP_Player_C")
    (return _hitactor true)
    (else
      (return _hitactor false))))

(fn `UserConstructionScript`)