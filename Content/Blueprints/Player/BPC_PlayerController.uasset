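; Player controller for local multiplayer that routes Enhanced Input movement, light/heavy attacks and pause to its possessed BP_Player.
; Player zero alone creates the HUD, binds to game-over and device-connection events, and can pause; a controller disconnect also toggles pause.
; Possession initializes the pawn, input mapping and controller rumble component, which fires on attacks.
; Win, lose and modifier pop-up events forward to the HUD, with a win also clearing the player count.
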(event `/Game/Interfaces/BPI_PlayerController.Init`
  (params (GameMode :type "/Game/Blueprints/Player/BP_Gamemode Object Reference"))
  ; Init Logic
  (bind _output_get (set `self.GameMode` GameMode))
  (set `self.GameInstance` (`/Game/Blueprints/Player/BP_Gamemode.GameInstance` _output_get))
  ;;[0.162 0.02956 0.3515] Only do UI setup etc. if this is the first player controller
  (`self.CheckPlayerZero`
    (:`Player 0`
      ;;[0.162 0.02956 0.3515] HUD Setup
      (bind _returnvalue (`|CreateWidget` "/Game/UI/HUD/WBP_HUD.WBP_HUD_C"))
      (bind _output_get_2 (set `self.HUD` _returnvalue))
      (`/Game/UI/HUD/WBP_HUD.Init` _output_get_2 (`/Game/Blueprints/GI_GameInstance.CurrentJoinCount` (`self.GameInstance`)))
      (`UserWidget.AddToViewport` _output_get_2 0)
      (bind _ac_playermanager (`/Game/Blueprints/Player/BP_Gamemode.AC_PlayerManager` _output_get))
      (`/Engine/EditorBlueprintResources/StandardMacros.IsValid` _ac_playermanager
        (:`Is Valid`
          (bind _output_get_3 (set `self.Player Manager` _ac_playermanager))
          ;;[0.06301 0.6939 0.1441] Death Setup
          (add `/Game/Components/GameMode/AC_PlayerManager.OnGameOver` _output_get_3 (`|CreateDelegate` :!event `LoseGame`))
          ;[1 1 1] Triggers when a controller is disconnected
          (add `GameInstance.OnInputDeviceConnectionChange` (`self.GameInstance`) (`|CreateDelegate` :!event `Controller Disconnected`)))))))

(event `EnhancedInput|/Game/Input/IA_PrimaryAttack`
  (params (ActionValue :type Boolean) (ElapsedSeconds :type "Float (double-precision)") (TriggeredSeconds :type "Float (double-precision)") (InputAction :type "InputAction Object Reference" :default "/Game/Input/IA_PrimaryAttack.IA_PrimaryAttack"))
  (bind _playerpawn (`self.PlayerPawn`))
  (bind _ac_controllerrumble (`self.AC_ControllerRumble`))
  ;[0 0.15 0.147 0.502] Attack Setup
  (:`Triggered`
    ;;[0.06301 0.6939 0.1441] Attack Controller Rumble
    (`/Game/Components/Controllers/AC_ControllerRumble.Heavy Attack FF` _ac_controllerrumble)
    (`/Game/Blueprints/Player/BP_Player.HeavyAttack` _playerpawn))
  (:`Canceled`
    (`/Game/Components/Controllers/AC_ControllerRumble.Light Attack FF` _ac_controllerrumble)
    (`/Game/Blueprints/Player/BP_Player.PrimaryAttack` _playerpawn)))

(event `Controller Disconnected`
  (params (NewConnectionState :type "EInputDeviceConnectionState Enum" :default "Invalid") (PlatformUserId :type "PlatformUserId Structure") (InputDeviceId :type "InputDeviceId Structure"))
  ;[1 1 1] Pauses Game on disconnect
  (if (`|EnumEquality` NewConnectionState "Disconnected")
    ;;[1 1 1] TODO: Change this to something different - maybe a specific screen saying a controller has been disconected
    (`/Game/UI/HUD/WBP_HUD.TogglePause` (`self.HUD`))))

(event `EnhancedInput|/Game/Input/IA_Movement`
  (params (ActionValue :type "Vector2D Structure") (ElapsedSeconds :type "Float (double-precision)") (TriggeredSeconds :type "Float (double-precision)") (InputAction :type "InputAction Object Reference" :default "/Game/Input/IA_Movement.IA_Movement"))
  ; Movement
  (:`Triggered`
    (`Pawn.AddMovementInput` (`self.PlayerPawn`) (`KismetMathLibrary.Conv_Vector2DToVector` ActionValue) 1.0 false)))

(event `self.ReceivePossess`
  (params (PossessedPawn :type "Pawn Object Reference"))
  (bind _output_get (set `self.PlayerPawn` (cast `/Game/Blueprints/Player/BP_Player` PossessedPawn :!pure true)))
  (`/Game/Blueprints/Player/BP_Player.Init` _output_get self)
  (`EnhancedInputSubsystemInterface.AddMappingContext` (subsystem `EnhancedInputLocalPlayerSubsystem`) "/Game/Input/IMC_Controls.IMC_Controls" 0 (struct))
  ;[0.06301 0.6939 0.1441] Int controller rumble
  (`/Game/Components/Controllers/AC_ControllerRumble.Initialise` (`self.AC_ControllerRumble`) (`self.PlayerPawn`) self null))

(event `EnhancedInput|/Game/Input/IA_Pause`
  (params (ActionValue :type Boolean) (ElapsedSeconds :type "Float (double-precision)") (TriggeredSeconds :type "Float (double-precision)") (InputAction :type "InputAction Object Reference" :default "/Game/Input/IA_Pause.IA_Pause"))
  (:`Started`
    ;[0.162 0.02956 0.3515] Maybe allow other players to pause?
    (`self.CheckPlayerZero`
      (:`Player 0`
        (`/Game/UI/HUD/WBP_HUD.TogglePause` (`self.HUD`))))))

(event `LoseGame`
  (bind _hud (`self.HUD`))
  ;[0.162 0.02956 0.3515] Lose
  (`/Engine/EditorBlueprintResources/StandardMacros.IsValid` _hud
    (:`Is Valid`
      (`/Game/UI/HUD/WBP_HUD.DisplayEnd` _hud false))))

(event `/Game/Interfaces/BPI_PlayerController.WinGame`
  (bind _hud (`self.HUD`))
  ;[0.162 0.02956 0.3515] Win
  (`/Engine/EditorBlueprintResources/StandardMacros.IsValid` _hud
    (:`Is Valid`
      (`/Game/Blueprints/GI_GameInstance.Clear Player Count` (`self.GameInstance`))
      (`/Game/UI/HUD/WBP_HUD.DisplayEnd` _hud true))))

(event `/Game/Interfaces/BPI_PlayerController.DisplayModifierPopUp`
  (params (Name :type Name) (Description :type Text))
  (bind _hud (`self.HUD`))
  ;[0.162 0.02956 0.3515] Modifier PopUp
  (`/Engine/EditorBlueprintResources/StandardMacros.IsValid` _hud
    (:`Is Valid`
      (`/Game/UI/HUD/WBP_HUD.DisplayModifierPopUp` _hud Name Description))))

(fn `UserConstructionScript`)