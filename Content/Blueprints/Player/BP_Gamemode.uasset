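; Game mode for a local multiplayer, room-based game that sets up players, a random modifier and room progression with loot.
; BeginPlay spawns and possesses joined players at slot-matched locations with their chosen weapons, creating debug players if none joined, then adds a shared camera and disables input.
; FinishedLoad restores input once, shows the modifier popup and starts the room and enemy managers.
; UpdateRooms completes the room and drops chest loot.
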(event `self.ReceiveBeginPlay`
  (bind _gameinstance (`self.GameInstance`))
  (bind _gameinstance_2 (`self.GameInstance`))
  (bind _output_get (set `self.GameInstance` (cast `/Game/Blueprints/GI_GameInstance` (`GameplayStatics.GetGameInstance`) :!pure true)))
  (`GameplayStatics.SpawnSound2D` "/Game/Audio/SW_GameMusicLoop.SW_GameMusicLoop" 1.0 1.0 0.0 null)
  ;[0 0.15 0.147 0.502] Very important for debug testing
  (`/Engine/EditorBlueprintResources/StandardMacros.IsValid` _output_get
    (:`Is Valid`
      (if (not (not (== (`/Game/Blueprints/GI_GameInstance.CurrentJoinCount` _output_get) 0)))
        ;[0 0.15 0.147 0.502] Testing Logic
        (`BlueprintMapLibrary.Map_Add` (`/Game/Blueprints/GI_GameInstance.JoinedPlayersMap` _gameinstance_2) 0 1)
        (`/Engine/EditorBlueprintResources/StandardMacros.IncrementInt` (`/Game/Blueprints/GI_GameInstance.CurrentJoinCount` _gameinstance_2)
          (:`  `
            (for _index (range 1 (`self.DebugPlayerCount`))
              (bind _returnvalue (`GameplayStatics.CreatePlayer` _index))
              (`BlueprintMapLibrary.Map_Add` (`/Game/Blueprints/GI_GameInstance.JoinedPlayersMap` (`self.GameInstance`)) (`GameplayStatics.GetPlayerControllerID` _returnvalue) (+ _index 1))
              (`/Engine/EditorBlueprintResources/StandardMacros.IncrementInt` (`/Game/Blueprints/GI_GameInstance.CurrentJoinCount` (`self.GameInstance`)))))))
      (bind _outactors (`GameplayStatics.GetAllActorsOfClass` "/Game/Blueprints/LevelActors/BP_EmptySpawnLocation.BP_EmptySpawnLocation_C"))
      (set `self.SpawnLocations` _outactors)
      (for _index_2 (range (`GameplayStatics.GetNumLocalPlayerControllers`))
        (bind _returnvalue_2 (`GameplayStatics.GetPlayerController` _index_2))
        (bind _returnvalue_3 (`GameplayStatics.GetPlayerControllerID` _returnvalue_2))
        (bind (_value _returnvalue_4) (`BlueprintMapLibrary.Map_Find` (`/Game/Blueprints/GI_GameInstance.JoinedPlayersMap` _gameinstance) _returnvalue_3))
        (if _returnvalue_4
          (for _array_element (`self.SpawnLocations`)
            (if (== (`/Game/Blueprints/LevelActors/BP_EmptySpawnLocation.PlayerSlot` _array_element) _value)
              (bind _returnvalue_5 (`|SpawnActorFromClass` "/Game/Blueprints/Player/BP_Player.BP_Player_C" (`self.GetTransform` _array_element) "Undefined" "MultiplyWithRoot" null null))
              (`KismetArrayLibrary.Array_Add` (`self.PlayerControllers`) _returnvalue_2)
              (message `/Game/Interfaces/BPI_PlayerController.Init` _returnvalue_2 _gameinstance self)
              (`Controller.Possess` _returnvalue_2 _returnvalue_5)
              (set `/Game/Blueprints/Player/BP_Player.ChosenWeaponType` (`BlueprintMapLibrary.Map_Find` (`/Game/Blueprints/GI_GameInstance.EquippedWeaponsMap` _gameinstance) _returnvalue_3) _returnvalue_5)
              (`/Game/Blueprints/Player/BP_Player.SetCurrentWeapon` _returnvalue_5)))))
      (bind _returnvalue_6 (`|SpawnActorFromClass` "/Game/Blueprints/LevelActors/BP_Camera.BP_Camera_C" (`KismetMathLibrary.MakeTransform` (0.0 0.0 0.0)) "Undefined" "MultiplyWithRoot" null null))
      (`/Game/Blueprints/LevelActors/BP_Camera.UpdateControllers` _returnvalue_6 (`self.PlayerControllers`))
      (`/Game/Components/GameMode/AC_PlayerManager.Initialise` (`self.AC_PlayerManager`))
      (`/Game/Components/GameMode/AC_PickupSpawning.Initialise` (`self.AC_PickupSpawning`) self)
      (bind _returnvalue_7 (`|AddComponentByClass` (`KismetArrayLibrary.Array_Random` (`self.Modifiers`))))
      (set `self.Modifier` _returnvalue_7)
      (for _array_element_2 (`self.PlayerControllers`)
        (`self.DisableInput` _array_element_2 _array_element_2)
        (`self.DisableInput` (`Controller.K2_GetPawn` _array_element_2) _array_element_2)))))

(event `FinishedLoad`
  (params (InitialiseDelay :type "Float (double-precision)"))
  (bind _ac_enemymanager (`self.AC_EnemyManager`))
  (bind _modifier (`self.Modifier`))
  (`/Engine/EditorBlueprintResources/StandardMacros.DoOnce` false
    (:`Completed`
      (for _array_element (`self.PlayerControllers`)
        (bind _returnvalue (`Controller.K2_GetPawn` _array_element))
        (message `/Game/Interfaces/BPI_PlayerInterface.PostLoad` _returnvalue)
        (`self.EnableInput` _array_element _array_element)
        (`self.EnableInput` _returnvalue _array_element))
      (`KismetSystemLibrary.Delay` InitialiseDelay)
      (message `/Game/Interfaces/BPI_PlayerController.DisplayModifierPopUp` (`/Game/Blueprints/BPFL_CommonFunctions.FindFirstPlayerController` (`self.GameInstance`) true) (`/Game/Components/Modifiers/AC_RoomModifierBase.ModifierName` _modifier) (`KismetTextLibrary.Conv_NameToText` (`/Game/Components/Modifiers/AC_RoomModifierBase.ModifierDescription` _modifier)))
      (bind _returnvalue_2 (`GameplayStatics.GetActorOfClass` "/Game/Blueprints/LevelManagement/BP_RoomExitDoor.BP_RoomExitDoor_C"))
      (`/Engine/EditorBlueprintResources/StandardMacros.IsValid` _returnvalue_2
        (:`Is Valid`
          (`/Game/Components/GameMode/AC_RoomManager.Initialise` (`self.AC_RoomManager`) self _returnvalue_2)
          (add `/Game/Components/GameMode/AC_EnemyManager.OnRoomComplete` _ac_enemymanager (`|CreateDelegate` :!event `UpdateRooms`))
          (`/Game/Components/GameMode/AC_EnemyManager.Init` _ac_enemymanager)
          (bind _returnvalue_3 (`GameplayStatics.GetActorOfClass` "/Game/Blueprints/Pickup/BP_LootChest.BP_LootChest_C"))
          (set `self.Loot Chest` _returnvalue_3))))))

(event `UpdateRooms`
  ;[0.162 0.02956 0.3515] Open the door and stuff
  (`/Game/Components/GameMode/AC_RoomManager.Room Completed` (`self.AC_RoomManager`))
  ;[1 1 1] Drops loot
  (`/Game/Blueprints/Pickup/BP_LootChest.Drop Loot` (`self.Loot Chest`)))

(fn `UserConstructionScript`)