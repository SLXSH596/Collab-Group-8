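; Player controller for the main menu, which puts up the menu UI and handles starting the game.
; On BeginPlay it caches the GI_GameInstance and creates WBP_MainMenuParent, adding it to the viewport with focus.
; Its StartGame event opens the LVL_StartLobby level, provided the cached game instance is valid.
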(event `self.ReceiveBeginPlay`
  (set `self.GameInstance` (cast `/Game/Blueprints/GI_GameInstance` (`GameplayStatics.GetGameInstance`) :!pure true))
  (bind _returnvalue (`|CreateWidget` "/Game/UI/MainMenu/WBP_MainMenuParent.WBP_MainMenuParent_C" self))
  (bind _output_get (set `self.Menu` _returnvalue))
  (`UserWidget.AddToViewport` _output_get 0)
  (`Widget.SetFocus` _output_get))

(event `Start Game`
  (`/Engine/EditorBlueprintResources/StandardMacros.IsValid` (`self.GameInstance`)
    (:`Is Valid`
      (`GameplayStatics.OpenLevelBySoftObjectPtr` "/Game/Maps/LVL_StartLobby.LVL_StartLobby"))))

(fn `UserConstructionScript`)