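; Player controller for local multiplayer that handles movement, attacks, pausing and lobby joining.
; A timer on held attack input slows the pawn and turns release into a heavy attack instead of a primary one.
; The first controller owns the shared HUD for player info, health, end screens, modifier pop-ups and disconnect pauses.
; Joining registers the player, moves the pawn to its slot, triggers rumble and swaps lobby input for game controls.
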(event `/Game/Interfaces/BPI_PlayerController.Init`
  (params (GameInstance :type "/Game/Blueprints/GI_GameInstance Object Reference") (OptionalGameMode :type "/Game/Blueprints/Player/BP_Gamemode Object Reference"))
  (bind _gameinstance (`self.GameInstance`))
  ; Init Logic
  (bind _output_get (set `self.GameInstance` GameInstance))
  (`/Engine/EditorBlueprintResources/StandardMacros.IsValid` _output_get
    (:`Is Valid`
      (bind _output_get_2 (set `self.Optional Game Mode` OptionalGameMode))
      ;[1 1 1] Triggers when a controller is disconnected
      (add `GameInstance.OnInputDeviceConnectionChange` _gameinstance (`|CreateDelegate` :!event `Controller Disconnected`))
      (bind _firstplayercontroller (`/Game/Blueprints/BPFL_CommonFunctions.FindFirstPlayerController` _gameinstance (`KismetSystemLibrary.IsValid` _output_get_2)))
      ;[0.162 0.02956 0.3515] HUD Setup
      (if (== _firstplayercontroller self)
        (bind _returnvalue (`|CreateWidget` "/Game/UI/HUD/WBP_HUD.WBP_HUD_C"))
        (bind _output_get_3 (set `self.HUD` _returnvalue))
        (`UserWidget.AddToViewport` _output_get_3 0)
        (`/Engine/EditorBlueprintResources/StandardMacros.IsValid` _output_get_2
          (:`Is Valid`
            (`/Game/Interfaces/BPI_PlayerController.UpdatePlayerInfoNum` self)
            (bind _output_get_4 (set `self.Player Manager` (`/Game/Blueprints/Player/BP_Gamemode.AC_PlayerManager` _output_get_2)))
            (add `/Game/Components/GameMode/AC_PlayerManager.OnGameOver` _output_get_4 (`|CreateDelegate` :!event `LoseGame`))))
        (else
          (`/Engine/EditorBlueprintResources/StandardMacros.IsValid` _output_get_2
            (:`Is Valid`
              (message `/Game/Interfaces/BPI_PlayerController.UpdatePlayerInfoNum` _firstplayercontroller self))))))
    (:`Is Not Valid`
      (`KismetSystemLibrary.RaiseScriptError` "Game Instance Not Valid"))))

(event `EnhancedInput|/Game/Input/IA_PrimaryAttack`
  (params (ActionValue :type Boolean) (ElapsedSeconds :type "Float (double-precision)") (TriggeredSeconds :type "Float (double-precision)") (InputAction :type "InputAction Object Reference" :default "/Game/Input/IA_PrimaryAttack.IA_PrimaryAttack"))
  (bind _playerpawn (`self.PlayerPawn`))
  (bind _attacktimerhandle (`self.AttackTimerHandle`))
  ;[0 0.15 0.147 0.502] Attack Setup
  (:`Started`
    (bind _returnvalue (`KismetSystemLibrary.K2_SetTimerDelegate` (delegate `Heavy Attack Ready`) (* (`/Game/Components/Weapons/AC_WeaponBase.AttackCooldown` (`/Game/Blueprints/Player/BP_Player.CurrentWeapon` (`self.PlayerPawn`))) 1.5)))
    (set `self.AttackTimerHandle` _returnvalue))
  (:`Completed`
    (if (`/Game/Blueprints/Player/BP_Player.bCanAttack` (`self.PlayerPawn`))
      (set `CharacterMovementComponent.MaxWalkSpeed` (`self.WalkSpeed`) (`Character.CharacterMovement` (`self.PlayerPawn`)))
      (if (`KismetSystemLibrary.K2_IsTimerActiveHandle` _attacktimerhandle)
        (`KismetSystemLibrary.K2_ClearAndInvalidateTimerHandle` _attacktimerhandle)
        (`/Game/Blueprints/Player/BP_Player.PrimaryAttack` _playerpawn)
        (else
          (`/Game/Blueprints/Player/BP_Player.HeavyAttack` _playerpawn)
          (set `CharacterMovementComponent.MaxWalkSpeed` (`self.WalkSpeed`) (`Character.CharacterMovement` (`self.PlayerPawn`))))))))

(event `Heavy Attack Ready`
  ;[0 0.15 0.147 0.502] Attack Setup
  (set `CharacterMovementComponent.MaxWalkSpeed` (/ (`self.WalkSpeed`) 2.0) (`Character.CharacterMovement` (`self.PlayerPawn`))))

(event `self.ReceivePossess`
  (params (PossessedPawn :type "Pawn Object Reference"))
  (bind _returnvalue (subsystem `EnhancedInputLocalPlayerSubsystem`))
  ;[0.162 0.02956 0.3515] Possession Logic
  (bind _output_get (set `self.PlayerPawn` (cast `/Game/Blueprints/Player/BP_Player` PossessedPawn :!pure true)))
  (set `self.WalkSpeed` (`CharacterMovementComponent.MaxWalkSpeed` (`Character.CharacterMovement` _output_get)))
  ;;[0.162 0.02956 0.3515] Check if we are in game or the lobby
  (`/Engine/EditorBlueprintResources/StandardMacros.IsValid` (`self.Optional Game Mode`)
    (:`Is Valid`
      (`/Game/Blueprints/Player/BP_Player.Init` _output_get self)
      (`EnhancedInputSubsystemInterface.AddMappingContext` _returnvalue "/Game/Input/IMC_Controls.IMC_Controls" 0 (struct))
      ;;[0.06301 0.6939 0.1441] Int controller rumble
      (`/Game/Components/Controllers/AC_ControllerRumble.Initialise` (`self.AC_ControllerRumble`) (`self.PlayerPawn`) self))
    (:`Is Not Valid`
      (`EnhancedInputSubsystemInterface.AddMappingContext` _returnvalue "/Game/Input/IMC_LobbyControls.IMC_LobbyControls" 0 (struct)))))

(event `EnhancedInput|/Game/Input/IA_Movement`
  (params (ActionValue :type "Vector2D Structure") (ElapsedSeconds :type "Float (double-precision)") (TriggeredSeconds :type "Float (double-precision)") (InputAction :type "InputAction Object Reference" :default "/Game/Input/IA_Movement.IA_Movement"))
  ; Movement
  (:`Triggered`
    (`Pawn.AddMovementInput` (`self.PlayerPawn`) (`KismetMathLibrary.Conv_Vector2DToVector` ActionValue) 1.0 false)))

(event `Controller Disconnected`
  (params (NewConnectionState :type "EInputDeviceConnectionState Enum" :default "Invalid") (PlatformUserId :type "PlatformUserId Structure") (InputDeviceId :type "InputDeviceId Structure"))
  ;[1 1 1] Pauses Game on disconnect
  (if (`|EnumEquality` NewConnectionState "Disconnected")
    ;;[1 1 1] TODO: Change this to something different - maybe a specific screen saying a controller has been disconected
    (`/Game/UI/HUD/WBP_HUD.TogglePause` (`self.HUD`))))

(event `/Game/Interfaces/BPI_PlayerController.UpdateUI`
  (params (PlayerIndex :type Integer) (NewPercentage :type "Float (double-precision)"))
  (bind _hud (`self.HUD`))
  ;[0.162 0.02956 0.3515] Health Updates
  (`/Engine/EditorBlueprintResources/StandardMacros.IsValid` _hud
    (:`Is Valid`
      (`/Game/UI/HUD/WBP_HUD.UpdateHealthValue` _hud PlayerIndex NewPercentage))))

(event `EnhancedInput|/Game/Input/IA_Pause`
  (params (ActionValue :type Boolean) (ElapsedSeconds :type "Float (double-precision)") (TriggeredSeconds :type "Float (double-precision)") (InputAction :type "InputAction Object Reference" :default "/Game/Input/IA_Pause.IA_Pause"))
  (:`Started`
    ;[0.162 0.02956 0.3515] Maybe allow other players to pause?
    (`self.CheckPlayerZero`
      (:`Player 0`
        (`/Game/UI/HUD/WBP_HUD.TogglePause` (`self.HUD`))))))

(event `/Game/Interfaces/BPI_PlayerController.UpdatePlayerInfoNum`
  (params (NewController :type "PlayerController Object Reference"))
  (bind _hud (`self.HUD`))
  ;[0.162 0.02956 0.3515] Update the UI on player 0 if it is valid
  (`/Engine/EditorBlueprintResources/StandardMacros.IsValid` _hud
    (:`Is Valid`
      (`/Game/UI/HUD/WBP_HUD.AddPlayerInfo` _hud (`GameplayStatics.GetPlayerControllerID` NewController)))))

(event `LoseGame`
  (bind _hud (`self.HUD`))
  ;[0.162 0.02956 0.3515] Lose
  (`/Engine/EditorBlueprintResources/StandardMacros.IsValid` _hud
    (:`Is Valid`
      (`/Game/UI/HUD/WBP_HUD.DisplayEnd` _hud false))))

(event `/Game/Interfaces/BPI_PlayerController.WinGame`
  (bind _hud (`self.HUD`))
  ;[0.162 0.02956 0.3515] Win
  (`/Engine/EditorBlueprintResources/StandardMacros.IsValid` _hud
    (:`Is Valid`
      (`/Game/UI/HUD/WBP_HUD.DisplayEnd` _hud true))))

(event `/Game/Interfaces/BPI_PlayerController.DisplayModifierPopUp`
  (params (Name :type Name) (Description :type Text))
  (bind _hud (`self.HUD`))
  ;[0.162 0.02956 0.3515] Modifier PopUp
  (`/Engine/EditorBlueprintResources/StandardMacros.IsValid` _hud
    (:`Is Valid`
      (`/Game/UI/HUD/WBP_HUD.DisplayModifierPopUp` _hud Name Description))))

(event `SetupPlayer`
  (bind _playerpawn (`self.PlayerPawn`))
  ;[0.162 0.02956 0.3515] Called once joined if in lobby
  (`/Engine/EditorBlueprintResources/StandardMacros.IsValid` _playerpawn
    (:`Is Valid`
      (`/Game/Blueprints/Player/BP_Player.Init` _playerpawn self))))

(event `EnhancedInput|/Game/Input/IA_JoinLobby`
  (params (ActionValue :type Boolean) (ElapsedSeconds :type "Float (double-precision)") (TriggeredSeconds :type "Float (double-precision)") (InputAction :type "InputAction Object Reference" :default "/Game/Input/IA_JoinLobby.IA_JoinLobby"))
  (bind _returnvalue (subsystem `EnhancedInputLocalPlayerSubsystem`))
  (bind _ac_controllerrumble (`self.AC_ControllerRumble`))
  (bind _returnvalue_2 (`GameplayStatics.GetPlayerControllerID` self))
  (bind _currentjoincount (`/Game/Blueprints/GI_GameInstance.CurrentJoinCount` (`self.GameInstance`)))
  (bind _joinedplayersmap (`/Game/Blueprints/GI_GameInstance.JoinedPlayersMap` (`self.GameInstance`)))
  (bind _returnvalue_3 (`GameplayStatics.GetPlayerPawn` (`GameplayStatics.GetPlayerControllerID` self)))
  ;[0 0.15 0.147 0.502] New Join Logic
  (:`Started`
    (if (not (`BlueprintMapLibrary.Map_Contains` _joinedplayersmap _returnvalue_2))
      (`BlueprintMapLibrary.Map_Add` _joinedplayersmap _returnvalue_2 (+ _currentjoincount 1))
      (`/Engine/EditorBlueprintResources/StandardMacros.IncrementInt` _currentjoincount
        (:`  `
          (`|ExecutionSequence`
            (:`then_0`
              (`self.SetupPlayer`)
              (message `/Game/Interfaces/BPI_PlayerController.UpdatePlayerInfoNum` (`/Game/Blueprints/BPFL_CommonFunctions.FindFirstPlayerController` (`self.GameInstance`)) self)
              ;;[0.06301 0.6939 0.1441] Join Game Rumble
              (`/Game/Components/Controllers/AC_ControllerRumble.Initialise` _ac_controllerrumble (`self.PlayerPawn`) self)
              (`/Game/Components/Controllers/AC_ControllerRumble.Player Joined FF` _ac_controllerrumble))
            (:`then_1`
              (bind _outactors (`GameplayStatics.GetAllActorsOfClass` "/Game/Blueprints/LevelActors/BP_EmptySpawnLocation.BP_EmptySpawnLocation_C"))
              (for _array_element _outactors
                (if (== (`/Game/Blueprints/LevelActors/BP_EmptySpawnLocation.PlayerSlot` _array_element) (`/Game/Blueprints/GI_GameInstance.CurrentJoinCount` (`self.GameInstance`)))
                  (`|ExecutionSequence`
                    (:`then_0`
                      ;;[0.162 0.02956 0.3515] Prevents hat physics bug as well as giving time for future VFX pop in
                      (`self.SetActorHiddenInGame` _returnvalue_3 true)
                      (`self.K2_SetActorLocation` _returnvalue_3 (`self.K2_GetActorLocation` _array_element) false false)
                      (`KismetSystemLibrary.Delay` 0.15)
                      (`self.SetActorHiddenInGame` _returnvalue_3 false)
                      (`/Game/Blueprints/Player/BP_Player.Init` (`self.PlayerPawn`) self))
                    (:`then_1`
                      ;;[1 1 1] Setting controls to normal ingame controls once joined
                      (`EnhancedInputSubsystemInterface.RemoveMappingContext` _returnvalue "/Game/Input/IMC_LobbyControls.IMC_LobbyControls" (struct))
                      (`EnhancedInputSubsystemInterface.AddMappingContext` _returnvalue "/Game/Input/IMC_Controls.IMC_Controls" 0 (struct))
                      (message `/Game/Interfaces/BPI_LobbyGameMode.PlayerJoined` (`GameplayStatics.GetGameMode`) self))))))))))))

(fn `UserConstructionScript`)