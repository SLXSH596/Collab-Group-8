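; Lobby player controller that lets local players join the lobby and control their BP_Player pawn.
; On possess it applies lobby controls; player 0 also creates the HUD, handling pause and controller-disconnect events.
; Joining records the controller in the GameInstance, moves the pawn to its slot's spawn, switches to gameplay controls and notifies the lobby GameMode.
; Movement and attack input, copied from BPC_PlayerController, drive the pawn, with rumble on attacks and joining.
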(event `EnhancedInput|/Game/Input/IA_PrimaryAttack`
  (params (ActionValue :type Boolean) (ElapsedSeconds :type "Float (double-precision)") (TriggeredSeconds :type "Float (double-precision)") (InputAction :type "InputAction Object Reference" :default "/Game/Input/IA_PrimaryAttack.IA_PrimaryAttack"))
  (bind _playerpawn (`self.PlayerPawn`))
  (bind _ac_controllerrumble (`self.AC_ControllerRumble`))
  ;[1 1 1] Copied over from BPC_PlayerController
  ;;[0 0.15 0.147 0.502] Attack Setup
  (:`Triggered`
    ;;;[0.06301 0.6939 0.1441] Attack Controller Rumble
    (`/Game/Components/Controllers/AC_ControllerRumble.Heavy Attack FF` _ac_controllerrumble)
    (`/Game/Blueprints/Player/BP_Player.HeavyAttack` _playerpawn))
  (:`Canceled`
    (`/Game/Components/Controllers/AC_ControllerRumble.Light Attack FF` _ac_controllerrumble)
    (`/Game/Blueprints/Player/BP_Player.PrimaryAttack` _playerpawn)))

(event `Controller Disconnected`
  (params (NewConnectionState :type "EInputDeviceConnectionState Enum" :default "Invalid") (PlatformUserId :type "PlatformUserId Structure") (InputDeviceId :type "InputDeviceId Structure"))
  ;[1 1 1] Pauses Game on disconnect
  (if (`|EnumEquality` NewConnectionState "Disconnected")
    ;;[1 1 1] TODO: Change this to something different - maybe a specific screen saying a controller has been disconected
    (`/Game/UI/HUD/WBP_HUD.TogglePause` (`self.HUD`))))

(event `self.ReceivePossess`
  (params (PossessedPawn :type "Pawn Object Reference"))
  ;[0 0.15 0.147 0.502] Begin Play
  (`KismetSystemLibrary.DelayUntilNextTick`)
  (`EnhancedInputSubsystemInterface.AddMappingContext` (subsystem `EnhancedInputLocalPlayerSubsystem`) "/Game/Input/IMC_LobbyControls.IMC_LobbyControls" 0 (struct))
  (bind _asbp_lobby_game_mode (cast `/Game/Blueprints/Player/BP_LobbyGameMode` (`GameplayStatics.GetGameMode`)))
  (bind _output_get (set `self.LobbyGameMode` _asbp_lobby_game_mode))
  (set `self.GameInstance` (`/Game/Blueprints/Player/BP_LobbyGameMode.GameInstance` _output_get))
  ;[0.162 0.02956 0.3515] Only do UI setup etc. if this is the first player controller
  (`self.Check Player 0`
    (:`Player 0`
      ;[0.162 0.02956 0.3515] HUD Setup
      (bind _returnvalue (`|CreateWidget` "/Game/UI/HUD/WBP_HUD.WBP_HUD_C"))
      (bind _output_get_2 (set `self.HUD` _returnvalue))
      (`UserWidget.AddToViewport` _output_get_2 0)
      ;[1 1 1] Triggers when a controller is disconnected
      (add `GameInstance.OnInputDeviceConnectionChange` (`self.GameInstance`) (`|CreateDelegate` :!event `Controller Disconnected`)))))

(event `EnhancedInput|/Game/Input/IA_Movement`
  (params (ActionValue :type "Vector2D Structure") (ElapsedSeconds :type "Float (double-precision)") (TriggeredSeconds :type "Float (double-precision)") (InputAction :type "InputAction Object Reference" :default "/Game/Input/IA_Movement.IA_Movement"))
  ;[1 1 1] Manages movement
  (:`Triggered`
    (`Pawn.AddMovementInput` (`self.PlayerPawn`) (`KismetMathLibrary.Conv_Vector2DToVector` ActionValue) 1.0 false)))

(event `SetupPlayer`
  ;[1 1 1] Assigning input mapping
  (bind _output_get (set `self.PlayerPawn` (cast `/Game/Blueprints/Player/BP_Player` (`self.K2_GetPawn`) :!pure true)))
  (`/Game/Blueprints/Player/BP_Player.Init` _output_get self)
  ;;[0.06301 0.6939 0.1441] Int Controller Rumble
  (`/Game/Components/Controllers/AC_ControllerRumble.Initialise` (`self.AC_ControllerRumble`) (`self.PlayerPawn`) null self))

(event `EnhancedInput|/Game/Input/IA_JoinLobby`
  (params (ActionValue :type Boolean) (ElapsedSeconds :type "Float (double-precision)") (TriggeredSeconds :type "Float (double-precision)") (InputAction :type "InputAction Object Reference" :default "/Game/Input/IA_JoinLobby.IA_JoinLobby"))
  (bind _returnvalue (subsystem `EnhancedInputLocalPlayerSubsystem`))
  (bind _returnvalue_2 (`GameplayStatics.GetPlayerControllerID` self))
  (bind _currentjoincount (`/Game/Blueprints/GI_GameInstance.CurrentJoinCount` (`self.GameInstance`)))
  (bind _joinedplayersmap (`/Game/Blueprints/GI_GameInstance.JoinedPlayersMap` (`self.GameInstance`)))
  ;[0 0.15 0.147 0.502] New Join Logic
  (:`Started`
    (if (`BlueprintMapLibrary.Map_Contains` _joinedplayersmap _returnvalue_2)
      (`KismetSystemLibrary.PrintString` "Already joined!")
      (else
        (`BlueprintMapLibrary.Map_Add` _joinedplayersmap _returnvalue_2 (+ _currentjoincount 1))
        (bind _result (`/Engine/EditorBlueprintResources/StandardMacros.IncrementInt` _currentjoincount)
          (:`  `
            (`KismetSystemLibrary.PrintString` (`KismetStringLibrary.Concat_StrStr` "Controller:  " (`KismetStringLibrary.Conv_IntToString` _returnvalue_2) "Joined as player: " (`KismetStringLibrary.Conv_IntToString` _result)))
            (`self.SetupPlayer`)
            (`/Game/Components/Controllers/AC_ControllerRumble.Initialise` (`self.AC_ControllerRumble`) (`self.PlayerPawn`) null self)
            ;;[0.06301 0.6939 0.1441] Join Game Rumble
            (`/Game/Components/Controllers/AC_ControllerRumble.Player Joined FF` (`self.AC_ControllerRumble`))
            (bind _outactors (`GameplayStatics.GetAllActorsOfClass` "/Game/Blueprints/LevelActors/BP_EmptySpawnLocation.BP_EmptySpawnLocation_C"))
            (for _array_element _outactors
              (if (== (`/Game/Blueprints/LevelActors/BP_EmptySpawnLocation.PlayerSlot` _array_element) (`/Game/Blueprints/GI_GameInstance.CurrentJoinCount` (`self.GameInstance`)))
                (`self.K2_SetActorLocation` (`GameplayStatics.GetPlayerPawn` (`GameplayStatics.GetPlayerControllerID` self)) (`self.K2_GetActorLocation` _array_element) false false)
                (`/Game/Blueprints/Player/BP_Player.Init` (`self.PlayerPawn`) self)
                (`EnhancedInputSubsystemInterface.RemoveMappingContext` _returnvalue "/Game/Input/IMC_LobbyControls.IMC_LobbyControls" (struct))
                ;;[1 1 1] Setting controls to normal ingame controls once joined
                (`EnhancedInputSubsystemInterface.AddMappingContext` _returnvalue "/Game/Input/IMC_Controls.IMC_Controls" 0 (struct))
                ;;;[1 1 1 0.5] This triggers the countdown in BP_StartGameArea to reset
                (`/Game/Blueprints/Player/BP_LobbyGameMode.Player Joined` (`self.LobbyGameMode`))))))))))

(event `EnhancedInput|/Game/Input/IA_Pause`
  (params (ActionValue :type Boolean) (ElapsedSeconds :type "Float (double-precision)") (TriggeredSeconds :type "Float (double-precision)") (InputAction :type "InputAction Object Reference" :default "/Game/Input/IA_Pause.IA_Pause"))
  ;[0 0.15 0.147 0.502] New Join Logic
  (:`Triggered`
    ;;[0.162 0.02956 0.3515] Maybe allow other players to pause?
    (`self.Check Player 0`
      (:`Player 0`
        (`/Game/UI/HUD/WBP_HUD.TogglePause` (`self.HUD`))))))

(fn `UserConstructionScript`)