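; Player character Blueprint for a multiplayer action game, handling aiming, melee-style attack montages, health feedback and per-player colours.
; Init sets up health, knockback, dash, interaction and stat components, using controller ID to pick textures and stencil values.
; The chosen weapon becomes a runtime-added component, persisted per player through GameInstance.
; Montage notifies release attack buffering, health changes update UI and face texture, and a room modifier can mark enemy aggro targets.
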(event `PrimaryAttack`
  (bind _currentweapon (`self.CurrentWeapon`))
  (bind _charactermovement (`self.CharacterMovement`))
  (bind _returnvalue (select `/Game/Blueprints/Data/E_AvailableWeaponTypes` (`self.ChosenWeaponType`) :`NewEnumerator0` "/Game/Animation/Player/AM_PlayerSwordLightSwing.AM_PlayerSwordLightSwing" :`NewEnumerator2` "/Game/Animation/Player/AM_PlayerStaffLightSwing.AM_PlayerStaffLightSwing" :!type "AnimMontage Object Reference"))
  ;[0 0.15 0.147 0.502] Light Attack Logic (sends event call to weapon component)
  (`/Engine/EditorBlueprintResources/StandardMacros.IsValid` _currentweapon
    (:`Is Valid`
      (if (and (`/Game/Components/Weapons/AC_WeaponBase.bCanAttack` _currentweapon) (not (`/Game/Components/Pawns/AC_DashAbility.IsDashing?` (`self.AC_DashAbility`))) (not (`self.AttackBuffer`)))
        (set `CharacterMovementComponent.MaxWalkSpeed` (/ (`self.WalkSpeed`) (`self.AttackSpeedDivider`)) _charactermovement)
        (`/Engine/EditorBlueprintResources/StandardMacros.IsValid` _returnvalue
          (:`Is Valid`
            (`|PlayMontage` (`self.Mesh`) _returnvalue
              (:`then`
                (set `self.AttackBuffer` true))
              (:`OnCompleted`
                (set `CharacterMovementComponent.MaxWalkSpeed` (`self.WalkSpeed`) _charactermovement :!label _label))
              (:`OnInterrupted`
                (set `self.AttackBuffer` false)
                (goto _label))
              (:`OnNotifyBegin`
                (set `self.AttackBuffer` false)))))))))

(event `HeavyAttack`
  (bind _currentweapon (`self.CurrentWeapon`))
  (bind _charactermovement (`self.CharacterMovement`))
  (bind _returnvalue (select `/Game/Blueprints/Data/E_AvailableWeaponTypes` (`self.ChosenWeaponType`) :`NewEnumerator0` "/Game/Animation/Player/AM_PlayerSwordHeavySwing.AM_PlayerSwordHeavySwing" :`NewEnumerator2` "/Game/Animation/Player/AM_PlayerStaffHeavySwing.AM_PlayerStaffHeavySwing" :!type "AnimMontage Object Reference"))
  ;[0 0.15 0.147 0.502] Heavy Attack Logic
  (`/Engine/EditorBlueprintResources/StandardMacros.IsValid` _currentweapon
    (:`Is Valid`
      (if (and (`/Game/Components/Weapons/AC_WeaponBase.bCanAttack` _currentweapon) (not (`/Game/Components/Pawns/AC_DashAbility.IsDashing?` (`self.AC_DashAbility`))) (not (`self.AttackBuffer`)))
        (set `CharacterMovementComponent.MaxWalkSpeed` (/ (`self.WalkSpeed`) (`self.AttackSpeedDivider`)) _charactermovement)
        (`/Engine/EditorBlueprintResources/StandardMacros.IsValid` _returnvalue
          (:`Is Valid`
            (`|PlayMontage` (`self.Mesh`) _returnvalue
              (:`then`
                (set `self.AttackBuffer` true))
              (:`OnCompleted`
                (set `CharacterMovementComponent.MaxWalkSpeed` (`self.WalkSpeed`) _charactermovement :!label _label_2))
              (:`OnInterrupted`
                (set `self.AttackBuffer` false)
                (goto _label_2))
              (:`OnNotifyBegin`
                (set `self.AttackBuffer` false)))))))))

(event `EnhancedInput|/Game/Input/IA_Aim_Controller`
  (params (ActionValue :type "Vector2D Structure") (ElapsedSeconds :type "Float (double-precision)") (TriggeredSeconds :type "Float (double-precision)") (InputAction :type "InputAction Object Reference" :default "/Game/Input/IA_Aim_Controller.IA_Aim_Controller"))
  (bind (_returnvalue_roll _returnvalue_pitch _returnvalue_yaw) (`KismetMathLibrary.BreakRotator` (`KismetMathLibrary.RInterpTo` (`self.K2_GetActorRotation`) (`KismetMathLibrary.MakeRotator` 0.0 0.0 (+ (`KismetMathLibrary.DegAtan2` ActionValue_Y ActionValue_X) 90.0)) (`GameplayStatics.GetWorldDeltaSeconds`) (`self.CharacterRotationSpeed`))))
  ;[0 0.15 0.147 0.502] Controller Character Rotation
  (:`Triggered`
    (set `self.bIsControllerAiming` true)
    (set `CharacterMovementComponent.bOrientRotationToMovement` false (`self.CharacterMovement`))
    (if (`self.bIsControllerAiming`)
      (`self.K2_SetActorRotation` (`KismetMathLibrary.MakeRotator` 0.0 0.0 _returnvalue_yaw))))
  (:`Canceled`
    (set `CharacterMovementComponent.bOrientRotationToMovement` true (`self.CharacterMovement`) :!label _label_3))
  (:`Completed`
    (goto _label_3)))

(event `RespawnDone`
  ;[0.162 0.02956 0.3515] Reenables input etc. once the respawn timer is finished
  (`/Game/Components/Player/AC_Respawn.OnRespawnAnimFinished` (`self.AC_Respawn`)))

(event `EnhancedInput|/Game/Input/IA_Aim_Mouse`
  (params (ActionValue :type Boolean) (ElapsedSeconds :type "Float (double-precision)") (TriggeredSeconds :type "Float (double-precision)") (InputAction :type "InputAction Object Reference" :default "/Game/Input/IA_Aim_Mouse.IA_Aim_Mouse"))
  (bind _returnvalue (`GameplayStatics.GetPlayerController` 0))
  (bind (_returnvalue_roll _returnvalue_pitch _returnvalue_yaw) (`KismetMathLibrary.BreakRotator` (`KismetMathLibrary.FindLookAtRotation` (`self.K2_GetActorLocation`) (`.Location` (`GameplayStatics.BreakHitResult` (`PlayerController.GetHitResultUnderCursorByChannel` _returnvalue "TraceTypeQuery1" true))))))
  (bind (_returnvalue_roll_2 _returnvalue_pitch_2 _returnvalue_yaw_2) (`KismetMathLibrary.BreakRotator` (`KismetMathLibrary.RInterpTo` (`self.K2_GetActorRotation`) (`KismetMathLibrary.MakeRotator` _returnvalue_roll 0.0 _returnvalue_yaw) (`GameplayStatics.GetWorldDeltaSeconds`) (`self.CharacterRotationSpeed`))))
  ;[0 0.15 0.147 0.502] Mouse Character Rotation
  (:`Triggered`
    (set `self.bIsMouseAiming` true)
    (set `CharacterMovementComponent.bOrientRotationToMovement` false (`self.CharacterMovement`))
    (if (`self.bIsMouseAiming`)
      (set `PlayerController.bShowMouseCursor` true _returnvalue)
      (`self.K2_SetActorRotation` (`KismetMathLibrary.MakeRotator` _returnvalue_roll_2 0.0 _returnvalue_yaw_2))))
  (:`Canceled`
    (set `self.bIsMouseAiming` false :!label _label_4)
    (set `PlayerController.bShowMouseCursor` true (`GameplayStatics.GetPlayerController` 0))
    (set `CharacterMovementComponent.bOrientRotationToMovement` true (`self.CharacterMovement`)))
  (:`Completed`
    (goto _label_4)))

(event `Init`
  (params (PlayerController :type "/Game/Blueprints/Player/PC_PlayerController Object Reference"))
  (bind _ac_health (`self.AC_Health`))
  (bind _mesh (`self.Mesh`))
  (bind _returnvalue (`GameplayStatics.GetPlayerControllerID` (`self.PlayerController`)))
  ;[0 0.15 0.147 0.502] Begin Play Logic
  (bind _returnvalue_2 (`PrimitiveComponent.CreateDynamicMaterialInstance` (`self.Mesh`) 2 "/Game/Materials/M_PlayerFaceBase.M_PlayerFaceBase" "None"))
  (set `self.FaceMaterial` _returnvalue_2)
  (`SkeletalMeshComponent.SetAllBodiesBelowSimulatePhysics` (`self.Mesh`) "Head" true false)
  (bind _output_get (set `self.PlayerController` PlayerController))
  (set `self.GameInstance` (`/Game/Blueprints/Player/PC_PlayerController.GameInstance` _output_get))
  (if (`.ReturnValue` (`BlueprintMapLibrary.Map_Find` (`/Game/Blueprints/GI_GameInstance.JoinedPlayersMap` (`self.GameInstance`)) _returnvalue))
    ;[0.162 0.02956 0.3515] Colouring Setup
    (bind _returnvalue_3 (`PrimitiveComponent.CreateDynamicMaterialInstance` _mesh 0 "/Game/Materials/M_PlayerSkinBase.M_PlayerSkinBase" "None"))
    (bind _output_get_2 (set `self.SkinMaterial` _returnvalue_3))
    (`MaterialInstanceDynamic.SetTextureParameterValue` _output_get_2 "FaceTexture" (select `int` _returnvalue :`0` "/Game/Textures/T_Player_Skin_BaseColor_Red.T_Player_Skin_BaseColor_Red" :`1` "/Game/Textures/T_Player_Skin_BaseColor_Yellow.T_Player_Skin_BaseColor_Yellow" :`2` "/Game/Textures/T_Player_Skin_BaseColor_Green.T_Player_Skin_BaseColor_Green" :`3` "/Game/Textures/T_Player_Skin_BaseColor_Blue.T_Player_Skin_BaseColor_Blue" :!type "Texture Object Reference"))
    (bind _returnvalue_4 (`PrimitiveComponent.CreateDynamicMaterialInstance` _mesh 1 "/Game/Materials/M_PlayerClothesBase.M_PlayerClothesBase" "None"))
    (bind _output_get_3 (set `self.ClothesMaterial` _returnvalue_4))
    (`MaterialInstanceDynamic.SetTextureParameterValue` _output_get_3 "ClothesTexture" (select `int` _returnvalue :`0` "/Game/Textures/T_Player_Clothes_BaseColor_Red.T_Player_Clothes_BaseColor_Red" :`1` "/Game/Textures/T_Player_Clothes_BaseColor_Yellow.T_Player_Clothes_BaseColor_Yellow" :`2` "/Game/Textures/T_Player_Clothes_BaseColor_Green.T_Player_Clothes_BaseColor_Green" :`3` "/Game/Textures/T_Player_Clothes_BaseColor_Blue.T_Player_Clothes_BaseColor_Blue" :!type "Texture Object Reference"))
    (`PrimitiveComponent.SetCustomDepthStencilValue` (`self.Mesh`) (+ (`GameplayStatics.GetPlayerControllerID` (`self.PlayerController`)) 1))
    (`PrimitiveComponent.SetCustomDepthStencilValue` (`self.WeaponMesh`) (+ (`GameplayStatics.GetPlayerControllerID` (`self.PlayerController`)) 1))
    ;[0.162 0.02956 0.3515] Component Initialisation
    (add `/Game/Components/Player/AC_HealthComponent.OnHealthChange` _ac_health (`|CreateDelegate` :!event `PlayerHealthChange`))
    (`/Game/Components/Player/AC_HealthComponent.HealthCompInit` _ac_health)
    (`/Game/Components/Pawns/AC_KnockbackComponent.Initialise` (`self.AC_KnockbackComponent`) self)
    (`/Game/Components/Pawns/AC_DashAbility.Initialise` (`self.AC_DashAbility`) self)
    (`/Game/Components/Player/AC_Interacting.Initialise` (`self.AC_Interacting`) self)
    (`self.CheckWeapon`)
    (`self.SetCurrentWeapon`)
    (cast `/Game/Blueprints/Player/BP_LobbyGameMode` (`GameplayStatics.GetGameMode`)
      (:`then`
        (`/Game/Components/Player/AC_StatComponent.Initialise` (`self.AC_StatComponent`))
        (`/Game/Components/Player/AC_StatComponent.CreatePlayerBuffData` (`self.AC_StatComponent`))
        ;[1 0 0] TEMPORARY!!! FIXES RESPAWN IN LOBBY UNTIL LOADING SCREEN IS PROPERLY IMPLEMENTED
        (`/Game/Interfaces/BPI_PlayerInterface.PostLoad`)
        (`/Game/Components/Pawns/AC_DamageIndicator.Initiate` (`self.AC_DamageIndicator`) (`self.Mesh`) 1.2)
        ;[0.06301 0.6939 0.1441] Damage Indicator
        (set `self.WalkSpeed` (`CharacterMovementComponent.MaxWalkSpeed` (`self.CharacterMovement`))))
      (:`CastFailed`
        ;[0.06301 0.6939 0.1441] Damage Indicator
        (`/Game/Components/Pawns/AC_DamageIndicator.Initiate` (`self.AC_DamageIndicator`) (`self.Mesh`) 1.2)
        (set `self.WalkSpeed` (`CharacterMovementComponent.MaxWalkSpeed` (`self.CharacterMovement`)))
        (`/Game/Components/Player/AC_StatComponent.Initialise` (`self.AC_StatComponent`))))))

(event `SetCurrentWeapon`
  (bind _returnvalue (`self.K2_GetComponentsByClass` "/Game/Components/Weapons/AC_WeaponBase.AC_WeaponBase_C"))
  (bind _currentweapon (`self.CurrentWeapon`))
  ;[0 0.15 0.147 0.502] Takes Enum to set Weapon Class
  (if (not (`KismetArrayLibrary.Array_IsEmpty` _returnvalue))
    (for _array_element _returnvalue
      (set `self.CurrentWeaponDamage` (`/Game/Components/Weapons/AC_WeaponBase.BaseDamage` _currentweapon))
      (set `self.CurrentWeaponCooldown` (`/Game/Components/Weapons/AC_WeaponBase.AttackCooldown` _currentweapon))
      (`ActorComponent.K2_DestroyComponent` _array_element))
    (set `self.WeaponInitialised` true)
    (else
      (set `self.WeaponInitialised` false)))
  (`|AddComponentByClass` (select `/Game/Blueprints/Data/E_AvailableWeaponTypes` (`self.ChosenWeaponType`) :`NewEnumerator0` "/Game/Components/Weapons/AC_Sword.AC_Sword_C" :`NewEnumerator1` "/Game/Components/Weapons/AC_Bow.AC_Bow_C" :`NewEnumerator2` "/Game/Components/Weapons/AC_MageStaff.AC_MageStaff_C" :`NewEnumerator3` "/Game/Components/Weapons/AC_Hammer.AC_Hammer_C" :`NewEnumerator4` "/Game/Components/Weapons/AC_SuperBow.AC_SuperBow_C" :!type "ActorComponent Class Reference"))
  (`self.GetCurrentWeapon`))

(event `CheckWeapon`
  (bind (_value _returnvalue) (`BlueprintMapLibrary.Map_Find` (`/Game/Blueprints/GI_GameInstance.EquippedWeaponsMap` (`self.GameInstance`)) (`GameplayStatics.GetPlayerControllerID` (`self.PlayerController`))))
  ;[0 0.15 0.147 0.502] Checks Weapon - For persistent weapons
  (if (`BlueprintMapLibrary.Map_Contains` (`/Game/Blueprints/GI_GameInstance.EquippedWeaponsMap` (`self.GameInstance`)) (`GameplayStatics.GetPlayerControllerID` (`self.PlayerController`)))
    (if _returnvalue
      (set `self.ChosenWeaponType` _value))
    (else
      (`BlueprintMapLibrary.Map_Add` (`/Game/Blueprints/GI_GameInstance.EquippedWeaponsMap` (`self.GameInstance`)) (`GameplayStatics.GetPlayerControllerID` (`self.PlayerController`)) (`self.ChosenWeaponType`)))))

(event `/Game/Interfaces/BPI_PlayerInterface.PostLoad`
  ;[0.162 0.02956 0.3515] Important to stop problems with level loading
  (`/Game/Components/Player/AC_Respawn.Initialise` (`self.AC_Respawn`) (`self.PlayerController`) self))

(event `WeaponSelectPersistent`
  (bind _returnvalue (`GameplayStatics.GetPlayerControllerID` (`self.PlayerController`)))
  ;[0 0.15 0.147 0.502] Persistence from Weapon Selector
  (if (`BlueprintMapLibrary.Map_Contains` (`/Game/Blueprints/GI_GameInstance.JoinedPlayersMap` (`self.GameInstance`)) _returnvalue)
    (`BlueprintMapLibrary.Map_Add` (`/Game/Blueprints/GI_GameInstance.EquippedWeaponsMap` (`self.GameInstance`)) _returnvalue (`self.ChosenWeaponType`))))

(event `Remove Current Weapon`
  (bind _returnvalue (`self.GetComponentByClass` "/Game/Components/Weapons/AC_WeaponBase.AC_WeaponBase_C"))
  ;[0 0.15 0.147 0.502] Destroy Weapon
  (`/Engine/EditorBlueprintResources/StandardMacros.IsValid` _returnvalue
    (:`Is Valid`
      (`ActorComponent.K2_DestroyComponent` _returnvalue)
      (`BlueprintMapLibrary.Map_Remove` (`/Game/Blueprints/GI_GameInstance.EquippedWeaponsMap` (`self.GameInstance`)) (`GameplayStatics.GetPlayerControllerID` (`self.PlayerController`))))))

(event `PlayerHealthChange`
  (params (NewHealth :type "Float (double-precision)") (MaxHealth :type "Float (double-precision)"))
  (bind _returnvalue (/ NewHealth MaxHealth))
  (bind _facematerial (`self.FaceMaterial`))
  ;[0.162 0.02956 0.3515] Face Changing per health
  (message `/Game/Interfaces/BPI_PlayerController.UpdateUI` (`GameplayStatics.GetPlayerController` 0) (`GameplayStatics.GetPlayerControllerID` (`self.PlayerController`)) _returnvalue)
  (if (> _returnvalue 0.0)
    (if (> _returnvalue 0.5)
      (`MaterialInstanceDynamic.SetTextureParameterValue` _facematerial "FaceTexture" "/Game/Textures/T_Player_Face_Regular.T_Player_Face_Regular")
      (else
        (`MaterialInstanceDynamic.SetTextureParameterValue` _facematerial "FaceTexture" "/Game/Textures/T_Player_Face_Hurt.T_Player_Face_Hurt")))
    (else
      (`MaterialInstanceDynamic.SetTextureParameterValue` _facematerial "FaceTexture" "/Game/Textures/T_Player_Face_Dead.T_Player_Face_Dead"))))

(event `GetCurrentWeapon`
  (bind _returnvalue (`self.GetComponentByClass` "/Game/Components/Weapons/AC_WeaponBase.AC_WeaponBase_C"))
  (bind _returnvalue_2 (`self.GetComponentByClass` "/Game/Components/Weapons/AC_WeaponBase.AC_WeaponBase_C"))
  ;[0 0.15 0.147 0.502] Gets current weapon from player
  (if (`self.WeaponInitialised`)
    (bind _output_get (set `self.CurrentWeapon` _returnvalue_2))
    (set `/Game/Components/Weapons/AC_WeaponBase.BaseDamage` (`self.CurrentWeaponDamage`) _output_get)
    (set `/Game/Components/Weapons/AC_WeaponBase.AttackCooldown` (`self.CurrentWeaponCooldown`) _output_get)
    (`/Game/Components/Weapons/AC_WeaponBase.Initialisation` _returnvalue_2 self)
    (else
      (set `self.CurrentWeapon` _returnvalue)
      (`/Game/Components/Weapons/AC_WeaponBase.Initialisation` _returnvalue self))))

(event `/Game/Interfaces/BPI_PlayerMovementPass.PlayerWalkTrigger`
  (bind _footarrow (`self.FootArrow`))
  (`NiagaraFunctionLibrary.SpawnSystemAtLocation` "/Game/VFX/NiagaraSystem/NS_FootDust.NS_FootDust" (`SceneComponent.K2_GetComponentLocation` _footarrow) (`SceneComponent.K2_GetComponentRotation` _footarrow)))

(event `SaveWeaponChoiceForModifierRounds`
  ;[0 0.15 0.147 0.502] Saves the weapon choice to set back to after modifier round end (custom weapon removed, re-add weapon)
  (set `self.ModifierSaveWeapon` (`self.ChosenWeaponType`)))

(event `/Game/Interfaces/BPI_PlayerMovementPass.PlayerDashTrigger`
  (bind _footarrow (`self.FootArrow`))
  (`NiagaraFunctionLibrary.SpawnSystemAtLocation` "/Game/VFX/NiagaraSystem/NS_JumpDust.NS_JumpDust" (`SceneComponent.K2_GetComponentLocation` _footarrow) (`SceneComponent.K2_GetComponentRotation` _footarrow)))

(event `Weapon Pick Up`
  ;[1 1 1] Runs all weapon info updates above when a new weapon is selected
  (`self.Remove Current Weapon`)
  (`self.WeaponSelectPersistent`)
  (`self.SetCurrentWeapon`))

(event `EnemyAgroModifier`
  (params (Modifer :type "/Game/Components/Modifiers/AC_EnemyAgroModifier Object Reference") (IsTarget :type Boolean))
  ;[1 0.004025 0.7835] Handles Enemy Agro Modifier Logic
  (set `self.RoomModifier` Modifer)
  (set `self.EnemyAgroActive` true)
  (if IsTarget
    (`self.SetAgroTarget`))
  (`/Game/Components/Player/AC_HealthComponent.EnemyAgro` (`self.AC_Health`) self))

(event `SwapEnemyAgroTarget`
  (params (Player :type "/Game/Blueprints/Player/BP_Player Object Reference"))
  ;[1 0.004025 0.7835] Handles Enemy Agro Modifier Logic
  (`self.SetAgroTarget` Player)
  (`/Game/Components/Modifiers/AC_EnemyAgroModifier.ChangeEnemyTarget` (`self.RoomModifier`) Player)
  (set `self.ModifierTarget` false)
  (`SceneComponent.SetWorldScale3D` (`self.ModiferTargetArrow`) (0.0 0.0 0.0)))

(event `SetAgroTarget`
  ;[1 0.004025 0.7835] Handles Enemy Agro Modifier Logic
  (set `self.ModifierTarget` true)
  (`SceneComponent.SetWorldScale3D` (`self.ModiferTargetArrow`) (1.0 1.0 1.0)))

(fn `ChosenWeaponPass`
  (returns (ChosenWeapons :type "/Game/Blueprints/Data/E_AvailableWeaponTypes Enum"))
  (return (`self.ChosenWeaponType`)))

(fn `IsDead`
  (returns (IsDead :type Boolean))
  (return (<= (`/Game/Components/Player/AC_HealthComponent.CurrentHealth` (`self.AC_Health`)) 0.0)))

(fn `StartAttack`)

(fn `UserConstructionScript`
  (`SceneComponent.K2_AttachToComponent` (`self.WeaponMesh`) (`self.Mesh`) "WeaponSocket" "KeepRelative" "KeepRelative" "KeepWorld" true))