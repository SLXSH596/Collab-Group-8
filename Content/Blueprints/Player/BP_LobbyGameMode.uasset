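; Lobby game mode for local multiplayer that handles player joining and starting the game.
; BeginPlay resets the GameInstance player count, starts looping music, creates the extra local players, hands each controller the GameInstance and spawns a shared BP_Camera.
; PlayerJoined adds unique controllers to the list the camera tracks, then calls CallPlayerJoined.
; StartGame delegates level selection to the GameInstance.
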(event `self.ReceiveBeginPlay`
  ;[0 0.15 0.147 0.502] Begin Play Logic
  (bind _asgi_game_instance (cast `/Game/Blueprints/GI_GameInstance` (`GameplayStatics.GetGameInstance`)))
  (bind _output_get (set `self.GameInstance` _asgi_game_instance))
  (`/Game/Blueprints/GI_GameInstance.Clear Player Count` _output_get)
  (`GameplayStatics.SpawnSound2D` "/Game/Audio/SW_GameMusicLoop.SW_GameMusicLoop" 1.0 1.0 0.0 null)
  (for _index (range 1 4)
    (`GameplayStatics.CreatePlayer` _index))
  (for _index_2 (range (`GameplayStatics.GetNumLocalPlayerControllers`))
    (message `/Game/Interfaces/BPI_PlayerController.Init` (`GameplayStatics.GetPlayerControllerFromID` _index_2) _output_get null))
  ;[0.162 0.02956 0.3515] Spawn camera and don't pass any controller references to start
  (bind _returnvalue (`|SpawnActorFromClass` "/Game/Blueprints/LevelActors/BP_Camera.BP_Camera_C" (`KismetMathLibrary.MakeTransform` (0.0 0.0 0.0)) "Undefined" "MultiplyWithRoot" null null))
  (bind _output_get_2 (set `self.Camera` _returnvalue))
  (`/Game/Blueprints/LevelActors/BP_Camera.UpdateControllers` :`self` _output_get_2))

(event `Start Game`
  ;[0 0.15 0.147 0.502] Basic Start Game
  (`/Game/Blueprints/GI_GameInstance.SelectNewLevel` (`self.GameInstance`)))

(event `/Game/Interfaces/BPI_LobbyGameMode.PlayerJoined`
  (params (JoinedPlayer :type "/Game/Blueprints/Player/PC_PlayerController Object Reference"))
  (bind _joinedcontrollers (`self.JoinedControllers`))
  ;[0.162 0.02956 0.3515] Update the camera with the new controller to track
  (`KismetArrayLibrary.Array_AddUnique` _joinedcontrollers JoinedPlayer)
  (`/Game/Blueprints/LevelActors/BP_Camera.UpdateControllers` (`self.Camera`) _joinedcontrollers)
  (`self.Player Joined`))

(fn `UserConstructionScript`)