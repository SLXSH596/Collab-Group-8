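; Game mode for the menu that resets game state, starts the looping menu music and restores saved audio settings.
; On BeginPlay it calls ClearAll on GI_GameInstance, plays the music as a 2D sound, then loads the SG_Settings save if one exists.
; SetSoundMixValues applies the saved volumes as class overrides on SCM_Main for the master, music, SFX, ambience and voice sound classes, with no fade on load.
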(event `self.ReceiveBeginPlay`
  (bind _settingsslotname (`self.SettingsSlotName`))
  (bind _asgi_game_instance (cast `/Game/Blueprints/GI_GameInstance` (`GameplayStatics.GetGameInstance`)))
  (`/Game/Blueprints/GI_GameInstance.Clear All` _asgi_game_instance)
  (`GameplayStatics.SpawnSound2D` "/Game/Audio/SW_MenuMusicLoop.SW_MenuMusicLoop" 1.0 1.0 0.0 null)
  (bind _returnvalue (`GameplayStatics.DoesSaveGameExist` _settingsslotname))
  (if _returnvalue
    (bind _returnvalue_2 (`GameplayStatics.LoadGameFromSlot` _settingsslotname))
    (bind _assg_settings (cast `/Game/Blueprints/Data/SG_Settings` _returnvalue_2))
    (`self.SetSoundMixValues` _assg_settings)))

(fn `SetSoundMixValues`
  (params (SettingsMenu :type "/Game/Blueprints/Data/SG_Settings Object Reference") (FadeInTime :type "Float (single-precision)"))
  (`GameplayStatics.SetSoundMixClassOverride` "/Game/Audio/SCM_Main.SCM_Main" "/Game/Audio/SC_Master.SC_Master" (`/Game/Blueprints/Data/SG_Settings.MasterVolume` SettingsMenu) 1.0 FadeInTime)
  (`GameplayStatics.SetSoundMixClassOverride` "/Game/Audio/SCM_Main.SCM_Main" "/Game/Audio/SC_Music.SC_Music" (`/Game/Blueprints/Data/SG_Settings.MusicVolume` SettingsMenu) 1.0 FadeInTime)
  (`GameplayStatics.SetSoundMixClassOverride` "/Game/Audio/SCM_Main.SCM_Main" "/Game/Audio/SC_SFX.SC_SFX" (`/Game/Blueprints/Data/SG_Settings.SFXVolume` SettingsMenu) 1.0 FadeInTime)
  (`GameplayStatics.SetSoundMixClassOverride` "/Game/Audio/SCM_Main.SCM_Main" "/Game/Audio/SC_Ambience.SC_Ambience" (`/Game/Blueprints/Data/SG_Settings.AmbienceVolume` SettingsMenu) 1.0 FadeInTime)
  (`GameplayStatics.SetSoundMixClassOverride` "/Game/Audio/SCM_Main.SCM_Main" "/Game/Audio/SC_Voice.SC_Voice" (`/Game/Blueprints/Data/SG_Settings.VoiceVolume` SettingsMenu) 1.0 FadeInTime)
  (return))

(fn `UserConstructionScript`)