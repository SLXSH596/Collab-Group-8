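; BP_PlayerManager tracks how many players are alive and signals game over when none remain.
; On BeginPlay it binds to the death and respawn events of player 0's health and respawn components, then seeds the count from the game instance's player number.
; Decrease and increase events adjust the clamped count with debug prints.
; At zero it cancels respawn and calls the game-over dispatcher.
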(event `Decrease Alive Players`
  (bind _alive_players (`self.Alive Players`))
  ;[0 0.15 0.000607 0.502] Update number of alive players
  (if (not (<= _alive_players 0))
    (bind _output_get (set `self.Alive Players` (`KismetMathLibrary.Clamp` (- _alive_players 1) 0 (`self.Player Num`))))
    (`KismetSystemLibrary.PrintString` (`KismetStringLibrary.Concat_StrStr` "Players Alive: " (`KismetStringLibrary.Conv_IntToString` _output_get)))
    ;[0 0.15 0.000607 0.502] Game Over
    (if (<= (`self.Alive Players`) 0)
      (`/Game/Blueprints/Components/AC_Respawn.Cancel Respawn` (`self.Respawn Component`))
      (`KismetSystemLibrary.PrintString` "GAME OVER" true true (struct :`R` 1.0 :`G` 0.813439 :`A` 1.0))
      (`self.OnGameOver`))))

(event `self.ReceiveBeginPlay`
  ;[0 0.15 0.000607 0.502] Initualise
  (`self.Initualise`)
  (`self.AlivePlayers`))

(event `Initualise`
  (bind _player_ref (`self.Player Ref`))
  ;[0 0.15 0.000607 0.502] Initualise
  (bind _asbp_player (cast `/Game/Blueprints/BP_Player` (`GameplayStatics.GetPlayerCharacter` 0)))
  (set `self.Player Ref` _asbp_player)
  (bind _output_get (set `self.Health Component` (`self.GetComponentByClass` _player_ref "/Game/Blueprints/Components/AC_HealthComponent.AC_HealthComponent_C")))
  (bind _output_get_2 (set `self.Respawn Component` (`self.GetComponentByClass` _player_ref "/Game/Blueprints/Components/AC_Respawn.AC_Respawn_C")))
  (add `/Game/Blueprints/Components/AC_HealthComponent.DeathEvent` _output_get (`|CreateDelegate` :!event `Decrease Alive Players`))
  (add `/Game/Blueprints/Components/AC_Respawn.OnRespawn` _output_get_2 (`|CreateDelegate` :!event `Increase Alive Players`)))

(event `Increase Alive Players`
  ;[0 0.15 0.000607 0.502] Update number of alive players
  (bind _output_get (set `self.Alive Players` (`KismetMathLibrary.Clamp` (+ (`self.Alive Players`) 1) 0 (`self.Player Num`))))
  (`KismetSystemLibrary.PrintString` (`KismetStringLibrary.Concat_StrStr` "Players Alive: " (`KismetStringLibrary.Conv_IntToString` _output_get))))

(fn `AlivePlayers`
  (bind _playernum (`/Game/Blueprints/GI_GameInstance.PlayerNum` (`/Game/Blueprints/BP_Gamemode.Game Instance` (cast `/Game/Blueprints/BP_Gamemode` (`GameplayStatics.GetGameMode`) :!pure true))))
  ;[0 0.15 0.000607 0.502] Number of players alive
  (set `self.Player Num` _playernum)
  (bind _output_get (set `self.Alive Players` _playernum))
  (`KismetSystemLibrary.PrintString` (`KismetStringLibrary.Concat_StrStr` "Players Alive: " (`KismetStringLibrary.Conv_IntToString` _output_get))))

(fn `UserConstructionScript`)