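; Lobby player controller that moves its possessed BP_Player and handles local join input.
; It registers itself with BP_LobbyGameMode on begin play, then applies the lobby input mapping and game-only input mode on possession.
; The join action loops over registered controllers, creating and registering a new local player for each one that is not itself, with debug prints.
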(event `EnhancedInput|/Game/Input/IA_Movement`
  (params (ActionValue :type "Vector2D Structure") (ElapsedSeconds :type "Float (double-precision)") (TriggeredSeconds :type "Float (double-precision)") (InputAction :type "InputAction Object Reference" :default "/Game/Input/IA_Movement.IA_Movement"))
  (:`Triggered`
    (`Pawn.AddMovementInput` (`self.PlayerPawn`) (`KismetMathLibrary.Conv_Vector2DToVector` ActionValue) 100.0 false)))

(event `self.ReceiveBeginPlay`
  (bind _asbp_lobby_game_mode (cast `/Game/Blueprints/BP_LobbyGameMode` (`GameplayStatics.GetGameMode`)))
  (set `self.As BP Lobby Game Mode` _asbp_lobby_game_mode)
  (`KismetArrayLibrary.Array_Add` (`/Game/Blueprints/BP_LobbyGameMode.ConnectedPlayerControllers` (`self.As BP Lobby Game Mode`)) self))

(event `self.ReceivePossess`
  (params (PossessedPawn :type "Pawn Object Reference"))
  (set `self.PlayerPawn` (cast `/Game/Blueprints/BP_Player` PossessedPawn :!pure true))
  (`EnhancedInputSubsystemInterface.AddMappingContext` (subsystem `EnhancedInputLocalPlayerSubsystem`) "/Game/Input/IMC_LobbyControls.IMC_LobbyControls" 0 (struct))
  (`WidgetBlueprintLibrary.SetInputMode_GameOnly` self true))

(event `EnhancedInput|/Game/Input/IA_JoinLobby`
  (params (ActionValue :type Boolean) (ElapsedSeconds :type "Float (double-precision)") (TriggeredSeconds :type "Float (double-precision)") (InputAction :type "InputAction Object Reference" :default "/Game/Input/IA_JoinLobby.IA_JoinLobby"))
  (:`Started`
    (`KismetSystemLibrary.PrintString` "press")
    (for _array_element (`/Game/Blueprints/BP_LobbyGameMode.ConnectedPlayerControllers` (`self.As BP Lobby Game Mode`))
      (if (== _array_element self)
        (`KismetSystemLibrary.PrintString` "already in")
        (else
          (bind _returnvalue (`GameplayStatics.CreatePlayer` -1))
          (`KismetArrayLibrary.Array_Add` (`/Game/Blueprints/BP_LobbyGameMode.ConnectedPlayerControllers` (`self.As BP Lobby Game Mode`)) _returnvalue)
          (`KismetSystemLibrary.PrintString` (`KismetSystemLibrary.GetDisplayName` self)))))))

(fn `UserConstructionScript`)