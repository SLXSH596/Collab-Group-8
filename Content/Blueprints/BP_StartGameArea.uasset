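; Lobby trigger zone that starts the game once every player is standing inside it.
; Box overlaps count BP_Player actors as ready and compare against the connected controller count from BP_LobbyGameMode, shown on a text render.
; A full match starts a countdown timer that calls StartGame on the game mode.
; A mismatch on entry or exit, or a player-joined event from the game mode, cancels the countdown.
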(event `self.ReceiveBeginPlay`
  ;[1 1 1] Binding to event of a player joining on the gamemode
  (bind _asbp_lobby_game_mode (cast `/Game/Blueprints/BP_LobbyGameMode` (`GameplayStatics.GetGameMode`)))
  (bind _output_get (set `self.As BP Lobby Game Mode` _asbp_lobby_game_mode))
  (add `/Game/Blueprints/BP_LobbyGameMode.Player Joined` _asbp_lobby_game_mode (delegate `Update values - player joined`))
  (add `/Game/Blueprints/BP_LobbyGameMode.Player Joined` _output_get (delegate `Update values - player joined`))
  ;[1 1 1] Updates values for a new player joining
  (set `self.Number of players in game` (`KismetArrayLibrary.Array_Length` (`/Game/Blueprints/BP_LobbyGameMode.OrderOfConnectedControllers` (`self.As BP Lobby Game Mode`))) :!label _label)
  (`self.Update Text`)
  ;[1 1 1] Cancels countdown when not everyone is ready
  (`KismetSystemLibrary.K2_ClearAndInvalidateTimerHandle` (`self.Level start timer`) :!label _label_2))

(event `Update values - player joined`
  ;[1 1 1] Updates values for a new player joining
  (goto _label))

(event `Start Countdown`
  ;[1 1 1] When timer ends start first level
  (`/Game/Blueprints/BP_LobbyGameMode.Start game` (`self.As BP Lobby Game Mode`)))

(event `self.Box.OnComponentBeginOverlap`
  (params (OverlappedComponent :type "PrimitiveComponent Object Reference") (OtherActor :type "Actor Object Reference") (OtherComp :type "PrimitiveComponent Object Reference") (OtherBodyIndex :type Integer) (bFromSweep :type Boolean) (SweepResult :type "HitResult Structure (by ref)"))
  ;[1 1 1] Increases player count in the box on entry
  (if (== (`GameplayStatics.GetObjectClass` OtherActor) "/Game/Blueprints/BP_Player.BP_Player_C")
    (`/Engine/EditorBlueprintResources/StandardMacros.IncrementInt` (`self.Number of players ready`)
      (:`  `
        (`self.Update Text`)
        ;[1 1 1] Check if all players are in the zone
        (if (== (`self.Number of players ready`) (`self.Number of players in game`)) :!label _label_3
          ;[1 1 1] Countdown to start level
          (bind _returnvalue (`KismetSystemLibrary.K2_SetTimerDelegate` (delegate `Start Countdown`) (`self.Count Down length to start level`)))
          (set `self.Level start timer` _returnvalue)
          (else
            (goto _label_2)))))))

(event `self.Box.OnComponentEndOverlap`
  (params (OverlappedComponent :type "PrimitiveComponent Object Reference") (OtherActor :type "Actor Object Reference") (OtherComp :type "PrimitiveComponent Object Reference") (OtherBodyIndex :type Integer))
  ;[1 1 1] Decreases player count in the box on exit
  (if (== (`GameplayStatics.GetObjectClass` OtherActor) "/Game/Blueprints/BP_Player.BP_Player_C")
    (`/Engine/EditorBlueprintResources/StandardMacros.DecrementInt` (`self.Number of players ready`)
      (:`  `
        (`self.Update Text`)
        (goto _label_3)))))

(event `Update Text`
  ;[1 1 1] Sets text above box to show players in lobby and ready to start
  (`TextRenderComponent.K2_SetText` (`self.TextRender`) (`KismetTextLibrary.Conv_StringToText` (`KismetStringLibrary.Concat_StrStr` (`KismetStringLibrary.Conv_IntToString` (`self.Number of players ready`)) "/" (`KismetStringLibrary.Conv_IntToString` (`self.Number of players in game`)) "players ready"))))

(fn `UserConstructionScript`)