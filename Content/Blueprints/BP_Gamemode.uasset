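; BP_Gamemode is a game mode that sets up a local multiplayer match on BeginPlay.
; It reads the player count from GI_GameInstance, creates the additional local players and gathers each player's BPC_PlayerController.
; It spawns a single BP_Camera and initialises it with all of those controllers.
; It then initialises its player manager and pickup spawning components, passing itself to the latter.
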(event `self.ReceiveBeginPlay`
  (bind _game_instance (`self.Game Instance`))
  (bind _playercontrollers (`self.PlayerControllers`))
  (set `self.Game Instance` (cast `/Game/Blueprints/GI_GameInstance` (`GameplayStatics.GetGameInstance`) :!pure true))
  (`/Engine/EditorBlueprintResources/StandardMacros.IsValid` _game_instance
    (:`Is Valid`
      (for _ (range (+ (- (`/Game/Blueprints/GI_GameInstance.PlayerNum` _game_instance) 2) 1))
        (`GameplayStatics.CreatePlayer` -1))
      (for _index (range (`/Game/Blueprints/GI_GameInstance.PlayerNum` (`self.Game Instance`)))
        (`KismetArrayLibrary.Array_Add` _playercontrollers (cast `/Game/Blueprints/BPC_PlayerController` (`GameplayStatics.GetPlayerController` _index) :!pure true)))
      (bind _returnvalue (`|SpawnActorFromClass` "/Game/Blueprints/BP_Camera.BP_Camera_C" (`KismetMathLibrary.MakeTransform` (0.0 0.0 0.0)) "Undefined" "MultiplyWithRoot" null null))
      (bind _output_get (set `self.Camera` _returnvalue))
      (`/Game/Blueprints/BP_Camera.Init` _output_get _playercontrollers)
      (`/Game/Blueprints/Components/AC_PlayerManager.Initialise` (`self.AC_PlayerManager`))
      (`/Game/Blueprints/Components/AC_PickupSpawning.Initialise` :`self` (`self.AC_PickupSpawning`) :`GameMode` self))))

(fn `UserConstructionScript`)