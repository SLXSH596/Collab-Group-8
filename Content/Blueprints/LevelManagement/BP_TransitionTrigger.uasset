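; Level transition actor that runs a timed load screen when play begins, in either game or lobby levels.
; BeginPlay casts the game mode to initialise ACTransitionComponent, start the load screen and bind its finish event.
; In game levels, completion calls the LoadFinished dispatcher.
; In the lobby, it clears LobbyLoaded on every player controller, then sets it once loading ends; a boss behaviour-tree start is left unconnected.
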(event `self.ReceiveBeginPlay`
  ;[0.162 0.02956 0.3515] Initialisation - there might be a better way to do this without a cast?
  (bind _asbp_game_mode (cast `/Game/Blueprints/Player/BP_Gamemode` (`GameplayStatics.GetGameMode`))
    (:`then`
      (bind _output_get (set `self.Gamemode` _asbp_game_mode))
      (bind _output_get_2 (set `self.Game Instance` (`/Game/Blueprints/Player/BP_Gamemode.GameInstance` _output_get)))
      (`/Game/Components/Objects/AC_TransitionComponent.Initialise` (`self.AC_TransitionComponent`) _output_get_2 (`self.Gamemode`))
      (`/Game/Components/Objects/AC_TransitionComponent.StartLoadScreen` (`self.AC_TransitionComponent`) 5.0)
      (add `/Game/Components/Objects/AC_TransitionComponent.LoadFinished` (`self.AC_TransitionComponent`) (delegate `LoadComplete`)))
    (:`CastFailed`
      (bind _asbp_lobby_game_mode (cast `/Game/Blueprints/Player/BP_LobbyGameMode` (`GameplayStatics.GetGameMode`)))
      (bind _outactors (`GameplayStatics.GetAllActorsOfClass` "/Game/Blueprints/Player/PC_PlayerController.PC_PlayerController_C"))
      (for _array_element _outactors
        (set `/Game/Blueprints/Player/PC_PlayerController.LobbyLoaded` false _array_element)
        (`KismetArrayLibrary.Array_Add` (`self.Players`) _array_element))
      (`/Game/Components/Objects/AC_TransitionComponent.Initialise` (`self.AC_TransitionComponent`) (`/Game/Blueprints/Player/BP_LobbyGameMode.GameInstance` _asbp_lobby_game_mode) null)
      (`/Game/Components/Objects/AC_TransitionComponent.StartLoadScreen` (`self.AC_TransitionComponent`) 5.0)
      (add `/Game/Components/Objects/AC_TransitionComponent.LoadFinished` (`self.AC_TransitionComponent`) (delegate `InitPlayer`)))))

(event `LoadComplete`
  (`self.Load Finished`))

(event `InitPlayer`
  (for _array_element (`self.Players`)
    (set `/Game/Blueprints/Player/PC_PlayerController.LobbyLoaded` true _array_element)
    (`KismetSystemLibrary.PrintString` "loaded")))

(fn `UserConstructionScript`)