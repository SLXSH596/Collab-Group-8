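; BP_RoomExitArea is a trigger volume that advances the game to a new level once every joined player stands inside it.
; A tick after BeginPlay it caches BP_Gamemode and its GameInstance.
; Each Box overlap counts the BP_Player actors inside and, when that equals CurrentJoinCount, calls SelectNewLevel on the GameInstance.
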(event `self.ReceiveBeginPlay`
  ;[0.162 0.02956 0.3515] Initialisation - there might be a better way to do this without a cast?
  (`KismetSystemLibrary.DelayUntilNextTick`)
  (bind _asbp_gamemode (cast `/Game/Blueprints/Player/BP_Gamemode` (`GameplayStatics.GetGameMode`)))
  (bind _output_get (set `self.Gamemode` _asbp_gamemode))
  (set `self.Game Instance` (`/Game/Blueprints/Player/BP_Gamemode.GameInstance` _output_get)))

(event `self.Box.OnComponentBeginOverlap`
  (params (OverlappedComponent :type "PrimitiveComponent Object Reference") (OtherActor :type "Actor Object Reference") (OtherComp :type "PrimitiveComponent Object Reference") (OtherBodyIndex :type Integer) (bFromSweep :type Boolean) (SweepResult :type "HitResult Structure (by ref)"))
  ;[0.162 0.02956 0.3515] Check if all players are in the area, and open the next level if so.
  (if (== (`KismetArrayLibrary.Array_Length` (`PrimitiveComponent.GetOverlappingActors` OverlappedComponent "/Game/Blueprints/Player/BP_Player.BP_Player_C")) (`/Game/Blueprints/GI_GameInstance.CurrentJoinCount` (`self.Game Instance`)))
    (`/Game/Blueprints/GI_GameInstance.SelectNewLevel` (`self.Game Instance`))))

(fn `UserConstructionScript`)