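; Actor component that holds a movement speed stat boost for the BP_Player character that owns it.
; On BeginPlay it casts its owner to BP_Player and caches the reference.
; IncreaseSpeed sets MaxWalkSpeed to the current movement mode's max speed plus SpeedIncreaseValue, then returns the new value, so repeated calls can stack.
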(event `self.ReceiveBeginPlay`
  (`self.Initialise`))

(fn `IncreaseSpeed`
  (returns (NewSpeed :type "Float (double-precision)"))
  (bind _charactermovement (`Character.CharacterMovement` (`self.Owner`)))
  (bind _output_get (set `CharacterMovementComponent.MaxWalkSpeed` (+ (`MovementComponent.GetMaxSpeed` _charactermovement) (`self.SpeedIncreaseValue`)) _charactermovement))
  (return _output_get))

(fn `Initialise`
  (bind _asbp_player (cast `/Game/Blueprints/BP_Player` (`self.GetOwner`)))
  (set `self.Owner` _asbp_player))