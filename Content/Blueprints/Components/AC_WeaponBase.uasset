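; Base weapon component for BP_Player that handles twin-stick-style aiming and defines attack entry points.
; Controller aim derives yaw from stick direction, while mouse aim looks at the cursor's hit point.
; Both interpolate the player's rotation and suspend orient-to-movement until aim input ends.
; Primary attack input calls StartAttack, which is an empty stub like StopAttack, intended for ending auto or charge attacks.
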(event `self.ReceiveBeginPlay`
  (bind _asbp_player (cast `/Game/Blueprints/BP_Player` (`self.GetOwner`)))
  (set `self.PlayerRef` _asbp_player))

(event `EnhancedInput|/Game/Input/IA_Aim_Controller`
  (params (ActionValue :type "Vector2D Structure") (ElapsedSeconds :type "Float (double-precision)") (TriggeredSeconds :type "Float (double-precision)") (InputAction :type "InputAction Object Reference" :default "/Game/Input/IA_Aim_Controller.IA_Aim_Controller"))
  (bind _playerref (`self.PlayerRef`))
  (bind (_returnvalue_roll _returnvalue_pitch _returnvalue_yaw) (`KismetMathLibrary.BreakRotator` (`KismetMathLibrary.RInterpTo` (`Actor.K2_GetActorRotation` _playerref) (`KismetMathLibrary.MakeRotator` 0.0 0.0 (+ (`KismetMathLibrary.DegAtan2` ActionValue_Y ActionValue_X) 90.0)) (`GameplayStatics.GetWorldDeltaSeconds`) (`self.CharacterRotationSpeed`))))
  (:`Triggered`
    (set `self.bIsControllerAiming` true)
    (set `CharacterMovementComponent.bOrientRotationToMovement` false (`Character.CharacterMovement` (`self.PlayerRef`)))
    (if (`self.bIsControllerAiming`)
      (`Actor.K2_SetActorRotation` _playerref (`KismetMathLibrary.MakeRotator` 0.0 0.0 _returnvalue_yaw) false)))
  (:`Canceled`
    (set `CharacterMovementComponent.bOrientRotationToMovement` true (`Character.CharacterMovement` (`self.PlayerRef`)) :!label _label))
  (:`Completed`
    (goto _label)))

(event `EnhancedInput|/Game/Input/IA_Aim_Mouse`
  (params (ActionValue :type Boolean) (ElapsedSeconds :type "Float (double-precision)") (TriggeredSeconds :type "Float (double-precision)") (InputAction :type "InputAction Object Reference" :default "/Game/Input/IA_Aim_Mouse.IA_Aim_Mouse"))
  (bind _returnvalue (`GameplayStatics.GetPlayerController` 0))
  (bind _playerref (`self.PlayerRef`))
  (bind (_returnvalue_roll _returnvalue_pitch _returnvalue_yaw) (`KismetMathLibrary.BreakRotator` (`KismetMathLibrary.FindLookAtRotation` (`Actor.K2_GetActorLocation` _playerref) (`.Location` (`GameplayStatics.BreakHitResult` (`PlayerController.GetHitResultUnderCursorByChannel` _returnvalue "TraceTypeQuery1" true))))))
  (bind (_returnvalue_roll_2 _returnvalue_pitch_2 _returnvalue_yaw_2) (`KismetMathLibrary.BreakRotator` (`KismetMathLibrary.RInterpTo` (`Actor.K2_GetActorRotation` _playerref) (`KismetMathLibrary.MakeRotator` _returnvalue_roll 0.0 _returnvalue_yaw) (`GameplayStatics.GetWorldDeltaSeconds`) (`self.CharacterRotationSpeed`))))
  (:`Triggered`
    (set `self.bIsMouseAiming` true)
    (set `CharacterMovementComponent.bOrientRotationToMovement` false (`Character.CharacterMovement` (`self.PlayerRef`)))
    (if (`self.bIsMouseAiming`)
      (set `PlayerController.bShowMouseCursor` true _returnvalue)
      (`Actor.K2_SetActorRotation` _playerref (`KismetMathLibrary.MakeRotator` _returnvalue_roll_2 0.0 _returnvalue_yaw_2) false)))
  (:`Canceled`
    (set `self.bIsMouseAiming` false :!label _label_2)
    (set `PlayerController.bShowMouseCursor` true (`GameplayStatics.GetPlayerController` 0))
    (set `CharacterMovementComponent.bOrientRotationToMovement` true (`Character.CharacterMovement` (`self.PlayerRef`))))
  (:`Completed`
    (goto _label_2)))

(event `StartAttack`)

(event `StopAttack`
  ; For stopping auto attacks OR charge attacks
)

(event `EnhancedInput|/Game/Input/IA_PrimaryAttack`
  (params (ActionValue :type Boolean) (ElapsedSeconds :type "Float (double-precision)") (TriggeredSeconds :type "Float (double-precision)") (InputAction :type "InputAction Object Reference" :default "/Game/Input/IA_PrimaryAttack.IA_PrimaryAttack"))
  ;[0.15 0 0 0.5] To be added to player
  (:`Triggered`
    (`self.StartAttack`)))