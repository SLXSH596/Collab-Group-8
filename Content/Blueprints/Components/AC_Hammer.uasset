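; Hammer attack component that deals melee area damage in front of its owning actor.
; StartAttack, gated by CanAttack, runs a multi-sphere trace along the owner's forward vector, with debug drawing left on.
; Each hit takes hammer-type damage, scaled by FriendlyFireMultiplier when FriendlyFireCheck flags friendly fire.
; A timer calls MeleeCooldown to re-enable attacking after AttackCooldown, whether or not anything was hit.
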(event `self.StartAttack`
  (bind _returnvalue (`self.GetOwner`))
  (bind _returnvalue_2 (`self.GetOwner`))
  ;[0 0.15 0.147 0.502] Spear Attack Logic
  (if (`self.bCanAttack`)
    (set `self.bCanAttack` false)
    (bind (_outhits _returnvalue_3) (`KismetSystemLibrary.SphereTraceMultiForObjects` (+ (* (`Actor.GetActorForwardVector` _returnvalue_2) (/ (`self.AttackRange`) 1.5)) (`Actor.K2_GetActorLocation` _returnvalue_2)) (+ (* (`Actor.GetActorForwardVector` _returnvalue_2) (`self.AttackRange`)) (`Actor.K2_GetActorLocation` _returnvalue_2)) 100.0 (`self.DefaultObjectType`) false (`|MakeArray` _returnvalue_2) "ForDuration"))
    (if _returnvalue_3
      (for _array_element _outhits
        ;;[0 0.15 0.147 0.502] Ensures no friendly fire (false to cause friendly fire)
        (bind (_hitactor _bwasfriendlyfire) (`self.FriendlyFireCheck` _array_element))
        (if (not _bwasfriendlyfire)
          (`GameplayStatics.ApplyDamage` _hitactor (`self.BaseDamage`) null _returnvalue "/Game/Blueprints/WeaponDamageTypes/BP_DamageType_Hammer.BP_DamageType_Hammer_C")
          (else
            (`GameplayStatics.ApplyDamage` _hitactor (* (`self.BaseDamage`) (`self.FriendlyFireMultiplier`)) null _returnvalue "/Game/Blueprints/WeaponDamageTypes/BP_DamageType_Hammer.BP_DamageType_Hammer_C")))))
    (`KismetSystemLibrary.K2_SetTimerDelegate` (delegate `MeleeCooldown`) (`self.AttackCooldown`))))

(event `MeleeCooldown`
  ;[0 0.15 0.147 0.502] Spear Attack Logic
  (set `self.bCanAttack` true))