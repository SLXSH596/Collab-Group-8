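; Actor component that gives its owner a spear melee attack with a cooldown.
; StartAttack sweeps a multi-sphere object trace between a point at attack range along the owner's forward vector and the owner's location, ignoring the owner.
; Hits passing a friendly-fire check take spear-type damage with the owner as causer.
; A timer then fires MeleeCooldown to re-enable attacking.
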(event `self.StartAttack`
  (bind _returnvalue (`self.GetOwner`))
  (bind _returnvalue_2 (`Actor.K2_GetActorLocation` _returnvalue))
  ;[0 0.15 0.147 0.502] Spear Attack Logic
  (if (`self.bCanAttack`)
    (set `self.bCanAttack` false)
    (bind (_outhits _returnvalue_3) (`KismetSystemLibrary.SphereTraceMultiForObjects` (+ (* (`Actor.GetActorForwardVector` _returnvalue) (`self.AttackRange`)) _returnvalue_2) _returnvalue_2 30.0 (`self.DefaultObjectType`) false (`|MakeArray` _returnvalue) "ForDuration"))
    (if _returnvalue_3
      (for _array_element _outhits
        ;;[0 0.15 0.147 0.502] Ensures no friendly fire (false to cause friendly fire)
        (bind (_hitactor _bwasfriendlyfire) (`self.FriendlyFireCheck` _array_element))
        (if (not _bwasfriendlyfire)
          (`GameplayStatics.ApplyDamage` _hitactor (`self.BaseDamage`) null (`self.GetOwner`) "/Game/Blueprints/WeaponDamageTypes/BP_DamageType_Spear.BP_DamageType_Spear_C"))))
    (`KismetSystemLibrary.K2_SetTimerDelegate` (delegate `MeleeCooldown`) (`self.AttackCooldown`))))

(event `MeleeCooldown`
  ;[0 0.15 0.147 0.502] Spear Attack Logic
  (set `self.bCanAttack` true))