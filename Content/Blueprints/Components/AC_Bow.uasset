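; Bow attack component that fires BP_Arrow projectiles from the player, limited by a cooldown.
; StartAttack checks and clears CanAttack, then spawns an arrow just ahead of the player along its forward vector, using the player's rotation.
; A timer then calls RangedCooldown after AttackCooldown to re-enable attacking.
; The spawn point is a placeholder until it uses the bow's location.
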(event `self.StartAttack`
  (bind _playerref (`self.PlayerRef`))
  (if (`self.bCanAttack`)
    (set `self.bCanAttack` false)
    (`|SpawnActorFromClass` "/Game/Blueprints/WeaponProjectiles/BP_Arrow.BP_Arrow_C" (`KismetMathLibrary.MakeTransform` (+ (* (`Actor.GetActorForwardVector` _playerref) 80.0) (`Actor.K2_GetActorLocation` _playerref)) (`Actor.K2_GetActorRotation` _playerref)) "Undefined" "MultiplyWithRoot" null null)
    (`KismetSystemLibrary.K2_SetTimerDelegate` (delegate `RangedCooldown`) (`self.AttackCooldown`))))

(event `RangedCooldown`
  (set `self.bCanAttack` true))