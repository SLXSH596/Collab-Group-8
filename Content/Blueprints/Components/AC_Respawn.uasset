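; Actor component for BP_Player that handles death and timed respawn at the level's PlayerStart location.
; On BeginPlay it caches the player, controller and health component, stores the spawn point and binds to the death event.
; Death disables input and movement and starts a cancellable respawn timer.
; Respawn restores control, moves the player back, heals by applying negative max-health damage and fires an OnRespawn dispatcher.
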(event `Set Spawn Point`
  ;[0.06301 0.6939 0.1441] Set spawn point
  (bind _returnvalue (`GameplayStatics.GetActorOfClass` "/Script/Engine.PlayerStart"))
  (set `self.Respawn Location` (`Actor.K2_GetActorLocation` _returnvalue)))

(event `Cancel Respawn`
  ;[0.06301 0.6939 0.1441] Stop respawn timer
  (`KismetSystemLibrary.K2_ClearAndInvalidateTimerHandle` (`self.Respawn Handle`)))

(event `On Death`
  (bind _player_ref (`self.Player Ref`))
  ;[0.06301 0.6939 0.1441] Player Death
  (`Actor.DisableInput` _player_ref (`self.Player Controller`))
  (`CharacterMovementComponent.SetMovementMode` (`Character.CharacterMovement` _player_ref) "MOVE_None" 0)
  (bind _returnvalue (`KismetSystemLibrary.K2_SetTimerDelegate` (`|CreateDelegate` :!event `On Respawn `) (`self.Respawn Time`)))
  (set `self.Respawn Handle` _returnvalue))

(event `self.ReceiveBeginPlay`
  ;[0.06301 0.6939 0.1441] Initualise
  ;;[0.06301 0.6939 0.1441] (Consider moving to BP_Player)
  (`self.Initialise`)
  (`self.Set Spawn point`)
  (add `/Game/Blueprints/Components/AC_HealthComponent.DeathEvent` (`self.Health Component`) (`|CreateDelegate` :!event `On Death`)))

(event `On Respawn`
  (bind _player_ref (`self.Player Ref`))
  ;[0.06301 0.6939 0.1441] Player Respawn
  (`Actor.EnableInput` _player_ref (`self.Player Controller`))
  (`CharacterMovementComponent.SetMovementMode` (`Character.CharacterMovement` _player_ref) "MOVE_Walking" 0)
  (`Actor.K2_SetActorLocation` (`self.Player Ref`) (`self.Respawn Location`) false false)
  (`GameplayStatics.ApplyDamage` (`self.Player Ref`) (/ (`/Game/Blueprints/Components/AC_HealthComponent.MaxHealth` (`self.Health Component`)) -1.0))
  (`self.OnRespawn`))

(fn `Initialise`
  (bind _returnvalue (`self.GetOwner`))
  (set `self.Player Ref` (cast `/Game/Blueprints/BP_Player` _returnvalue :!pure true))
  (set `self.Health Component` (`Actor.GetComponentByClass` _returnvalue "/Game/Blueprints/Components/AC_HealthComponent.AC_HealthComponent_C"))
  (set `self.Player Controller` (`GameplayStatics.GetPlayerController` 0)))