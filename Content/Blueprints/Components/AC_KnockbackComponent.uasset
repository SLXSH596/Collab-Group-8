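; Actor component that applies knockback to characters in the game.
; ApplyKnockback launches a target Character along the normalized direction away from the instigator, scaled by Strength, adding to its current velocity rather than overriding it.
; Initialise casts the component's owner to BP_Player and stores it as Owner, though the knockback function does not use that reference.
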(fn `ApplyKnockback`
  (params (TargetActor :type "Actor Object Reference") (InstigatorActor :type "Actor Object Reference") (Strength :type "Float (double-precision)"))
  (bind _ascharacter (cast `Character` TargetActor))
  (`Character.LaunchCharacter` _ascharacter (* (`KismetMathLibrary.Normal` (- (`Actor.K2_GetActorLocation` TargetActor) (`Actor.K2_GetActorLocation` InstigatorActor))) Strength) false false))

(fn `Initialise`
  (bind _asbp_player (cast `/Game/Blueprints/BP_Player` (`self.GetOwner`)))
  (set `self.Owner` _asbp_player))