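; Actor component that tracks whether its owning pickup can currently be interacted with.
; On BeginPlay it casts the owner to BP_BasePickup and caches it, while enable and disable functions set the CanInteract flag and print it.
; The IA_Interact input event is empty, and the CanInteract-gated PickupItem call is disconnected, so the component never triggers a pickup itself.
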(event `self.ReceiveBeginPlay`
  (`self.Initialise`))

(event `EnhancedInput|/Game/Input/IA_Interact`
  (params (ActionValue :type Boolean) (ElapsedSeconds :type "Float (double-precision)") (TriggeredSeconds :type "Float (double-precision)") (InputAction :type "InputAction Object Reference" :default "/Game/Input/IA_Interact.IA_Interact")))

(fn `Disable Interact`
  (bind _output_get (set `self.Can Interact?` false))
  (`KismetSystemLibrary.PrintString` (`KismetStringLibrary.Conv_BoolToString` _output_get)))

(fn `Enable Interact`
  (bind _output_get (set `self.Can Interact?` true))
  (`KismetSystemLibrary.PrintString` (`KismetStringLibrary.Conv_BoolToString` _output_get)))

(fn `Initialise`
  (bind _asbp_base_pickup (cast `/Game/Blueprints/Pickup/BP_BasePickup` (`self.GetOwner`)))
  (set `self.Pickup` _asbp_base_pickup))