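; Room manager component that opens room exits in sequence and triggers pickup spawning as rooms are completed.
; On BeginPlay it gathers all rooms, spawns an actor at each room's arrow, then caches the exit actors.
; A looping timer fires OnRoomCompleted, standing in for real completion logic.
; Completion handling opens the next exit, then points the GameMode's AC_PickupSpawning at the room with the advanced index.
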(event Custom|Room%20Completed
  (CallFunction|OpenDoor)
  (CallFunction|CallPickupEvent))

(event Custom|Open%20Door
  (if (>= (Variables|Index|GetNext%20Open%20Exit) (Variables|Index|GetExit%20Index))
    (Development|PrintString "NO MORE DOORS TO OPEN" true true "(R=1.000000,G=0.010666,B=0.000251,A=1.000000)" 2.0 "1")
    (else
      (Utilities|IsValid (Utilities|Array|Get(acopy) (Variables|References|GetRoomExits) (Variables|Index|GetNext%20Open%20Exit))
        (:Is%20Valid
          (Default|OpenExit (Utilities|Array|Get(acopy) (Variables|References|GetRoomExits) (Variables|Index|GetNext%20Open%20Exit)))
          (bind _result (Math|Integer|IncrementInt (Variables|Index|GetNext%20Open%20Exit))
            (:%20%20
              (Variables|Index|SetNext%20Open%20Exit (Math|Integer|Clamp(Integer) _result 0 (Variables|Index|GetExit%20Index))))))))))

(event Custom|Reset%20Spawn%20Pickups
  (bind _roomexits (Variables|References|GetRoomExits))
  (bind _output (Utilities|Array|Get(acopy) _roomexits 2))
  ;[0.06301 0.6939 0.1441] Old (Delete Later)
  (Utilities|FlowControl|DoOnce false) ; enters at Reset
)

(event Custom|CustomEvent
  (Default|CallOnRoomCompleted))

(event Custom|Call%20Pickup%20Event
  (bind _gamemode (Variables|References|GetGamemode))
  (bind _next_open_exit (Variables|Index|GetNext%20Open%20Exit))
  (bind _room_parent (Variables|References|GetRoom%20Parent))
  (bind _returnvalue (Actor|GetComponentbyClass _gamemode "/Game/Blueprints/Components/AC_PickupSpawning.AC_PickupSpawning_C"))
  (bind _output (Utilities|Array|Get(acopy) _room_parent _next_open_exit))
  (Utilities|IsValid _returnvalue
    (:Is%20Valid
      (Utilities|IsValid _output
        (:Is%20Valid
          (Variables|/Game/Blueprints/Components/AC_PickupSpawning.AC_PickupSpawning_C|SetSpawnLocation _returnvalue (+ (Transformation|GetActorLocation _output) "0.000000,0.000000,150.000000"))
          (Default|SpawnPickups _returnvalue))
        (:Is%20Not%20Valid
          (Development|PrintString "NO MORE PICKUPS" true true "(R=1.000000,G=0.010666,B=0.000251,A=1.000000)" 2.0 "2"))))))

(event EventBeginPlay
  (Utilities|FlowControl|Sequence
    (:then_0
      (Utilities|Time|SetTimerbyEvent (delegate Custom|CustomEvent) 6.0 true))
    (:then_1
      (CallFunction|Initialise)
      (EventDispatchers|BindEventtoOnRoomCompleted (EventDispatchers|CreateEvent :!event Custom|Room%20Completed)))))

(fn Initialise
  (bind _asbp_gamemode (Utilities|Casting|CastToBP_Gamemode (Game|GetGameMode)))
  (Variables|References|SetGamemode _asbp_gamemode)
  (bind _outactors (Actor|GetAllActorsOfClass "/Game/Blueprints/PCGMapGen/BP_RoomPARENT.BP_RoomPARENT_C"))
  (bind _output_get (Variables|References|SetRoom%20Parent _outactors))
  (Variables|Index|SetRoom%20Index (Utilities|Array|Length _output_get))
  (for _array_element _output_get
    (Utilities|IsValid _array_element
      (:Is%20Valid
        (Game|SpawnActorfromClass "/Game/Blueprints/PCGMapGen/BP_RoomExit.BP_RoomExit_C" (Math|Transform|MakeTransform (+ (Transformation|GetWorldLocation (Variables|/Game/Blueprints/PCGMapGen/BP_RoomPARENT.BP_RoomPARENT_C|GetArrow _array_element)) "0.000000,0.000000,75.000000") (Transformation|GetWorldRotation (Variables|/Game/Blueprints/PCGMapGen/BP_RoomPARENT.BP_RoomPARENT_C|GetArrow _array_element)) "1.000000,1.000000,1.000000") "Undefined" "MultiplyWithRoot" 0 0))))
  (bind _outactors_2 (Actor|GetAllActorsOfClass "/Game/Blueprints/PCGMapGen/BP_RoomExit.BP_RoomExit_C"))
  (bind _output_get_2 (Variables|References|SetRoomExits _outactors_2))
  (Variables|Index|SetExit%20Index (Utilities|Array|Length _output_get_2)))