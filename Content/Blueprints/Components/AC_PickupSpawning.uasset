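; Actor component that spawns speed pickups at random points around a spawn location when play begins.
; On BeginPlay it caches the game mode, gathers all BP_Player actors, then loops over the player count to spawn BP_SpeedPickup actors.
; Each point offsets X and Y independently within the radius, giving a square area at a fixed height, and each spawn is printed for debugging.
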(event `self.ReceiveBeginPlay`
  (`self.Initialise` (`GameplayStatics.GetGameMode`))
  (`self.Get_PlayerCount`)
  (`self.Spawn_Pickups`))

(fn `Get_PlayerCount`
  (bind _outactors (`GameplayStatics.GetAllActorsOfClass` "/Game/Blueprints/BP_Player.BP_Player_C"))
  (set `self.Players` _outactors))

(fn `GetRandomPointInRadius`
  (params (Origin :type "Vector Structure") (Radius :type "Float (double-precision)"))
  (returns (`Random Point` :type "Vector Structure"))
  (bind _returnvalue (* Radius -1.0))
  (return (`KismetMathLibrary.MakeVector` (+ (.x Origin) (`KismetMathLibrary.RandomFloatInRange` _returnvalue Radius)) (+ (.y Origin) (`KismetMathLibrary.RandomFloatInRange` _returnvalue Radius)) 150.0)))

(fn `Initialise`
  (params (`Game Mode` :type "GameModeBase Object Reference"))
  (bind _asgame_mode (cast `GameMode` `Game Mode`))
  (set `self.GameMode` _asgame_mode))

(fn `Spawn_Pickups`
  (for _index (range (+ (`KismetArrayLibrary.Array_Length` (`self.Players`)) 1))
    (bind _random_point (`self.GetRandomPointInRadius` (`self.SpawnLocation`) (`self.SpawnRadius`)))
    (`|SpawnActorFromClass` "/Game/Blueprints/Pickup/BP_SpeedPickup.BP_SpeedPickup_C" (`KismetMathLibrary.MakeTransform` _random_point) "Undefined" "MultiplyWithRoot" null null)
    (`KismetSystemLibrary.PrintString` (`KismetStringLibrary.Concat_StrStr` "Pickup: " (`KismetStringLibrary.Conv_IntToString` _index) " , spawned at: " (`KismetStringLibrary.Conv_VectorToString` _random_point)))))