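; Actor component that runs sequential enemy waves around its owner, with room completion still a debug print placeholder.
; StartWave expands wave data into a spawn queue, spawned on a looping timer or all at once.
; Enemies spawn at random points in a square around the owner at fixed height.
; Death events prune the alive list, advancing waves once it and the queue are exhausted.
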(event `SpawnNextEnemy`
  (bind _spawn_queue (`self.Spawn Queue`))
  (bind _current_spawn_index (`self.Current Spawn Index`))
  ;[0.4793 0.05127 0.0648] Spawn Enemy Wave (with spawn rate)
  (if (>= _current_spawn_index (`KismetArrayLibrary.Array_Length` _spawn_queue))
    ;;[0.4793 0.05127 0.0648] Stop Timer once Spawn Queue has been spawned
    (`KismetSystemLibrary.K2_ClearAndInvalidateTimerHandle` (`self.SpawnTimerHandle`))
    (else
      ;;[0.4793 0.05127 0.0648] Generate Random Spawn Point
      (bind _random_point (`self.GetRandomPointInRadius` (`Actor.K2_GetActorLocation` (`self.GetOwner`)) (`self.SpawnRadius`)))
      ;;[0.4793 0.05127 0.0648] Spawn next Enemy from the Spawn Queue, assign an OnEnemyDeath and add to list of Alive Enemies
      (bind _returnvalue (`|SpawnActorFromClass` (`|GetArrayItem` _spawn_queue _current_spawn_index) (`KismetMathLibrary.MakeTransform` _random_point) "AdjustIfPossibleButAlwaysSpawn" "MultiplyWithRoot" null null))
      (bind _output_get (set `self.SpawnedEnemy` _returnvalue))
      (add `/Game/AI/AIActors/BP_BasicEnemy.OnEnemyDeath` _output_get (`|CreateDelegate` :!event `EnemyDied`))
      (`KismetArrayLibrary.Array_Add` (`self.Alive Enemies`) _output_get)
      (`/Engine/EditorBlueprintResources/StandardMacros.IncrementInt` (`self.Current Spawn Index`)))))

(event `EnemyDied`
  (params (Enemy :type "/Game/AI/AIActors/BP_BasicEnemy Object Reference"))
  ;[0.4793 0.05127 0.0648] Remove Dead Enemy from the Array of Alive Enemies -> Then check if theres any still alive before progressing to the next Wave.
  (`KismetArrayLibrary.Array_RemoveItem` (`self.Alive Enemies`) Enemy)
  (`self.CheckWaveCompletion`))

(event `OnWaveCompleted`
  (bind _currentwaveindex (`self.CurrentWaveIndex`))
  ;[0.4793 0.05127 0.0648] A Wave has been Completed -> Check if there is another and start that wave if so
  ;;[0.4793 0.05127 0.0648] No wave in progress
  (set `self.IsWaveInProgress?` false)
  ;;[0.4793 0.05127 0.0648] Increment Wave Count
  (`/Engine/EditorBlueprintResources/StandardMacros.IncrementInt` _currentwaveindex
    (:`  `
      (if (< _currentwaveindex (`KismetArrayLibrary.Array_Length` (`self.Waves`)))
        ;;[0.4793 0.05127 0.0648] Start the Next Wave
        (`self.StartWave`)
        (else
          ;;[0.4793 0.05127 0.0648] LOGIC FOR ROOM COMPLETION HERE
          (`KismetSystemLibrary.PrintString` "ALL WAVES COMPLETE"))))))

(fn `CheckWaveCompletion`
  (if (and (== (`KismetArrayLibrary.Array_Length` (`self.Alive Enemies`)) 0) (>= (`self.Current Spawn Index`) (`KismetArrayLibrary.Array_Length` (`self.Spawn Queue`))))
    ;[0.4793 0.05127 0.0648] Wave has been completed
    (`self.OnWaveCompleted`)))

(fn `ClearSpawnData`
  ;[0.4793 0.05127 0.0648] Resets all Spawn Info
  (`KismetArrayLibrary.Array_Clear` (`self.Spawn Queue`))
  (`KismetArrayLibrary.Array_Clear` (`self.Alive Enemies`))
  (set `self.Current Spawn Index` 0))

(fn `GetRandomPointInRadius`
  (params (Origin :type "Vector Structure") (Radius :type "Float (double-precision)"))
  (returns (`Random Point` :type "Vector Structure"))
  (bind _returnvalue (* Radius -1.0))
  (return (`KismetMathLibrary.MakeVector` (+ (.x Origin) (`KismetMathLibrary.RandomFloatInRange` _returnvalue Radius)) (+ (.y Origin) (`KismetMathLibrary.RandomFloatInRange` _returnvalue Radius)) 150.0)))

(fn `Initialise`)

(fn `SpawnAllEnemies`
  ;[0.4793 0.05127 0.0648] Spawns all Enemies in a Wave - Better for debugging
  ;;[0.4793 0.05127 0.0648] Clear List of Alive Enemies
  (`KismetArrayLibrary.Array_Clear` (`self.Alive Enemies`))
  ;;[0.4793 0.05127 0.0648] Loop through the Spawn Queue
  (for _index (range (`KismetArrayLibrary.Array_Length` (`self.Spawn Queue`)))
    ;;[0.4793 0.05127 0.0648] Get EnemyManager's Location and generate a random spawn point with it
    (bind _random_point (`self.GetRandomPointInRadius` (`Actor.K2_GetActorLocation` (`self.GetOwner`)) (`self.SpawnRadius`)))
    ;;[0.4793 0.05127 0.0648] Spawn next Enemy from the Spawn Queue, assign an OnEnemyDeath and add to list of Alive Enemies
    (bind _returnvalue (`|SpawnActorFromClass` (`|GetArrayItem` (`self.Spawn Queue`) _index) (`KismetMathLibrary.MakeTransform` _random_point) "AdjustIfPossibleButAlwaysSpawn" "MultiplyWithRoot" null null))
    (add `/Game/AI/AIActors/BP_BasicEnemy.OnEnemyDeath` _returnvalue (`|CreateDelegate` :!event `EnemyDied`))
    (`KismetArrayLibrary.Array_Add` (`self.Alive Enemies`) _returnvalue))
  ;;[0.4793 0.05127 0.0648] Current amount of Enemies that are Spawned
  (set `self.Current Spawn Index` (`KismetArrayLibrary.Array_Length` (`self.Alive Enemies`))))

(fn `StartWave`
  ;[0.4793 0.05127 0.0648] Only Start new Wave if one isn't in progress
  (if (not (`self.IsWaveInProgress?`))
    (set `self.IsWaveInProgress?` true)
    ;[0.4793 0.05127 0.0648] Reset Spawn Data
    (`self.ClearSpawnData`)
    ;[0.4793 0.05127 0.0648] Gets Info of incoming Wave
    (bind _output_get (set `self.Current Wave` (`|GetArrayItem` (`self.Waves`) (`self.CurrentWaveIndex`))))
    (bind (_enemyspawninfo _wavename _spawnrate _spawnallatonce_) (break `/Game/Blueprints/Data/EnemySpawning/F_EnemyWaveData` _output_get))
    ;[0.4793 0.05127 0.0648] Build Spawn Queue (a list of all the enemies to spawn based on Wave Data)
    (for _array_element _enemyspawninfo
      (bind (_enemyclass _enemycount) (break `/Game/Blueprints/Data/EnemySpawning/F_EnemySpawnInfo` _array_element))
      (for _ (range _enemycount)
        (`KismetArrayLibrary.Array_Add` (`self.Spawn Queue`) _enemyclass)))
    ;[0.4793 0.05127 0.0648] Once Spawn Queue is built, should enemies spawn spawn all at once or on a timer?
    (if _spawnallatonce_
      ;[0.4793 0.05127 0.0648] Debug Purposes
      (`self.SpawnAllEnemies`)
      (else
        ;[0.4793 0.05127 0.0648] Start Spawning Enemies based on Spawn Rate
        (bind _returnvalue (`KismetSystemLibrary.K2_SetTimerDelegate` (`|CreateDelegate` :!event `SpawnNextEnemy`) _spawnrate true))
        (set `self.SpawnTimerHandle` _returnvalue)))))