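; Actor component that gives BP_Player a dash ability triggered by the IA_Dash input action.
; On BeginPlay it casts its owner to BP_Player and caches it.
; Each dash launches the character along the X and Y of its current velocity scaled by DashDistance, so strength depends on movement speed.
; An IsDashing flag blocks further dashes until the DashCooldown delay ends.
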(event `self.ReceiveBeginPlay`
  (`self.Initialise`))

(event `EnhancedInput|/Game/Input/IA_Dash`
  (params (ActionValue :type Boolean) (ElapsedSeconds :type "Float (double-precision)") (TriggeredSeconds :type "Float (double-precision)") (InputAction :type "InputAction Object Reference" :default "/Game/Input/IA_Dash.IA_Dash"))
  (bind _owner (`self.Owner`))
  (bind (_returnvalue_x _returnvalue_y) (`KismetMathLibrary.BreakVector` (* (`Actor.GetVelocity` _owner) (`self.Dash Distance`))))
  (:`Triggered`
    (if (not (`self.IsDashing?`))
      (set `self.IsDashing?` true)
      (`Character.LaunchCharacter` _owner (`KismetMathLibrary.MakeVector` _returnvalue_x _returnvalue_y) false false)
      (`KismetSystemLibrary.Delay` (`self.Dash Cooldown`))
      (set `self.IsDashing?` false))))

(fn `Initialise`
  (bind _asbp_player (cast `/Game/Blueprints/BP_Player` (`self.GetOwner`)))
  (set `self.Owner` _asbp_player))