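; Player manager component that tracks how many players are alive and signals game over when none remain.
; Initialise seeds the count from the GameInstance's PlayerNum via BP_Gamemode, then binds to every BP_Player's health death and respawn events.
; Decrease and increase events adjust the count, clamped between zero and PlayerNum, print it for debugging, and fire the OnGameOver dispatcher at zero.
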(event `Decrease Alive Players`
  (bind _alive_players (`self.Alive Players`))
  ;[0.06301 0.6939 0.1441] Update number of alive players
  (if (not (<= _alive_players 0))
    (bind _output_get (set `self.Alive Players` (`KismetMathLibrary.Clamp` (- _alive_players 1) 0 (`self.Player Num`))))
    (`KismetSystemLibrary.PrintString` (`KismetStringLibrary.Concat_StrStr` "Players Alive: " (`KismetStringLibrary.Conv_IntToString` _output_get)) true true (struct :`G` 0.66 :`B` 1.0 :`A` 1.0) 2.0 "5")
    ;[0.06301 0.6939 0.1441] Game Over
    (if (<= (`self.Alive Players`) 0)
      (`KismetSystemLibrary.PrintString` "GAME OVER" true true (struct :`R` 1.0 :`G` 0.813439 :`A` 1.0) 2.0 "6")
      (`self.OnGameOver`))))

(event `Initialise`
  ;[0.06301 0.6939 0.1441] Initialise
  (`self.AlivePlayers`)
  (bind _outactors (`GameplayStatics.GetAllActorsOfClass` "/Game/Blueprints/BP_Player.BP_Player_C"))
  (for _array_element _outactors
    (bind _output_get (set `self.Player Ref` (cast `/Game/Blueprints/BP_Player` _array_element :!pure true)))
    (set `self.Health Component` (`Actor.GetComponentByClass` _output_get "/Game/Blueprints/Components/AC_HealthComponent.AC_HealthComponent_C"))
    (set `self.Respawn Component` (`Actor.GetComponentByClass` (`self.Player Ref`) "/Game/Blueprints/Components/AC_Respawn.AC_Respawn_C"))
    (add `/Game/Blueprints/Components/AC_HealthComponent.DeathEvent` (`self.Health Component`) (`|CreateDelegate` :!event `Decrease Alive Players`))
    (add `/Game/Blueprints/Components/AC_Respawn.OnRespawn` (`self.Respawn Component`) (`|CreateDelegate` :!event `Increase Alive Players`))))

(event `Reset On Game Over`
  ;[0.06301 0.6939 0.1441] Game Over
  (`/Engine/EditorBlueprintResources/StandardMacros.DoOnce` false :!via `Reset`))

(event `Increase Alive Players`
  ;[0.06301 0.6939 0.1441] Update number of alive players
  (bind _output_get (set `self.Alive Players` (`KismetMathLibrary.Clamp` (+ (`self.Alive Players`) 1) 0 (`self.Player Num`))))
  (`KismetSystemLibrary.PrintString` (`KismetStringLibrary.Concat_StrStr` "Players Alive: " (`KismetStringLibrary.Conv_IntToString` _output_get)) true true (struct :`G` 0.66 :`B` 1.0 :`A` 1.0) 2.0 "5"))

(fn `AlivePlayers`
  (bind _playernum (`/Game/Blueprints/GI_GameInstance.PlayerNum` (`/Game/Blueprints/BP_Gamemode.Game Instance` (cast `/Game/Blueprints/BP_Gamemode` (`GameplayStatics.GetGameMode`) :!pure true))))
  ;[0.06301 0.6939 0.1441] Number of players alive
  (set `self.Player Num` _playernum)
  (bind _output_get (set `self.Alive Players` _playernum))
  (`KismetSystemLibrary.PrintString` (`KismetStringLibrary.Concat_StrStr` "Players Alive: " (`KismetStringLibrary.Conv_IntToString` _output_get)) true true (struct :`G` 0.66 :`B` 1.0 :`A` 1.0) 2.0 "5"))