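; Level actor, an interactable stump, that switches the player to the weapon type set on it.
; On BeginPlay it shows that type on its text component and binds to the interactable component's OnInteracted dispatcher.
; Interacting writes the type to the player's ChosenWeaponType, refreshes the text, prints a message and calls WeaponPickUp, leaving weapon updates to the player.
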(event `self.ReceiveBeginPlay`
  ;[0 0.15 0.147 0.502] Begin Play Logic
  (`TextRenderComponent.K2_SetText` (`self.WeaponText`) (`KismetTextLibrary.Conv_StringToText` (`|GetEnumeratorNameAsString` (`self.WeaponType`))))
  ;[1 1 1] Event dispatcher for when the stump is interacted with
  (add `/Game/Components/Objects/AC_Interactable.OnInteracted` (`self.AC_Interactable`) (delegate `Activate Weapon Swap`)))

(event `Activate Weapon Swap`
  (params (Owner :type "/Game/Blueprints/Player/BP_Player Object Reference"))
  ;[1 1 1] Event for running weapon swap
  (bind _output_get (set `self.Player` Owner))
  ;[0 0.15 0.147 0.502] Weapon Select Logic
  (bind _output_get_2 (set `/Game/Blueprints/Player/BP_Player.ChosenWeaponType` (`self.WeaponType`) _output_get))
  (bind _returnvalue (`|GetEnumeratorNameAsString` _output_get_2))
  (`KismetSystemLibrary.PrintString` (`KismetStringLibrary.Concat_StrStr` _returnvalue " selected."))
  (`TextRenderComponent.K2_SetText` (`self.WeaponText`) (`KismetTextLibrary.Conv_StringToText` _returnvalue))
  ;;[1 1 1] Runs all weapon updates on Player
  (`/Game/Blueprints/Player/BP_Player.Weapon Pick Up` (`self.Player`)))

(event `self.ReceiveActorBeginOverlap`
  (params (OtherActor :type "Actor Object Reference"))
  ;[0 0.15 0.147 0.502] Weapon Select Logic
)

(fn `UserConstructionScript`)