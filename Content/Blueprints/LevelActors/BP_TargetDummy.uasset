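; BP_TargetDummy is a target dummy actor that gives visual feedback when damaged.
; On BeginPlay it initializes ACDamageIndicator with the dummy mesh and caches the mesh's world rotation.
; Each hit is passed to the indicator, then one of two timelines tilts and spins the mesh, with more spin for heavy hits.
; When the timeline finishes, the cached world rotation is applied as relative rotation.
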(event `self.ReceiveBeginPlay`
  (`/Game/Components/Pawns/AC_DamageIndicator.Initiate` (`self.AC_DamageIndicator`) (`self.Dummy Mesh`) 1.2)
  (set `self.Original Rotation` (`SceneComponent.K2_GetComponentRotation` (`self.Dummy Mesh`))))

(event `self.ReceiveAnyDamage`
  (params (Damage :type "Float (single-precision)") (DamageType :type "DamageType Object Reference") (InstigatedBy :type "Controller Object Reference") (DamageCauser :type "Actor Object Reference"))
  (bind _dummy_mesh (`self.Dummy Mesh`))
  (bind _dummy_mesh_2 (`self.Dummy Mesh`))
  (`/Game/Components/Pawns/AC_DamageIndicator.Damage Indicator` (`self.AC_DamageIndicator`) self Damage)
  (if (>= Damage 60.0)
    (bind (_direction _alpha) (`Timeline|Timeline_0` :!via `PlayFromStart`)
      (:`Update`
        (`SceneComponent.K2_SetRelativeRotation` _dummy_mesh_2 (`KismetMathLibrary.RLerp` (struct :`Roll` -25.0) (struct :`Yaw` 720.0) _alpha) false false))
      (:`Finished`
        (`SceneComponent.K2_SetRelativeRotation` _dummy_mesh_2 (`self.Original Rotation`) false false)))
    (else
      (bind (_direction_2 _alpha_2) (`Timeline|Timeline` :!via `PlayFromStart`)
        (:`Update`
          (`SceneComponent.K2_SetRelativeRotation` _dummy_mesh (`KismetMathLibrary.RLerp` (struct :`Roll` -20.0) (struct :`Yaw` 360.0) _alpha_2) false false))
        (:`Finished`
          (`SceneComponent.K2_SetRelativeRotation` _dummy_mesh (`self.Original Rotation`) false false))))))

(fn `UserConstructionScript`)