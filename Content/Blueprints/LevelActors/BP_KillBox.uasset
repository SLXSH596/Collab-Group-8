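; BP_KillBox is a level actor that damages or relocates actors that overlap its Box, likely for falls off the map.
; Actors in the SpecificActor list are moved immediately; others take lethal-scale damage of the kill-box damage type, then move one second later if still valid.
; Moves go to the actor's AC_Respawn RespawnLocation, falling back to the MoveLocation component.
; The delayed move reads a shared OverlappedActor variable, overwritten by each new overlap.
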(event `Move Actor`
  (params (`Overlapped Actor` :type "Actor Object Reference"))
  (bind _returnvalue (`self.GetComponentByClass` `Overlapped Actor` "/Game/Components/Player/AC_Respawn.AC_Respawn_C"))
  ;[0 1 0.1359] Move Actor
  (`/Engine/EditorBlueprintResources/StandardMacros.IsValid` _returnvalue
    (:`Is Valid`
      (`self.K2_SetActorLocation` `Overlapped Actor` (`/Game/Components/Player/AC_Respawn.Respawn Location` _returnvalue) false false))
    (:`Is Not Valid`
      (`self.K2_SetActorLocation` `Overlapped Actor` (`SceneComponent.K2_GetComponentLocation` (`self.Move Location`)) false false))))

(event `self.Box.OnComponentBeginOverlap`
  (params (OverlappedComponent :type "PrimitiveComponent Object Reference") (OtherActor :type "Actor Object Reference") (OtherComp :type "PrimitiveComponent Object Reference") (OtherBodyIndex :type Integer) (bFromSweep :type Boolean) (SweepResult :type "HitResult Structure (by ref)"))
  (bind _overlapped_actor (`self.Overlapped Actor`))
  ;[0 1 0.1359] Activate kill box
  (set `self.Overlapped Actor` OtherActor)
  (if (`KismetArrayLibrary.Array_Contains` (`self.Specific Actor`) OtherActor)
    (`self.Move Actor` OtherActor)
    (else
      (`self.Killbox` OtherActor)
      (`KismetSystemLibrary.Delay` 1.0)
      (`/Engine/EditorBlueprintResources/StandardMacros.IsValid` _overlapped_actor
        (:`Is Valid`
          (`self.Move Actor` _overlapped_actor))))))

(event `Killbox`
  (params (`Overlapped Actor` :type "Actor Object Reference"))
  ;[0 1 0.1359] Kill Box
  (`GameplayStatics.ApplyDamage` `Overlapped Actor` 1000.0 null self "/Game/Blueprints/WeaponDamageTypes/BP_DamageType_KillBox.BP_DamageType_KillBox_C"))

(fn `UserConstructionScript`)