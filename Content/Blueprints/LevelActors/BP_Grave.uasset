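; BP_Grave is a short-lived grave actor that picks a random mesh variant, animates vertically and then removes itself.
; On BeginPlay it sets the mesh from GraveVarients, stores its location and starts the animation.
; A timeline's alpha lerps the root between 100 units below that location and the location itself, destroying the actor on finish.
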(event `self.ReceiveBeginPlay`
  (`StaticMeshComponent.SetStaticMesh` (`self.Grave Mesh`) (`KismetArrayLibrary.Array_Random` (`self.Grave Varients`)))
  (set `self.Start Loc` (`self.K2_GetActorLocation`))
  (`self.Start Grave Anim`))

(event `Start Grave Anim`
  (bind (_direction _alpha) (`Timeline|Timeline`)
    (:`Update`
      (`SceneComponent.K2_SetRelativeLocation` (`self.DefaultSceneRoot`) (`KismetMathLibrary.VLerp` (- (`self.Start Loc`) (0.0 0.0 100.0)) (`self.Start Loc`) _alpha) false false))
    (:`Finished`
      (`self.K2_DestroyActor`))))

(fn `UserConstructionScript`)