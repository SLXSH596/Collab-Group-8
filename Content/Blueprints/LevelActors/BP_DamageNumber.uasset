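; BP_DamageNumber is an actor that shows a damage amount as a moving number, then removes itself.
; On BeginPlay it passes DmgAmt to its WBP_DamageAmount widget and refreshes the displayed number.
; A timeline lerps the actor's location from StartLoc to EndLoc, and the actor is destroyed when the timeline finishes.
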(event `self.ReceiveBeginPlay`
  (bind _aswbp_damage_amount (cast `/Game/UI/WBP_DamageAmount` (`WidgetComponent.GetWidget` (`self.Widget`))))
  (set `/Game/UI/WBP_DamageAmount.DmgAmt` (`self.DmgAmt`) _aswbp_damage_amount)
  (`/Game/UI/WBP_DamageAmount.Update Number` _aswbp_damage_amount)
  (bind (_direction _alpha) (`Timeline|Timeline`)
    (:`Update`
      (`self.K2_SetActorLocation` (`KismetMathLibrary.VLerp` (`self.Start Loc`) (`self.End Loc`) _alpha)))
    (:`Finished`
      (`self.K2_DestroyActor`))))

(fn `UserConstructionScript`)