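; Shared multiplayer camera actor that follows and frames all player pawns, set as player 0's view target by UpdateControllers.
; Each tick it moves to the midpoint of the pawns' min/max coordinate bounds from FindMinMaxPlayerCoords.
; The spring arm eases toward the larger padded X or Y span within clamped limits, with padding growing as it lengthens.
; Arm length also drives Radius and Distance in the MPC_MaterialFading parameter collection.
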(event `UpdateControllers`
  (params (PlayerControllers :type "Array of PlayerController Object Reference"))
  ;[0 1 0 0.5] Init - sets view target and gets references to player pawns
  (bind _output_get (set `self.PlayerControllers` PlayerControllers))
  (`KismetArrayLibrary.Array_Clear` (`self.PlayerPawns`))
  (for _array_element _output_get
    (`KismetArrayLibrary.Array_AddUnique` (`self.PlayerPawns`) (`Controller.K2_GetPawn` _array_element)))
  (`PlayerController.SetViewTargetWithBlend` (`GameplayStatics.GetPlayerController` 0) self 0.0 "VTBlend_Linear" 0.0 false))

(event `self.ReceiveTick`
  (params (DeltaSeconds :type "Float (single-precision)"))
  (bind (_minx _maxx _miny _maxy _minz _maxz) (`self.FindMinMaxPlayerCoords`))
  (bind _springarm (`self.SpringArm`))
  ;[1 0 0 0.5] Average location of players to move camera to
  (`self.K2_SetActorLocation` (`KismetMathLibrary.MakeVector` (/ (+ _minx _maxx) 2.0) (/ (+ _miny _maxy) 2.0) (/ (+ _minz _maxz) 2.0)))
  (bind _output_get (set `self.CameraZoomOffsetMultipled` (* (`self.CameraZoomOffset`) (`KismetMathLibrary.MapRangeClamped` (`SpringArmComponent.TargetArmLength` (`self.SpringArm`)) (`self.MinArmLength`) (`self.MaxArmLength`) 1.0 3.0))))
  (bind _returnvalue (- (+ _maxx _output_get) (- _minx _output_get)))
  (bind _returnvalue_2 (- (+ _maxy _output_get) (- _miny _output_get)))
  ;[0.162 0.02956 0.3515] Set spring arm length accordingly and clamp
  (bind _output_get_2 (set `SpringArmComponent.TargetArmLength` (`KismetMathLibrary.FInterpTo` (`SpringArmComponent.TargetArmLength` _springarm) (`KismetMathLibrary.FClamp` (`KismetMathLibrary.SelectFloat` _returnvalue _returnvalue_2 (> _returnvalue _returnvalue_2)) (`self.MinArmLength`) (`self.MaxArmLength`)) DeltaSeconds 3.5) _springarm))
  (`KismetMaterialLibrary.SetScalarParameterValue` "/Game/AI/TestAssets/CHimeraTest/Environment/MPC_MaterialFading.MPC_MaterialFading" "Radius" (`KismetMathLibrary.MapRangeClamped` _output_get_2 (`self.MinArmLength`) (`self.MaxArmLength`) 1300.0 3000.0))
  (`KismetMaterialLibrary.SetScalarParameterValue` "/Game/AI/TestAssets/CHimeraTest/Environment/MPC_MaterialFading.MPC_MaterialFading" "Distance" (`KismetMathLibrary.MapRangeClamped` _output_get_2 (`self.MinArmLength`) (`self.MaxArmLength`) 2200.0 5500.0)))

(fn `FindMinMaxPlayerCoords`
  (returns (MinX :type "Float (double-precision)") (MaxX :type "Float (double-precision)") (MinY :type "Float (double-precision)") (MaxY :type "Float (double-precision)") (MinZ :type "Float (double-precision)") (MaxZ :type "Float (double-precision)"))
  (locals (MinXPos :type "Float (double-precision)" :default 99999.0) (MaxXPos :type "Float (double-precision)" :default -99999.0) (MinYPos :type "Float (double-precision)" :default 99999.0) (MaxYPos :type "Float (double-precision)" :default -99999.0) (MinZPos :type "Float (double-precision)") (MaxZPos :type "Float (double-precision)"))
  (bind _playerpawns (`self.PlayerPawns`))
  (bind _returnvalue (`KismetArrayLibrary.Array_IsNotEmpty` _playerpawns))
  ;[0.162 0.02956 0.3515] Calculates the bounds of player coords for usage in camera operations
  (for _array_element _playerpawns
    (`|ExecutionSequence`
      (:`then_0`
        (bind (_returnvalue_x _returnvalue_y _returnvalue_z) (`KismetMathLibrary.BreakVector` (`self.K2_GetActorLocation` _array_element)))
        (if (< _returnvalue_x (`local.MinXPos`))
          (set `local.MinXPos` _returnvalue_x)))
      (:`then_1`
        (if (> _returnvalue_x (`local.MaxXPos`))
          (set `local.MaxXPos` _returnvalue_x)))
      (:`then_2`
        (if (< _returnvalue_y (`local.MinYPos`))
          (set `local.MinYPos` _returnvalue_y)))
      (:`then_3`
        (if (> _returnvalue_y (`local.MaxYPos`))
          (set `local.MaxYPos` _returnvalue_y)))
      (:`then_4`
        (if (> _returnvalue_z (`local.MaxZPos`))
          (set `local.MaxZPos` _returnvalue_z)))
      (:`then_5`
        (if (< _returnvalue_z (`local.MaxZPos`))
          (set `local.MinZPos` _returnvalue_z)))))
  (return (`KismetMathLibrary.SelectFloat` (`local.MinXPos`) 0.0 _returnvalue) (`KismetMathLibrary.SelectFloat` (`local.MaxXPos`) 0.0 _returnvalue) (`KismetMathLibrary.SelectFloat` (`local.MinYPos`) 0.0 _returnvalue) (`KismetMathLibrary.SelectFloat` (`local.MaxYPos`) 0.0 _returnvalue) (`KismetMathLibrary.SelectFloat` (`local.MinZPos`) 0.0 _returnvalue) (`KismetMathLibrary.SelectFloat` (`local.MaxZPos`) 0.0 _returnvalue)))

(fn `UserConstructionScript`)